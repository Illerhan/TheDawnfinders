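; BP_ThrowableLantern is a thrown light actor that glides to a stop and later removes itself.
; Tick moves it along its forward vector without sweep or physics, reducing speed linearly from MaxSpeed to zero.
; Delays chained on Tick wait out the deceleration time plus DelayBeforeOff.
; A Timeline then drives the point light's intensity for the switch-off and destroys the actor when finished.
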(event `self.ReceiveBeginPlay`
  (set `self.CurrentSpeed` (`self.MaxSpeed`)))

(event `self.ReceiveTick`
  (params (DeltaSeconds :type "Float (single-precision)"))
  (bind _currentspeed (`self.CurrentSpeed`))
  (bind _output_get (set `self.CurrentSpeed` (`KismetMathLibrary.FClamp` (- _currentspeed (* (`self.SpeedDecrease`) DeltaSeconds)) 0.0 _currentspeed)))
  (`self.K2_SetActorLocation` (+ (`self.K2_GetActorLocation`) (* (`self.GetActorForwardVector`) (* _output_get DeltaSeconds))))
  (`KismetSystemLibrary.Delay` (/ (`self.MaxSpeed`) (`self.SpeedDecrease`)))
  (`KismetSystemLibrary.Delay` (`self.DelayBeforeOff`))
  (bind (_direction _alpha) (`Timeline|Timeline`)
    (:`Update`
      (`LightComponent.SetIntensity` (`self.PointLight`) (`KismetMathLibrary.Lerp` 0.0 2500.0 _alpha)))
    (:`Finished`
      (`self.K2_DestroyActor`))))

(fn `UserConstructionScript`)