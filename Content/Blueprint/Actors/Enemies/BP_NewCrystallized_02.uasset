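; Crystallized enemy that reacts to noise, shedding its crystal mesh and chasing the source once alerted.
; Overlapping BP_Noise actors raise cooldown-gated alertness, shown by material swaps and reset on a timer; the alerted state persists.
; Tick chases by per-frame lerp, facing the target.
; After a delay, a self-triggered alert spreads once to same-class enemies within AlertRadius and every BP_NewEnemy_01, whose distance check compares self to self.
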(event `self.ReceiveBeginPlay`
  (`SceneComponent.SetWorldScale3D` (`self.DetectionRange`) (`KismetMathLibrary.Conv_DoubleToVector` (`self.DetectionRadius`))))

(event `self.ReceiveActorBeginOverlap`
  (params (OtherActor :type "Actor Object Reference"))
  (bind _asbp_noise (cast `/Game/Blueprint/Actors/BP_Noise` OtherActor))
  (if (not (> (`self.DelayTimer`) 0.0))
    (bind _output_get (set `self.AlertnessLevel` (+ (`self.AlertnessLevel`) 1)))
    (set `self.DelayTimer` (`self.DelayBetweenAlerts`))
    (set `self.AlertnessTimer` (`self.AlertnessDuration`))
    (if (>= _output_get 2)
      (`self.Alert` _asbp_noise)
      (`PrimitiveComponent.SetMaterial` (`self.Cube`) 0 "/Game/Art/PlaceHolder/Materials/M_EnemyAlert.M_EnemyAlert")
      (else
        (`PrimitiveComponent.SetMaterial` (`self.Cube`) 0 "/Game/Art/PlaceHolder/Materials/M_EnemySuspect.M_EnemySuspect")))))

(event `self.ReceiveTick`
  (params (DeltaSeconds :type "Float (single-precision)"))
  (bind (_returnvalue_x _returnvalue_y) (`KismetMathLibrary.BreakVector` (`self.K2_GetActorLocation`)))
  (bind (_returnvalue_x_2 _returnvalue_y_2) (`KismetMathLibrary.BreakVector` (`self.K2_GetActorLocation` (`self.Target`))))
  (set `self.DelayTimer` (- (`self.DelayTimer`) DeltaSeconds))
  (bind _output_get (set `self.AlertnessTimer` (- (`self.AlertnessTimer`) DeltaSeconds)))
  (if (<= _output_get 0.0)
    (`PrimitiveComponent.SetMaterial` (`self.Cube`) 0 "/Game/Art/PlaceHolder/Materials/M_EnemyMove.M_EnemyMove")
    (set `self.AlertnessLevel` 0))
  (if (`self.isAlerted`)
    (`self.K2_SetActorLocation` (`KismetMathLibrary.VLerp` (`self.K2_GetActorLocation`) (`self.K2_GetActorLocation` (`self.Target`)) 0.01))
    (`self.K2_SetActorRotation` (`KismetMathLibrary.ComposeRotators` (`KismetMathLibrary.FindLookAtRotation` (`KismetMathLibrary.MakeVector` _returnvalue_x _returnvalue_y) (`KismetMathLibrary.MakeVector` _returnvalue_x_2 _returnvalue_y_2)) (struct :`Yaw` -90.0)))))

(event `Alert`
  (params (TargetActor :type "Actor Object Reference") (IsAlertedByOther :type Boolean))
  (if (not (`self.isAlerted`))
    (set `self.isAlerted` true)
    (`ActorComponent.K2_DestroyComponent` (`self.SM_VivianiteClusterBig_002`))
    (bind _output_get (set `self.Target` TargetActor))
    (if (not IsAlertedByOther)
      (`KismetSystemLibrary.Delay` 1.0)
      (`|ExecutionSequence`
        (:`then_0`
          (bind _outactors (`GameplayStatics.GetAllActorsOfClass` "/Game/Blueprint/Actors/Enemies/BP_NewEnemy_01.BP_NewEnemy_01_C"))
          (for _array_element _outactors
            (if (<= (`KismetMathLibrary.Vector_Distance` (`self.K2_GetActorLocation`) (`self.K2_GetActorLocation`)) (`self.AlertRadius`))
              (`/Game/Blueprint/Actors/Enemies/BP_NewEnemy_01.Alert` _array_element _output_get true))))
        (:`then_1`
          (bind _outactors_2 (`GameplayStatics.GetAllActorsOfClass` "BP_NewCrystallized_02_C"))
          (for _array_element_2 _outactors_2
            (if (<= (`KismetMathLibrary.Vector_Distance` (`self.K2_GetActorLocation` _array_element_2) (`self.K2_GetActorLocation`)) (`self.AlertRadius`))
              (`self.Alert` _array_element_2 _output_get true))))))))

(fn `UserConstructionScript`)