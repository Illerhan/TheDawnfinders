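; BP_AimLine is a player aim-line actor that shows a straight line from an origin actor along a given direction.
; Show and Hide toggle the Line component's visibility.
; SetPosition shows the line, moves the actor to the range's midpoint, yaws it toward the origin and scales the Line's Z to match the range.
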(event `Show`
  (`SceneComponent.SetVisibility` (`self.Line`) true false))

(event `Hide`
  (`SceneComponent.SetVisibility` (`self.Line`) false false))

(event `SetPosition`
  (params (Origin :type "Actor Object Reference") (Direction :type "Vector Structure") (Range :type "Float (double-precision)"))
  (bind _returnvalue (`self.K2_GetActorLocation` Origin))
  (`self.Show`)
  (`self.K2_SetActorLocation` (+ _returnvalue (* Direction (* Range 0.5))))
  (`self.K2_SetActorRotation` (`KismetMathLibrary.MakeRotator` 0.0 0.0 (`KismetMathLibrary.DegAtan2` (.y (- _returnvalue (`self.K2_GetActorLocation`))) (.x (- _returnvalue (`self.K2_GetActorLocation`))))))
  (`SceneComponent.SetWorldScale3D` (`self.Line`) (`KismetMathLibrary.MakeVector` 0.1 0.1 (* Range 0.01))))

(fn `UserConstructionScript`)