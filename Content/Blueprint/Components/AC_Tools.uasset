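; Actor component that manages a fixed-size tool inventory with a selected slot.
; BeginPlay creates empty slots, AddNewItem fills the first free one, and ChangeCurrentSlot cycles the selection with wraparound.
; Throw traces down from a fixed world-space offset beside the player pawn, spawns a BP_Item there with the slot's data, then empties the slot.
; Each change broadcasts OnInventoryChange with the slots and current index.
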(event `self.ReceiveBeginPlay`
  ; Begin Play
  (`parent.ReceiveBeginPlay`)
  (for _ (range 7)
    (`KismetArrayLibrary.Array_Add` (`self.InventorySlots`) (make `InventorySlot` null)))
  (`self.OnInventoryChange` (`self.InventorySlots`) (`self.CurrentSlotIndex`)))

(event `self.AddNewItem`
  (params (NewItem :type "ItemData Object Reference"))
  ; Add New Item
  (for (_array_element _array_index) (`self.InventorySlots`)
    (`/Engine/EditorBlueprintResources/StandardMacros.IsValid` (`.ItemData` (break `InventorySlot` _array_element))
      (:`Is Not Valid`
        (`KismetArrayLibrary.Array_Set` (`self.InventorySlots`) _array_index (make `InventorySlot` NewItem 1))
        (`self.OnInventoryChange` (`self.InventorySlots`) (`self.CurrentSlotIndex`))
        (break)))))

(event `self.Throw`
  (bind _itemdata (break `InventorySlot` (`|GetArrayItem` (`self.InventorySlots`) (`self.CurrentSlotIndex`))))
  (bind _returnvalue (+ (.location (`Actor.GetTransform` (`GameplayStatics.GetPlayerPawn` 0))) (100.0 0.0 0.0)))
  ; Throw
  (`/Engine/EditorBlueprintResources/StandardMacros.IsValid` _itemdata
    (:`Is Valid`
      (bind _outhit (`KismetSystemLibrary.LineTraceSingle` _returnvalue (+ _returnvalue (0.0 0.0 -2000.0)) "TraceTypeQuery1"))
      (`|SpawnActorFromClass` "/Game/Blueprint/Actors/LDElements/BP_Item.BP_Item_C" (`KismetMathLibrary.MakeTransform` (`.Location` (`GameplayStatics.BreakHitResult` _outhit))) "Undefined" "MultiplyWithRoot" null _itemdata null)
      (`KismetArrayLibrary.Array_Set` (`self.InventorySlots`) (`self.CurrentSlotIndex`) (make `InventorySlot` null))
      (`self.OnInventoryChange` (`self.InventorySlots`) (`self.CurrentSlotIndex`)))))

(fn `ChangeCurrentSlot`
  (params (IndexGoUp :type Boolean))
  (returns (ReturnValue :type "InventorySlot Structure"))
  (if IndexGoUp
    (bind _result (`/Engine/EditorBlueprintResources/StandardMacros.IncrementInt` (`self.CurrentSlotIndex`))
      (:`  `
        (if (>= _result (`KismetArrayLibrary.Array_Length` (`self.InventorySlots`)))
          (set `self.CurrentSlotIndex` 0))))
    (else
      (bind _result_2 (`/Engine/EditorBlueprintResources/StandardMacros.DecrementInt` (`self.CurrentSlotIndex`))
        (:`  `
          (if (< _result_2 0)
            (set `self.CurrentSlotIndex` (- (`KismetArrayLibrary.Array_Length` (`self.InventorySlots`)) 1)))))))
  (`self.OnInventoryChange` (`self.InventorySlots`) (`self.CurrentSlotIndex`))
  (return (`|GetArrayItem` (`self.InventorySlots`) (`self.CurrentSlotIndex`))))

(fn `GetCurrentSlot`
  (returns (ReturnValue :type "InventorySlot Structure"))
  (return (`|GetArrayItem` (`self.InventorySlots`) (`self.CurrentSlotIndex`))))