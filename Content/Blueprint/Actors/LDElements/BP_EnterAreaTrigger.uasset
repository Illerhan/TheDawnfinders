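; BP_EnterAreaTrigger is a level-design trigger actor that shows an area name on screen when the player enters it.
; Its box overlap filters for Player-tagged actors and records each one so the effect plays only once per actor.
; For a locally controlled character, it calls the enter-area widget on the custom HUD's main widget with its AreaName, keeping the display local to that player.
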(event `self.Box.OnComponentBeginOverlap`
  (params (OverlappedComponent :type "PrimitiveComponent Object Reference") (OtherActor :type "Actor Object Reference") (OtherComp :type "PrimitiveComponent Object Reference") (OtherBodyIndex :type Integer) (bFromSweep :type Boolean) (SweepResult :type "HitResult Structure (by ref)"))
  (bind _alreadytriggeredactors (`self.AlreadyTriggeredActors`))
  (if (`self.ActorHasTag` OtherActor "Player")
    (if (not (`KismetArrayLibrary.Array_Contains` _alreadytriggeredactors OtherActor))
      (`KismetArrayLibrary.Array_Add` _alreadytriggeredactors OtherActor)
      (bind _ascharacter (cast `Character` OtherActor))
      (if (`Pawn.IsLocallyControlled` _ascharacter)
        (bind _ashud_custom (cast `/Game/Blueprint/GameFramework/HUD_Custom` (`PlayerController.GetHUD` (`GameplayStatics.GetPlayerController` 0))))
        (`/Game/UI/Widgets/WBP_EnterArea.DoEffect` (`/Game/UI/Widgets/WBP_MainWidget.WBP_EnterArea` (`/Game/Blueprint/GameFramework/HUD_Custom.MainWidgetRef` _ashud_custom)) (`self.AreaName`))))))

(fn `UserConstructionScript`)