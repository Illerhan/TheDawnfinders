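; Handler actor that drives the blend weight of one post process from several local volumes.
; On BeginPlay it registers itself and an array index with each entry in its Volumes list.
; SetWeight stores a weight at the given index and sets the PostProcess BlendWeight to the maximum of all stored weights, so overlapping influences do not add up.
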(event `self.ReceiveBeginPlay`
  (for (_array_element _array_index) (`self.Volumes`)
    (`/Game/Blueprint/Actors/ProcessVolumes/BP_LocalVolume.SetHandler` _array_element self _array_index)))

(event `SetWeight`
  (params (Weight :type "Float (double-precision)") (Index :type Integer))
  (`KismetArrayLibrary.Array_Set` (`self.Weights`) Index Weight true)
  (set `PostProcessVolume.BlendWeight` (`.MaxValue` (`KismetMathLibrary.MaxOfFloatArray` (`self.Weights`))) (`self.PostProcess`)))

(fn `UserConstructionScript`)