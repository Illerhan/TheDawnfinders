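; BP_Brasero is an interactible brazier level element that lights up when used.
; On interaction, the server sets the point light to its lit intensity and enables overlap events on the FogOfWarCollider.
; NewIntensity has an OnRep that applies the light intensity on clients, while the overlap flag is set only in the authority branch.
; The collider's begin and end overlaps call FadeInMessage and FadeOutMessage on the overlapping actor.
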(event `self.BP_OnInteraction`
  (params (Player :type "APlayerCharacter Object Reference"))
  (`/Engine/EditorBlueprintResources/ActorMacros.Switch Has Authority`
    (:`Authority`
      (bind _output_get (set `self.New Intensity` (`self.LightIntensity`)))
      (`LightComponent.SetIntensity` (`self.PointLight`) _output_get)
      (set `PrimitiveComponent.bGenerateOverlapEvents` true (`self.FogOfWarCollider`)))))

(event `self.FogOfWarCollider.OnComponentBeginOverlap`
  (params (OverlappedComponent :type "PrimitiveComponent Object Reference") (OtherActor :type "Actor Object Reference") (OtherComp :type "PrimitiveComponent Object Reference") (OtherBodyIndex :type Integer) (bFromSweep :type Boolean) (SweepResult :type "HitResult Structure (by ref)"))
  (message `Fadeable.FadeIn` OtherActor))

(event `self.FogOfWarCollider.OnComponentEndOverlap`
  (params (OverlappedComponent :type "PrimitiveComponent Object Reference") (OtherActor :type "Actor Object Reference") (OtherComp :type "PrimitiveComponent Object Reference") (OtherBodyIndex :type Integer))
  (message `Fadeable.FadeOut` OtherActor))

(fn `OnRep_New Intensity`
  (`LightComponent.SetIntensity` (`self.PointLight`) (`self.New Intensity`)))

(fn `UserConstructionScript`)