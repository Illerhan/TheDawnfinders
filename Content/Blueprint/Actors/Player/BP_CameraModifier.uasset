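; BP_CameraModifier is a placeable trigger volume that overrides the player camera while the player stands inside it.
; On box overlap by an actor tagged Player, it tells the player character's camera component to force its position to the volume's location, using its distance and lerp speed parameters.
; When the player leaves the box, it returns the camera component to automatic control.
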(event `self.Box.OnComponentBeginOverlap`
  (params (OverlappedComponent :type "PrimitiveComponent Object Reference") (OtherActor :type "Actor Object Reference") (OtherComp :type "PrimitiveComponent Object Reference") (OtherBodyIndex :type Integer) (bFromSweep :type Boolean) (SweepResult :type "HitResult Structure (by ref)"))
  (if (`self.ActorHasTag` OtherActor "Player")
    (bind _asbp_player_character (cast `/Game/Blueprint/Actors/Player/BP_PlayerCharacter` OtherActor))
    (`PlayerCameraComponent.StartForcePosition` (`/Game/Blueprint/Actors/Player/BP_PlayerCharacter.Camera Component` _asbp_player_character) (`self.K2_GetActorLocation`) (`self.DistanceParameter`) (`self.LerpDistSpeedParameter`) (`self.LerpOffsetSpeedParameter`))))

(event `self.Box.OnComponentEndOverlap`
  (params (OverlappedComponent :type "PrimitiveComponent Object Reference") (OtherActor :type "Actor Object Reference") (OtherComp :type "PrimitiveComponent Object Reference") (OtherBodyIndex :type Integer))
  (if (`self.ActorHasTag` OtherActor "Player")
    (bind _asbp_player_character (cast `/Game/Blueprint/Actors/Player/BP_PlayerCharacter` OtherActor))
    (`PlayerCameraComponent.StartAutomaticControl` (`/Game/Blueprint/Actors/Player/BP_PlayerCharacter.Camera Component` _asbp_player_character))))

(fn `UserConstructionScript`)