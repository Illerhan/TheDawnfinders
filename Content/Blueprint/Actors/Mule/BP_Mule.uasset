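; The mule is a loot carrier that collects valuables and carried heavy items into itself.
; Its loot collider takes in vivianite and players' carried items, stores a loose valuable item behind a DoOnce, and tracks nearby player inventories.
; On Tick, the authority moves one treasure slot at a time from those inventories on per-inventory cooldowns, spawning a flying treasure effect and widget feedback for each transfer.
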(event `self.LootCollider.OnComponentBeginOverlap`
  (params (OverlappedComponent :type "PrimitiveComponent Object Reference") (OtherActor :type "Actor Object Reference") (OtherComp :type "PrimitiveComponent Object Reference") (OtherBodyIndex :type Integer) (bFromSweep :type Boolean) (SweepResult :type "HitResult Structure (by ref)"))
  (bind _asbp_carriable_vivianite (cast `/Game/Blueprint/Actors/LDElements/Interactibles/Carriables/BP_CarriableVivianite` OtherActor)
    (:`then`
      (`Carriable.PutInTargetActor` _asbp_carriable_vivianite self))
    (:`CastFailed`
      (bind _asbp_item (cast `/Game/Blueprint/Actors/LDElements/BP_Item` OtherActor)
        (:`then`
          (bind _itemdata (`Item.ItemData` _asbp_item))
          (if (`|EnumEquality` (`ItemData.ItemType` _itemdata) "Valuable")
            (`/Engine/EditorBlueprintResources/StandardMacros.DoOnce` false
              (:`Completed`
                (`InventoryComponent.AddNewItem` (`self.InventoryComponent`) (make `ItemInfos` _itemdata) 1)
                (`self.K2_DestroyActor` _asbp_item)))))
        (:`CastFailed`
          (bind _asbp_player_character (cast `/Game/Blueprint/Actors/Player/BP_PlayerCharacter` OtherActor))
          (bind _interactioncomponent (`APlayerCharacter.InteractionComponent` _asbp_player_character))
          (`/Engine/EditorBlueprintResources/StandardMacros.IsValid` (`InteractionComponent.CarriedItem` _interactioncomponent)
            (:`Is Valid`
              (`InteractionComponent.PutInHeavyItem` _interactioncomponent self))
            (:`Is Not Valid`
              _))
          (`KismetArrayLibrary.Array_Add` (`self.Inventory Components at Range`) (`APlayerCharacter.InventoryComponent` _asbp_player_character)))))))

(event `self.LootCollider.OnComponentEndOverlap`
  (params (OverlappedComponent :type "PrimitiveComponent Object Reference") (OtherActor :type "Actor Object Reference") (OtherComp :type "PrimitiveComponent Object Reference") (OtherBodyIndex :type Integer))
  (bind _asbp_player_character (cast `/Game/Blueprint/Actors/Player/BP_PlayerCharacter` OtherActor))
  (`KismetArrayLibrary.Array_RemoveItem` (`self.Inventory Components at Range`) (`APlayerCharacter.InventoryComponent` _asbp_player_character)))

(event `self.ReceiveTick`
  (params (DeltaSeconds :type "Float (single-precision)"))
  (`parent.ReceiveTick` DeltaSeconds)
  (`/Engine/EditorBlueprintResources/ActorMacros.Switch Has Authority`
    (:`Authority`
      (if (> (`KismetArrayLibrary.Array_Length` (`self.Inventory Components at Range`)) 0)
        (for (_array_element _array_index) (`self.Inventory Components at Range`)
          (if (> (`|GetArrayItem` (`self.Inventories Delays`) _array_index) 0.0)
            (`KismetArrayLibrary.Array_Set` (`self.Inventories Delays`) _array_index (- (`|GetArrayItem` (`self.Inventories Delays`) _array_index) DeltaSeconds))
            (else
              (bind _returnvalue (`InventoryComponent.GetHasTreasures` _array_element))
              (if _returnvalue
                (`self.TransferValuableFromPla` _array_element)
                (`KismetArrayLibrary.Array_Set` (`self.Inventories Delays`) _array_index 0.35)))))))))

(event `DoTreasureFeedback`
  (params (Data :type "ItemData Object Reference") (Start :type "Vector Structure"))
  (bind _returnvalue (`|SpawnActorFromClass` "/Game/Blueprint/Actors/Others/BP_TreasureToPalanquin.BP_TreasureToPalanquin_C" (`KismetMathLibrary.MakeTransform` Start) "Undefined" "MultiplyWithRoot" null null))
  (`/Game/Blueprint/Actors/Others/BP_TreasureToPalanquin.Setup` _returnvalue (`self.K2_GetActorLocation`) 0.4)
  (`KismetSystemLibrary.Delay` 0.3)
  (`WorldInteractibleWidget.DoTreasureFeedback` :`self` (`self.InteractibleWidget`) :`Text` (`ItemData.ItemName` Data)))

(event `TransferValuableFromPla`
  (params (InventoryComp :type "InventoryComponent Object Reference"))
  (bind _treasureslots (`InventoryComponent.TreasureSlots` InventoryComp))
  (for _array_element _treasureslots
    (`/Engine/EditorBlueprintResources/StandardMacros.IsValid` (break `ItemInfos` (break `InventorySlot` _array_element))
      (:`Is Valid`
        (`InventoryComponent.AddNewItem` (`self.InventoryComponent`) (make `ItemInfos` (break `ItemInfos` (break `InventorySlot` _array_element))) (`.Quantity` (break `InventorySlot` _array_element)))
        (`self.DoTreasureFeedback` (break `ItemInfos` (break `InventorySlot` _array_element)) (`self.K2_GetActorLocation` (`ActorComponent.GetOwner` InventoryComp)))
        (break))))
  (for (_array_element_2 _array_index) _treasureslots
    (`/Engine/EditorBlueprintResources/StandardMacros.IsValid` (break `ItemInfos` (break `InventorySlot` _array_element_2))
      (:`Is Valid`
        (`InventoryComponent.RemoveItemAtIndex` InventoryComp _array_index true true)
        (break)))))

(fn `UserConstructionScript`)