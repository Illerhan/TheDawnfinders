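; Tutorial trigger actor that drops a rock and sets off a linked spike trap when an actor overlaps it.
; Overlap plays a Wwise crumble sound above the Rock and activates it, then plays an impact sound after a timed delay.
; The Spike's trigger type switches to duration-based at impact and reverts to collider-enter shortly after, when the trigger destroys itself.
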(event `self.ReceiveActorBeginOverlap`
  (params (OtherActor :type "Actor Object Reference"))
  (bind _spike (`self.Spike`))
  (`AkGameplayStatics.PostEventAtLocation` "/Game/WwiseAudio/Events/Default_Work_Unit/Objets/Elements_de_LD/Rocks/Play_RockCrumble.Play_RockCrumble" (+ (`self.K2_GetActorLocation` (`self.Rock`)) (0.0 0.0 100.0)))
  (`/Game/Blueprint/Actors/LDElements/BP_Physics_Rocks.Activate` (`self.Rock`))
  (`KismetSystemLibrary.Delay` 1.1)
  (`AkGameplayStatics.PostEvent` "/Game/WwiseAudio/Events/Default_Work_Unit/Objets/Elements_de_LD/Rocks/Play_RockImpact.Play_RockImpact")
  (set `TrapBase.TrapTriggerType` "OnDuration" _spike)
  (`KismetSystemLibrary.Delay` 0.5)
  (set `TrapBase.TrapTriggerType` "OnColliderEnter" _spike)
  (`self.K2_DestroyActor`))

(fn `UserConstructionScript`)