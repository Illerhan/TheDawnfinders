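; Danger manager actor that escalates threat over time, on mule calls and on throttled enemy detections.
; Authority tick accumulates danger toward a multiplicatively scaled threshold, with RepNotifies refreshing the HUD danger widget.
; Each level-up activates that level's registered enemies, reveals a random pre-placed zealot and can open linked doors at a set level.
; It also changes the local player's max health and plays warning text, flame and radial blur effects.
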(event `Call Mule`
  ; Increase Danger Manager Events
  (`self.MuleCalled`))

(event `CreateDangerWidget`
  (params (OwningPlayer :type "PlayerController Object Reference"))
  (bind _ashud_custom (cast `/Game/Blueprint/GameFramework/HUD_Custom` (`PlayerController.GetHUD` (`GameplayStatics.GetPlayerController` 0))))
  (set `self.Widget` (`/Game/UI/Widgets/WBP_MainWidget.WBP_Danger` (`/Game/Blueprint/GameFramework/HUD_Custom.MainWidgetRef` _ashud_custom)))
  (bind _returnvalue (`|CreateWidget` "/Game/UI/Widgets/WBP_TutorialText.WBP_TutorialText_C" OwningPlayer))
  (bind _output_get (set `self.WidgetText` _returnvalue))
  (`UserWidget.AddToViewport` _output_get 0)
  (`self.Set Widget`)
  (`/Game/UI/Widgets/WBP_TutorialText.SetOpacity` (`self.WidgetText`) 0.0))

(event `Set Widget`
  (`/Game/UI/Widgets/WBP_Danger.Update Widget` (`self.Widget`) (/ (`self.CurrentDanger`) (`self.DangerPerLevel`)) (`self.CurrentLevel`) (`self.MaxLevel`)))

(event `self.MuleCalled`
  ; Increase Danger Manager Events
  (`self.IncreaseDangerLevel` (`self.MuleDangerCost`)))

(event `EnnemiesDetection`
  ; Increase Danger Manager Events
  (if (<= (`self.SmallTimer`) 0.0)
    (`self.IncreaseDangerLevel` (`self.EnnemiesCost`))
    (set `self.SmallTimer` 1.5)))

(event `self.IncreaseDangerLevel`
  (params (DangerCost :type "Float (single-precision)"))
  ; Increase Danger Level
  (if (< (`self.CurrentLevel`) (`self.MaxLevel`))
    (bind _output_get (set `self.CurrentDanger` (+ (`self.CurrentDanger`) DangerCost)))
    (if (>= _output_get (`self.DangerPerLevel`))
      (`self.Increase Level`)
      (else
        (`self.Set Widget`)))))

(event `Flame Opacity`
  (bind (_direction _alpha) (`Timeline|Timeline_1`)
    (:`Update`
      (`/Game/UI/Widgets/WBP_Danger.SetOpacity` (`self.Widget`) _alpha))))

(event `self.ReceiveTick`
  (params (DeltaSeconds :type "Float (single-precision)"))
  (if (`self.HasAuthority`)
    (`self.IncreaseDangerLevel` (* DeltaSeconds (`self.DangerPerSecond`)))
    (set `self.SmallTimer` (- (`self.SmallTimer`) DeltaSeconds))))

(event `Increase Level`
  ; Increase Danger Level
  (set `self.CurrentDanger` (- (`self.CurrentDanger`) (`self.DangerPerLevel`)))
  (set `self.DangerPerLevel` (* (`self.DangerPerLevel`) (`self.IncreasePerLevel`)))
  (`/Engine/EditorBlueprintResources/StandardMacros.IncrementInt` (`self.CurrentLevel`)
    (:`  `
      (`self.Set Widget`)
      (`self.Spawn New Enemies`)
      (`self.Spawn New Zealot`)
      (`self.Fade Text`)
      (`self.LoseMaxHealth`)
      (`self.Flame Opacity`)
      (bind (_direction _newtrack_0) (`Timeline|PostProcessTimeline` :!via `PlayFromStart`)
        (:`Update`
          (`KismetMaterialLibrary.SetScalarParameterValue` "/Game/Art/Materials/CollectionParameter/MPC_PostProcessEffects.MPC_PostProcessEffects" "RADIALBLUR-GeneralOpacity" _newtrack_0))))))

(event `Fade Text`
  (`/Game/UI/Widgets/WBP_TutorialText.SetText` (`self.WidgetText`) "Danger is rising. Servants of Apophis are awakening...")
  (bind (_direction _alpha) (`Timeline|Timeline` :!via `PlayFromStart`)
    (:`Update`
      (`/Game/UI/Widgets/WBP_TutorialText.SetOpacity` (`self.WidgetText`) _alpha))
    (:`Finished`
      (bind (_direction_2 _alpha_2) (`Timeline|Timeline_0` :!via `ReverseFromEnd`)
        (:`Update`
          (`/Game/UI/Widgets/WBP_TutorialText.SetOpacity` (`self.WidgetText`) _alpha_2))))))

(event `Spawn New Enemies`
  (bind _returnvalue (`EnemyRegistry.GetEnemiesByDangerLevel` (subsystem `EnemyRegistry`) (`self.CurrentLevel`)))
  ; Spawn Enemies
  (if (not (<= (`KismetArrayLibrary.Array_Length` _returnvalue) 0))
    (for _array_element _returnvalue
      (bind _asbp_enemy_master (cast `/Game/Blueprint/Actors/Enemies/BP_EnemyMaster` _array_element))
      (`/Game/Blueprint/Actors/Enemies/BP_EnemyMaster.ActivateEnemy` _asbp_enemy_master))
    (if (== (`self.LevelOpeningDoor`) (`self.CurrentLevel`))
      (for _array_element_2 (`self.LinkedDoors`)
        (`Doors.StartOpening` _array_element_2)))))

(event `LoseMaxHealth`
  (bind _returnvalue (`GameplayStatics.GetPlayerController` 0))
  ;[0.8229 0.2169 0 0.5] Curse
  (if (`Controller.IsLocalPlayerController` _returnvalue)
    (bind _asbp_player_character (cast `/Game/Blueprint/Actors/Player/BP_PlayerCharacter` (`Controller.K2_GetPawn` _returnvalue)))
    (`HealthComponent.ChangeCurrentMaxHealth` (`APlayerCharacter.HealthComponent` _asbp_player_character) (`self.HealthReduction`))))

(event `Spawn New Zealot`
  (bind _spawnablezealots (`self.SpawnableZealots`))
  (bind _returnvalue (`KismetArrayLibrary.Array_Length` _spawnablezealots))
  ; Spawn Enemies
  (if (> _returnvalue 0)
    (bind _output_get (set `self.RandomInt` (`KismetMathLibrary.RandomIntegerInRange` 0 (- _returnvalue 1))))
    (bind _output (`|GetArrayItem` _spawnablezealots _output_get))
    (`self.SetActorHiddenInGame` _output false)
    (`self.SetActorTickEnabled` _output true)
    (`self.SetActorEnableCollision` _output true)
    (`KismetArrayLibrary.Array_Remove` (`self.SpawnableZealots`) (`self.RandomInt`))))

(fn `OnRep_CurrentDanger`
  (`self.Set Widget`))

(fn `OnRep_CurrentLevel`
  (`self.Set Widget`))

(fn `UserConstructionScript`)