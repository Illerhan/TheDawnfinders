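; BP_TreasureToPalanquin is a short-lived actor that moves from its current location to a given end position, by its name a treasure flying to a palanquin.
; Setup records the start position, end position and duration, and resets the timer.
; Tick moves the actor along a sinusoidal ease-out between the two points, then only the authority destroys it once the duration has passed.
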(event `Setup`
  (params (EndPos :type "Vector Structure") (Duration :type "Float (double-precision)"))
  (set `self.EndPos` EndPos)
  (set `self.Timer` 0.0)
  (set `self.StartPos` (`self.K2_GetActorLocation`))
  (set `self.Duration` Duration))

(event `self.ReceiveTick`
  (params (DeltaSeconds :type "Float (single-precision)"))
  (bind _output_get (set `self.Timer` (+ (`self.Timer`) DeltaSeconds)))
  (`self.K2_SetActorLocation` (`|EaseFunction` "SinusoidalOut" (/ _output_get (`self.Duration`)) (`self.StartPos`) (`self.EndPos`)))
  (if (> (`self.Timer`) (`self.Duration`))
    (`/Engine/EditorBlueprintResources/ActorMacros.Switch Has Authority`
      (:`Authority`
        (`self.K2_DestroyActor`)))))

(fn `UserConstructionScript`)