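; BP_FogOfWar is a light-area actor that tells overlapping actors when they enter or leave its light for the fog-of-war system.
; Overlap begin and end events run only on the authority, calling BPI_FogOfWar light on/off messages on implementing actors.
; An IsPalanquin flag selects palanquin-specific messages; otherwise the generic messages pass along IsTorchLight.
; At BeginPlay, the Cone's collision is disabled, then switched to query-only after a brief delay.
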(event `self.ReceiveBeginPlay`
  (`PrimitiveComponent.SetCollisionEnabled` (`self.Cone`) "NoCollision")
  (`KismetSystemLibrary.Delay` 0.1)
  (`PrimitiveComponent.SetCollisionEnabled` (`self.Cone`) "QueryOnly"))

(event `self.ReceiveActorBeginOverlap`
  (params (OtherActor :type "Actor Object Reference"))
  (`/Engine/EditorBlueprintResources/ActorMacros.Switch Has Authority`
    (:`Authority`
      (if (`KismetSystemLibrary.DoesImplementInterface` OtherActor "/Game/Blueprint/Interface/BPI_FogOfWar.BPI_FogOfWar_C")
        (if (`self.isPalanquin`)
          (message `/Game/Blueprint/Interface/BPI_FogOfWar.Palanquin Light On` OtherActor)
          (else
            (message `/Game/Blueprint/Interface/BPI_FogOfWar.Light On` OtherActor (`self.isTorchLight`))))))))

(event `self.ReceiveActorEndOverlap`
  (params (OtherActor :type "Actor Object Reference"))
  (`/Engine/EditorBlueprintResources/ActorMacros.Switch Has Authority`
    (:`Authority`
      (if (`KismetSystemLibrary.DoesImplementInterface` OtherActor "/Game/Blueprint/Interface/BPI_FogOfWar.BPI_FogOfWar_C")
        (if (`self.isPalanquin`)
          (message `/Game/Blueprint/Interface/BPI_FogOfWar.Palanquin Light Off` OtherActor)
          (else
            (message `/Game/Blueprint/Interface/BPI_FogOfWar.Light Off` OtherActor (`self.isTorchLight`))))))))

(fn `UserConstructionScript`)