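; Main lobby game mode that tracks player controllers and seats each one on a BP_SpawnPoints actor.
; Spawn points are ordered by index tag, then UpdatePlayersOnSpawns fills free points and clears stale ones after login, seamless travel or a one-shot startup scan.
; It also requests client save loads, checks lobby readiness and backs up inventory and stash to PlayerState before seamless travel.
; Countdown events only loop and cast controllers.
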(event `self.ReceiveBeginPlay`
  (`self.SetUpSpawnPoints`)
  (bind _returnvalue (`KismetSystemLibrary.K2_SetTimerDelegate` (delegate `ChecklAndSPawnCharacters`) 0.5 true))
  (set `self.HandleSpawn` _returnvalue))

(event `AddPlayerAlive`
  (params (Player :type "APlayerCharacter Object Reference (by ref)"))
  (`KismetArrayLibrary.Array_Add` (`self.PlayersAlive`) Player))

(event `ChecklAndSPawnCharacters`
  (bind _asbp_custom_game_state (cast `/Game/Blueprint/GameFramework/BP_CustomGameState` (`GameplayStatics.GetGameState`)))
  (for _array_element (`GameStateBase.PlayerArray` _asbp_custom_game_state)
    (`KismetArrayLibrary.Array_Add` (`self.PCs`) (`PlayerState.GetPlayerController` _array_element)))
  (`KismetSystemLibrary.K2_ClearAndInvalidateTimerHandle` (`self.HandleSpawn`))
  (`self.UpdatePlayersOnSpawns`))

(event `RemovePlayerAlive`
  (params (Player :type "APlayerCharacter Object Reference (by ref)"))
  (`KismetArrayLibrary.Array_RemoveItem` (`self.PlayersAlive`) Player))

(event `self.K2_PostLogin`
  (params (NewPlayer :type "PlayerController Object Reference"))
  (`KismetSystemLibrary.Delay` 0.2)
  (`KismetArrayLibrary.Array_Add` (`self.PCs`) NewPlayer)
  (`self.UpdatePlayersOnSpawns`)
  (bind _asps_custom (cast `/Game/Blueprint/GameFramework/PS_Custom` (`Controller.PlayerState` NewPlayer)))
  (bind _aspc_custom (cast `/Game/Blueprint/GameFramework/PC_Custom` (`PlayerState.GetPlayerController` _asps_custom)))
  (`/Game/Blueprint/GameFramework/PC_Custom.Client_RequestLoadSave` _aspc_custom))

(event `OnSeamlessTravel`
  (`KismetSystemLibrary.Delay` 1.0)
  (for _array_element (`GameStateBase.PlayerArray` (`GameplayStatics.GetGameState`))
    (`KismetArrayLibrary.Array_Add` (`self.PCs`) (`PlayerState.GetPlayerController` _array_element)))
  (`self.UpdatePlayersOnSpawns`))

(event `SpawnUtilities`
  (params (PC :type "PlayerController Object Reference (by ref)")))

(event `StartCountfown`
  (bind _asbp_custom_game_state (cast `/Game/Blueprint/GameFramework/BP_CustomGameState` (`GameplayStatics.GetGameState`)))
  (for _array_element (`GameStateBase.PlayerArray` _asbp_custom_game_state)
    (cast `/Game/Blueprint/GameFramework/PC_Custom` (`PlayerState.GetPlayerController` _array_element))))

(event `StopCountdown`
  (bind _asbp_custom_game_state (cast `/Game/Blueprint/GameFramework/BP_CustomGameState` (`GameplayStatics.GetGameState`)))
  (for _array_element (`GameStateBase.PlayerArray` _asbp_custom_game_state)
    (cast `/Game/Blueprint/GameFramework/PC_Custom` (`PlayerState.GetPlayerController` _array_element))))

(event `self.K2_OnLogout`
  (params (ExitingController :type "Controller Object Reference"))
  (bind _asplayer_controller (cast `PlayerController` ExitingController))
  (`KismetArrayLibrary.Array_RemoveItem` (`self.PCs`) _asplayer_controller)
  (`self.IfSpawnSetUpIsDone`))

(event `BackupInventories`
  (for _array_element (`GameStateBase.PlayerArray` (`GameplayStatics.GetGameState`))
    (bind _asps_custom (cast `/Game/Blueprint/GameFramework/PS_Custom` _array_element))
    (bind _asbp_player_character (cast `/Game/Blueprint/Actors/Player/BP_PlayerCharacter` (`PlayerState.GetPawn` _asps_custom)))
    (set `CustomPlayerState.InventoryItems` (`InventoryComponent.InventorySlots` (`APlayerCharacter.InventoryComponent` _asbp_player_character)) _asps_custom)
    (set `CustomPlayerState.StashItems` (`InventoryComponent.InventorySlots` (`/Game/Blueprint/Actors/Player/BP_PlayerCharacter.StashInventory` _asbp_player_character)) _asps_custom)))

(event `self.OnPreSeamlessTravel`
  (params (PC :type "Controller Object Reference") (PS :type "CustomPlayerState Object Reference") (Players :type Integer))
  (`self.BackupInventories`)
  (`parent.OnPreSeamlessTravel` PC PS Players))

(fn `CheckLobbyReady`
  (returns (`Ready?` :type Boolean))
  (locals (`bAllReady?` :type Boolean))
  (for _array_element (`GameStateBase.PlayerArray` (`GameplayStatics.GetGameState`))
    (bind _asps_custom (cast `/Game/Blueprint/GameFramework/PS_Custom` _array_element))
    (bind _blobbyready (`/Game/Blueprint/GameFramework/PS_Custom.bLobbyReady` _asps_custom))
    (set `local.bAllReady?` _blobbyready)
    (if (not _blobbyready)
      (break)))
  (return (`local.bAllReady?`)))

(fn `HandleSeamlessTravelPlayer`
  (returns (C :type "Controller Object Reference"))
  (`self.OnSeamlessTravel`)
  (return null))

(fn `SetUpSpawnPoints`
  (bind _outactors (`GameplayStatics.GetAllActorsOfClass` "/Game/Blueprint/Actors/Others/BP_SpawnPoints.BP_SpawnPoints_C"))
  (for _index (range (+ (`KismetArrayLibrary.Array_LastIndex` _outactors) 1))
    (bind _outactors_2 (`GameplayStatics.GetAllActorsOfClassWithTag` "/Game/Blueprint/Actors/Others/BP_SpawnPoints.BP_SpawnPoints_C" (`KismetStringLibrary.Conv_StringToName` (`KismetStringLibrary.Conv_IntToString` _index))))
    (`KismetArrayLibrary.Array_Add` (`self.PlayerSpawns`) (`|GetArrayItem` _outactors_2)))
  (set `self.bSpawnSetUpDone` true))

(fn `UpdatePlayersOnSpawns`
  (locals (Loop_PC_AlreadyAdded :type Boolean))
  (for _array_element (`self.PCs`)
    (set `local.Loop_PC_AlreadyAdded` false)
    (for _array_element_2 (`self.PlayerSpawns`)
      (bind _pc (`/Game/Blueprint/Actors/Others/BP_SpawnPoints.PC` _array_element_2))
      (`/Engine/EditorBlueprintResources/StandardMacros.IsValid` _pc
        (:`Is Valid`
          (if (== _pc _array_element)
            (set `local.Loop_PC_AlreadyAdded` true)
            (break)))))
    (`local.Loop_PC_AlreadyAdded`
      (:`then`)
      (:`else`
        (for _array_element_3 (`self.PlayerSpawns`)
          (`/Engine/EditorBlueprintResources/StandardMacros.IsValid` (`/Game/Blueprint/Actors/Others/BP_SpawnPoints.PC` _array_element_3)
            (:`Is Not Valid`
              (`/Game/Blueprint/Actors/Others/BP_SpawnPoints.SpawnCharacter` _array_element_3 _array_element)
              (break)))))))
  (for _array_element_4 (`self.PlayerSpawns`)
    (if (not (`KismetArrayLibrary.Array_Contains` (`self.PCs`) (`/Game/Blueprint/Actors/Others/BP_SpawnPoints.PC` _array_element_4)))
      (`/Game/Blueprint/Actors/Others/BP_SpawnPoints.Clear` _array_element_4))))

(fn `UserConstructionScript`)