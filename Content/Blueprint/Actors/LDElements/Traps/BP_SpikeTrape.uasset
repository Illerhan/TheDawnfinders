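; BP_SpikeTrape is a spike trap that animates spikes vertically and damages players and other actors touching them.
; Activate and Deactivate both call DoTrapAction after a delay, while DoSpikeAnim runs a guarded timeline whose authority-side updates set spike height.
; Alongside the timeline, a delayed, brief collider window opens with a Wwise sound.
; Player damage is sent by the locally controlled client, other damage by the authority.
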(event `self.ReceiveBeginPlay`
  (`parent.ReceiveBeginPlay`)
  (set `self.Spikes` (`|MakeArray` (`self.SM_Traps_Spike_4x4_02`)))
  (for _array_element (`|MakeArray` (`self.SM_Traps_Spike_4x4_02`) :!type "MeshComponent Object Reference")
    (for (_array_element_2 _array_index) (`MeshComponent.GetMaterials` _array_element)
      (bind _returnvalue (`KismetMaterialLibrary.CreateDynamicMaterialInstance` _array_element_2))
      (`KismetArrayLibrary.Array_Add` (`self.Materials`) _returnvalue)
      (`MaterialInstanceDynamic.SetScalarParameterValue` _returnvalue "Opacity" 0.0)
      (`PrimitiveComponent.SetMaterial` _array_element _array_index _returnvalue)
      (`self.DoTrapAction` null))))

(event `self.Deactivate`
  (`KismetSystemLibrary.Delay` (`self.DelayAfterActivation`) :!label _label)
  (`self.DoTrapAction` null))

(event `self.Activate`
  (goto _label))

(event `self.DoSpikeAnim`
  (if (not (`self.IsDoingAnim`))
    (set `self.IsDoingAnim` true)
    (`|ExecutionSequence`
      (:`then_0`
        (bind (_direction _newtrack_0) (`Timeline|SpikeYTimeline` :!via `PlayFromStart`)
          (:`Update`
            (`/Engine/EditorBlueprintResources/ActorMacros.Switch Has Authority`
              (:`Authority`
                (`self.SetSpikeAnimValue` _newtrack_0)
                (`self.ApplySpikePosition` _newtrack_0))))
          (:`Finished`
            (set `self.IsDoingAnim` false))))
      (:`then_1`
        (`KismetSystemLibrary.Delay` 0.6)
        (`PrimitiveComponent.SetCollisionEnabled` (`self.SpikesOutCollider`) "QueryOnly")
        (`self.Multi_SpikeSound`)
        (`KismetSystemLibrary.Delay` 0.5)
        (`PrimitiveComponent.SetCollisionEnabled` (`self.SpikesOutCollider`) "NoCollision")))))

(event `self.ApplySpikePosition`
  (params (Value :type "Float (single-precision)"))
  (for _array_element (`self.Spikes`)
    (`SceneComponent.K2_SetRelativeLocation` _array_element (`KismetMathLibrary.MakeVector` (.x (`SceneComponent.RelativeLocation` _array_element)) (.y (`SceneComponent.RelativeLocation` _array_element)) (+ (* Value 100.0) -120.0)) false false)))

(event `Multi_SpikeSound`
  (`AkGameplayStatics.PostEvent` "/Game/WwiseAudio/Events/Default_Work_Unit/Objets/Elements_de_LD/Trap/Play_Trap_Spike.Play_Trap_Spike" self))

(event `self.SpikesOutCollider.OnComponentBeginOverlap`
  (params (OverlappedComponent :type "PrimitiveComponent Object Reference") (OtherActor :type "Actor Object Reference") (OtherComp :type "PrimitiveComponent Object Reference") (OtherBodyIndex :type Integer) (bFromSweep :type Boolean) (SweepResult :type "HitResult Structure (by ref)"))
  (if (`self.ActorHasTag` OtherActor "Player")
    (bind _ascharacter (cast `Character` OtherActor))
    (if (`Pawn.IsLocallyControlled` _ascharacter)
      (message `Damageable.ReceiveDamage` OtherActor (`KismetMathLibrary.Conv_IntToDouble` (`self.Damages`)) null))
    (elif (`self.HasAuthority`)
      (message `Damageable.ReceiveDamage` OtherActor (`KismetMathLibrary.Conv_IntToDouble` (`self.DamagesEnemies`)) null))))

(fn `IsActive`
  (returns (ReturnValue :type Boolean))
  (return false))

(fn `UserConstructionScript`)