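; BP_SwingBlade is a swinging blade trap actor with a blade mesh and a chain mesh.
; On BeginPlay, after the parent's logic, it creates a dynamic material instance for every material slot on both meshes.
; Each instance is stored in a Materials array and starts with zero Opacity, so any swinging or fade-in logic lies outside this graph.
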(event `self.ReceiveBeginPlay`
  (`parent.ReceiveBeginPlay`)
  (for _array_element (`|MakeArray` (`self.BladeMesh`) (`self.ChainMesh`) :!type "MeshComponent Object Reference")
    (for (_array_element_2 _array_index) (`MeshComponent.GetMaterials` _array_element)
      (bind _returnvalue (`KismetMaterialLibrary.CreateDynamicMaterialInstance` _array_element_2))
      (`KismetArrayLibrary.Array_Add` (`self.Materials`) _returnvalue)
      (`MaterialInstanceDynamic.SetScalarParameterValue` _returnvalue "Opacity" 0.0)
      (`PrimitiveComponent.SetMaterial` _array_element _array_index _returnvalue))))

(fn `UserConstructionScript`)