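; Actor that plays ambient environmental audio around the local player through Wwise.
; On BeginPlay it stores the first local player controller, starts a loud wind event on it and seeds a random delay.
; Tick counts the delay down, then posts one of four random one-shots, such as crackle or eerie whistle, at a random horizontal offset from the controller's location and re-rolls the delay.
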(event `self.ReceiveBeginPlay`
  (bind _returnvalue (`GameplayStatics.GetPlayerController` 0))
  (bind (_minmaxdelay_x _minmaxdelay_y) (`KismetMathLibrary.BreakVector` (`self.MinMaxDelay`)))
  (if (`Controller.IsLocalController` _returnvalue)
    (bind _output_get (set `self.Player` _returnvalue))
    (set `self.Timer` (`KismetMathLibrary.RandomFloatInRange` _minmaxdelay_x _minmaxdelay_y))
    (`AkGameplayStatics.PostEvent` "/Game/WwiseAudio/Events/Default_Work_Unit/Ambiance/Play_AMB_LoudWind.Play_AMB_LoudWind" _output_get)))

(event `self.ReceiveTick`
  (params (DeltaSeconds :type "Float (single-precision)"))
  (bind (_minmaxdelay_x _minmaxdelay_y) (`KismetMathLibrary.BreakVector` (`self.MinMaxDelay`)))
  (bind _output_get (set `self.Timer` (- (`self.Timer`) DeltaSeconds)))
  (if (<= _output_get 0.0)
    (`self.Play Random Sound`)
    (set `self.Timer` (`KismetMathLibrary.RandomFloatInRange` _minmaxdelay_x _minmaxdelay_y))))

(event `Play Random Sound`
  (bind _maxsoundrange (`self.MaxSoundRange`))
  (bind (_returnvalue_x _returnvalue_y _returnvalue_z) (`KismetMathLibrary.BreakVector` (`self.K2_GetActorLocation` (`self.Player`))))
  (bind _returnvalue (`KismetMathLibrary.RandomFloatInRange` (- 0.0 _maxsoundrange) _maxsoundrange))
  (`AkGameplayStatics.PostEventAtLocation` (select `int` (`KismetMathLibrary.RandomIntegerInRange` 0 3) :`0` "/Game/WwiseAudio/Events/Default_Work_Unit/Ambiance/Play_AMB_Crackle.Play_AMB_Crackle" :`1` "/Game/WwiseAudio/Events/Default_Work_Unit/Ambiance/Play_AMB_Sandfall.Play_AMB_Sandfall" :`2` "/Game/WwiseAudio/Events/Default_Work_Unit/Ambiance/Play_AMB_EerieWhistle.Play_AMB_EerieWhistle" :`3` "/Game/WwiseAudio/Events/Default_Work_Unit/Ambiance/Play_AMB_Hallucination.Play_AMB_Hallucination" :!type "AkAudioEvent Object Reference") (`KismetMathLibrary.MakeVector` (+ _returnvalue_x _returnvalue) (+ _returnvalue _returnvalue_y) _returnvalue_z)))

(fn `UserConstructionScript`)