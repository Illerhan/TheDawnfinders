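; BP_Shoot is a gamepad-driven weapon child actor that loads its "Revolver" stats from a data table.
; Holding aim narrows a debug-drawn cone, at a modified rate while the parent moves.
; Firing line-traces random shots within that cone, destroys specific enemies and columns, and briefly raises BP_Noise.
; Tick timers handle shot delay and interruptible auto-reload, while a face button deals short-range damage to columns.
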(event `Set up Data`
  (bind _returnvalue (`|GetDataTableRow` (`self.Data Table`) "Revolver")
    (:`then`
      (bind (_maxangle _minangle _aimingspeed _maxammos _reloadtime _noise _numberofshots _maxrange _speedmodifier) (break `/Game/NewWeapons` _returnvalue))
      (set `self.MaxAngle` _maxangle)
      (set `self.MinAngle` _minangle)
      (set `self.AimingSpeed` _aimingspeed)
      (set `self.MaxAmmosInWeapon` _maxammos)
      (set `self.ReloadTime` _reloadtime)
      (set `self.Noise` _noise)
      (set `self.NumberOfShots` _numberofshots)
      (set `self.MaxRange` _maxrange)
      (set `self.SpeedModifierWhenMoving` _speedmodifier))))

(event `Key|Gamepad_RightTrigger`
  (params (Key :type "Key Structure"))
  (:`Pressed`
    (`self.Shoot`)))

(event `Key|Gamepad_LeftTrigger`
  (params (Key :type "Key Structure"))
  (:`Pressed`
    (set `self.isAiming` true))
  (:`Released`
    (set `self.isAiming` false)
    (set `self.CurrentAngle` (`self.MaxAngle`))))

(event `self.ReceiveBeginPlay`
  (bind _returnvalue (`KismetMathLibrary.Clamp` (`self.MaxAmmosInWeapon`) 0 (`self.TotalAmmos`)))
  (`self.Set up Data`)
  (set `self.CurrentAngle` (`self.MaxAngle`))
  (set `self.CurrentAmmos` _returnvalue)
  (`KismetSystemLibrary.PrintString` (`KismetStringLibrary.Concat_StrStr` "Loaded " (`KismetStringLibrary.Conv_IntToString` _returnvalue) " ammos") true true (struct :`G` 0.66 :`B` 1.0 :`A` 1.0) 2.0 "1")
  (set `self.TotalAmmos` (- (`self.TotalAmmos`) _returnvalue))
  (set `self.WaitingReloadTimer` (`self.WaitingBeforeReload`))
  (set `self.ReloadTimer` (`self.ReloadTime`)))

(event `self.ReceiveTick`
  (params (DeltaSeconds :type "Float (single-precision)"))
  (bind _returnvalue (`self.K2_GetActorLocation`))
  (bind _returnvalue_2 (`self.GetActorForwardVector`))
  (bind _returnvalue_3 (* _returnvalue_2 (`self.MaxRange`)))
  (bind _returnvalue_4 (+ _returnvalue (* _returnvalue_2 100.0)))
  (`self.Shot Delay` DeltaSeconds)
  (`self.Reload Timer` DeltaSeconds)
  (`self.WaitForReload` DeltaSeconds)
  (if (`self.isAiming`)
    (`self.PreciseAim` DeltaSeconds)
    (`KismetSystemLibrary.LineTraceSingle` :`Start` _returnvalue_4 :`End` (+ _returnvalue (`KismetMathLibrary.RotateAngleAxis` _returnvalue_3 (`self.CurrentAngle`) (0.0 0.0 1.0))) :`TraceChannel` "TraceTypeQuery4" :`DrawDebugType` "ForDuration" :`TraceColor` (struct :`R` 1.0 :`G` 1.0 :`B` 1.0 :`A` 1.0) :`TraceHitColor` (struct :`R` 1.0 :`G` 1.0 :`B` 1.0 :`A` 1.0) :`DrawTime` 0.0)
    (`KismetSystemLibrary.LineTraceSingle` :`Start` _returnvalue_4 :`End` (+ _returnvalue (`KismetMathLibrary.RotateAngleAxis` _returnvalue_3 (- 0.0 (`self.CurrentAngle`)) (0.0 0.0 1.0))) :`TraceChannel` "TraceTypeQuery1" :`DrawDebugType` "ForDuration" :`TraceColor` (struct :`R` 1.0 :`G` 1.0 :`B` 1.0 :`A` 1.0) :`TraceHitColor` (struct :`R` 1.0 :`G` 1.0 :`B` 1.0 :`A` 1.0) :`DrawTime` 0.0)))

(event `Reload Timer`
  (params (DeltaTime :type "Float (double-precision)"))
  (if (and (and (< (`self.CurrentAmmos`) (`self.MaxAmmosInWeapon`)) (not (`self.isReloading`))) (> (`self.TotalAmmos`) 0))
    (bind _output_get (set `self.WaitingReloadTimer` (- (`self.WaitingReloadTimer`) DeltaTime)))
    (if (<= _output_get 0.0)
      (`self.Reload`))))

(event `Shot Delay`
  (params (DeltaTime :type "Float (double-precision)"))
  (set `self.DelayBetweenShotsTimer` (- (`self.DelayBetweenShotsTimer`) DeltaTime)))

(event `Reload`
  (`KismetSystemLibrary.PrintString` "RELOADING" true true (struct :`G` 0.66 :`B` 1.0 :`A` 1.0) 2.0 "4")
  (set `self.isReloading` true))

(event `WaitForReload`
  (params (DeltaTime :type "Float (double-precision)"))
  (if (`self.isReloading`)
    (bind _output_get (set `self.ReloadTimer` (- (`self.ReloadTimer`) DeltaTime)))
    (if (<= _output_get 0.0)
      (`KismetSystemLibrary.PrintString` "Reloading now")
      (bind _output_get_2 (set `self.BulletsToLoad` (`KismetMathLibrary.Clamp` (- (`self.MaxAmmosInWeapon`) (`self.CurrentAmmos`)) 0 (`self.TotalAmmos`))))
      (bind _output_get_3 (set `self.CurrentAmmos` (+ (`self.CurrentAmmos`) _output_get_2)))
      (bind _output_get_4 (set `self.TotalAmmos` (- (`self.TotalAmmos`) _output_get_2)))
      (set `self.isReloading` false)
      (set `self.WaitingReloadTimer` (`self.WaitingBeforeReload`))
      (`KismetSystemLibrary.PrintString` (`KismetStringLibrary.Concat_StrStr` "Current Ammos : " (`KismetStringLibrary.Conv_IntToString` _output_get_3) " / Ammos left : " (`KismetStringLibrary.Conv_IntToString` _output_get_4))))))

(event `PreciseAim`
  (params (DeltaTime :type "Float (double-precision)"))
  (set `self.CurrentAngle` (`KismetMathLibrary.FClamp` (- (`self.CurrentAngle`) (* (* DeltaTime (`self.AimingSpeed`)) (select `bool` (<= (`KismetMathLibrary.VSize` (`self.GetVelocity` (`self.GetParentActor`))) 1.0) :`false` (`self.SpeedModifierWhenMoving`) :`true` 1.0))) (`self.MinAngle`) (`self.MaxAngle`))))

(event `Shoot`
  (bind _returnvalue (`self.GetActorForwardVector`))
  (bind _currentangle (`self.CurrentAngle`))
  (bind _returnvalue_2 (+ (`self.K2_GetActorLocation`) (* _returnvalue 100.0)))
  (bind _hasammos (`self.CheckForAmmos`))
  (if _hasammos
    (if (<= (`self.DelayBetweenShotsTimer`) 0.0)
      (for _ (range 1 (+ (`self.NumberOfShots`) 1))
        (bind _outhit (`KismetSystemLibrary.LineTraceSingle` :`Start` _returnvalue_2 :`End` (+ _returnvalue_2 (`KismetMathLibrary.RotateAngleAxis` (* _returnvalue (`self.MaxRange`)) (`KismetMathLibrary.RandomFloatInRange` (- 0.0 _currentangle) _currentangle) (0.0 0.0 1.0))) :`TraceChannel` "TraceTypeQuery1" :`DrawDebugType` "ForDuration" :`TraceColor` (struct :`G` 0.32145 :`B` 1.0 :`A` 1.0) :`TraceHitColor` (struct :`G` 1.0 :`B` 0.810155 :`A` 1.0) :`DrawTime` 1.0))
        (`self.CheckForHit` (`.HitActor` (`GameplayStatics.BreakHitResult` _outhit))))
      (`self.Make Noise`)
      (set `self.CurrentAngle` (`self.MaxAngle`))
      (set `self.DelayBetweenShotsTimer` (`self.DelayBetweenShots`))
      (bind _result (`/Engine/EditorBlueprintResources/StandardMacros.DecrementInt` (`self.CurrentAmmos`))
        (:`  `
          (`KismetSystemLibrary.PrintString` (`KismetStringLibrary.Concat_StrStr` "Ammos left in chamber : " (`KismetStringLibrary.Conv_IntToString` _result)) true true (struct :`G` 0.66 :`B` 1.0 :`A` 1.0) 2.0 "2")
          (set `self.WaitingReloadTimer` (`self.WaitingBeforeReload`))
          (set `self.isReloading` false)
          (set `self.ReloadTimer` (`self.ReloadTime`))
          (if (<= (`self.CurrentAmmos`) 0)
            (set `self.isReloading` true)
            (`KismetSystemLibrary.PrintString` "RELOADING" true true (struct :`G` 0.66 :`B` 1.0 :`A` 1.0) 2.0 "4")))))
    (else
      (`KismetSystemLibrary.PrintString` "Out of Ammo"))))

(event `CheckForHit`
  (params (HitActor :type "Actor Object Reference"))
  (bind _asbp_new_enemy_01 (cast `/Game/Blueprint/Actors/Enemies/BP_NewEnemy_01` HitActor)
    (:`then`
      (`self.K2_DestroyActor` _asbp_new_enemy_01))
    (:`CastFailed`
      (bind _asbp_new_crystallized_02 (cast `/Game/Blueprint/Actors/Enemies/BP_NewCrystallized_02` HitActor)
        (:`then`
          (`self.K2_DestroyActor` _asbp_new_crystallized_02))
        (:`CastFailed`
          (bind _asbp_destructible_column (cast `/Game/Blueprint/Actors/BP_DestructibleColumn` HitActor))
          (`/Game/Blueprint/Actors/BP_DestructibleColumn.Destroy` _asbp_destructible_column))))))

(event `Make Noise`
  (bind _returnvalue (`GameplayStatics.GetActorOfClass` "/Game/Blueprint/Actors/BP_Noise.BP_Noise_C"))
  (set `/Game/Blueprint/Actors/BP_Noise.NoiseLocalAdder` (`self.Noise`) _returnvalue)
  (`KismetSystemLibrary.Delay` 0.4)
  (set `/Game/Blueprint/Actors/BP_Noise.NoiseLocalAdder` 0.0 _returnvalue))

(event `Key|Gamepad_FaceButton_Left`
  (params (Key :type "Key Structure"))
  (bind _returnvalue (`self.K2_GetActorLocation`))
  (bind _returnvalue_2 (`self.GetActorForwardVector`))
  (:`Pressed`
    (bind _outhit (`KismetSystemLibrary.LineTraceSingle` :`Start` (+ _returnvalue (* _returnvalue_2 100.0)) :`End` (+ _returnvalue (* _returnvalue_2 150.0)) :`TraceChannel` "TraceTypeQuery1" :`DrawDebugType` "ForDuration" :`DrawTime` 0.5))
    (bind _asbp_destructible_column (cast `/Game/Blueprint/Actors/BP_DestructibleColumn` (`.HitActor` (`GameplayStatics.BreakHitResult` _outhit))))
    (`/Game/Blueprint/Actors/BP_DestructibleColumn.TakeDamage` _asbp_destructible_column)))

(fn `CheckForAmmos`
  (returns (HasAmmos :type Boolean))
  (return (> (`self.CurrentAmmos`) 0)))

(fn `UserConstructionScript`)