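; AC_Item is an actor component that draws weapon aim and shot feedback lines for its owning Pawn.
; On BeginPlay it spawns two BP_AimLine actors, hidden at start, and one BP_ShootLine.
; ActualiseAimLines places the aim lines symmetrically around the owner's forward vector, rotated about Z by the current aim angle, out to the weapon's max range.
; DoShootFeedbacks positions the shoot line along a given direction at that range.
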(event `self.ReceiveBeginPlay`
  (`parent.ReceiveBeginPlay`)
  (bind _aspawn (cast `Pawn` (`self.GetOwner`)))
  (bind _returnvalue (`|SpawnActorFromClass` "/Game/Blueprint/Actors/Player/BP_AimLine.BP_AimLine_C" (`GeometryScriptLibrary_TransformFunctions.MakeTransformFromAxes` (0.0 0.0 0.0)) "Undefined" "MultiplyWithRoot" null _aspawn))
  (set `self.AimLineLeft` _returnvalue)
  (bind _returnvalue_2 (`|SpawnActorFromClass` "/Game/Blueprint/Actors/Player/BP_AimLine.BP_AimLine_C" (`KismetMathLibrary.MakeTransform` (0.0 0.0 0.0)) "Undefined" "MultiplyWithRoot" null _aspawn))
  (set `self.AimLineRight` _returnvalue_2)
  (`/Game/Blueprint/Actors/Player/BP_AimLine.Hide` (`self.AimLineLeft`))
  (`/Game/Blueprint/Actors/Player/BP_AimLine.Hide` (`self.AimLineRight`))
  (bind _returnvalue_3 (`|SpawnActorFromClass` "/Game/Blueprint/Actors/Player/BP_ShootLine.BP_ShootLine_C" (`KismetMathLibrary.MakeTransform` (0.0 0.0 0.0)) "Undefined" "MultiplyWithRoot" null _aspawn))
  (set `self.ShootLine` _returnvalue_3))

(event `self.ActualiseAimLines`
  (bind _returnvalue (`self.GetOwner`))
  (bind ((`MaxAngle` _maxangle) (`MinAngle` _minangle) (`AimingSpeed` _aimingspeed) (`MagazineSize` _magazinesize) (`ReloadDuration` _reloadduration) (`NoiseRange` _noiserange) (`NumberOfShots` _numberofshots) (`MaxRange` _maxrange)) (break `WeaponInfos` (`self.CurrentWeaponData`)))
  (`/Game/Blueprint/Actors/Player/BP_AimLine.SetPosition` (`self.AimLineLeft`) _returnvalue (`KismetMathLibrary.Normal` (`KismetMathLibrary.RotateAngleAxis` (`Actor.GetActorForwardVector` (`self.GetOwner`)) (`self.AimCurrentAngle`) (0.0 0.0 1.0))) _maxrange)
  (`/Game/Blueprint/Actors/Player/BP_AimLine.SetPosition` (`self.AimLineRight`) _returnvalue (`KismetMathLibrary.Normal` (`KismetMathLibrary.RotateAngleAxis` (`Actor.GetActorForwardVector` (`self.GetOwner`)) (* (`self.AimCurrentAngle`) -1.0) (0.0 0.0 1.0))) _maxrange))

(event `self.DoShootFeedbacks`
  (params (Direction :type "Vector Structure"))
  (`/Game/Blueprint/Actors/Player/BP_ShootLine.SetPosition` (`self.ShootLine`) (`self.GetOwner`) Direction (`.MaxRange` (break `WeaponInfos` (`self.CurrentWeaponData`)))))

(event `self.HideAimLines`
  (`/Game/Blueprint/Actors/Player/BP_AimLine.Hide` (`self.AimLineLeft`))
  (`/Game/Blueprint/Actors/Player/BP_AimLine.Hide` (`self.AimLineRight`)))