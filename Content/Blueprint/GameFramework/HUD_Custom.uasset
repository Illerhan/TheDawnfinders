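; HUD_Custom is a custom HUD that owns the player's main widget and feeds player states into its squad display.
; AddMainwidget creates WBP_MainWidget for the owning controller and adds it to the viewport, unless the stored one is already showing.
; AddPlayerState forwards a player state to that widget's WBPSquad for binding.
; BeginPlay is empty, and AddLobbyWidget only checks authority, with its widget creation left disconnected.
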(event `self.ReceiveBeginPlay`)

(fn `AddLobbyWidget`
  (if (`self.HasAuthority` (`self.GetOwningPlayerController`))
    _))

(fn `AddMainwidget`
  (bind _mainwidgetref (`self.MainWidgetRef`))
  (`/Engine/EditorBlueprintResources/StandardMacros.IsValid` _mainwidgetref
    (:`Is Valid`
      (if (not (`Widget.IsInViewport` _mainwidgetref))
        (bind _returnvalue (`|CreateWidget` "/Game/UI/Widgets/WBP_MainWidget.WBP_MainWidget_C" (`self.GetOwningPlayerController`) :!label _label))
        (bind _output_get (set `self.MainWidgetRef` _returnvalue))
        (bind _output_get_2 (set `self.MainWidget` _output_get))
        (`UserWidget.AddToViewport` _output_get_2 0)))
    (:`Is Not Valid`
      (goto _label))))

(fn `AddPlayerState`
  (params (PS :type "PlayerState Object Reference"))
  (`SquadWidget.BindNewPlayerState` (`/Game/UI/Widgets/WBP_MainWidget.WBP_Squad` (`self.MainWidgetRef`)) PS))

(fn `UserConstructionScript`)