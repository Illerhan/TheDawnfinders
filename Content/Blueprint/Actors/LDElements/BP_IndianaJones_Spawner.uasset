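; Overlap trigger that releases an Indiana Jones-style rolling boulder already placed in the level, despite the Spawner name.
; Any actor overlap unhides the referenced IndianaBall, enables its sphere collision and pushes it with a configurable force direction and strength.
; It also calls the ball's DestroyBall and posts the Wwise boulder-roll sound.
; After a short delay it sets the ball's HasStarted flag and destroys itself.
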(event `self.ReceiveActorBeginOverlap`
  (params (OtherActor :type "Actor Object Reference"))
  (bind _indianaball (`self.IndianaBall`))
  (`self.SetActorHiddenInGame` (`self.IndianaBall`) false)
  (`PrimitiveComponent.SetCollisionEnabled` (`/Game/Blueprint/Actors/LDElements/BP_IndianaJones_Ball.Sphere` (`self.IndianaBall`)) "QueryAndPhysics")
  (`PrimitiveComponent.AddForce` (`/Game/Blueprint/Actors/LDElements/BP_IndianaJones_Ball.Sphere` (`self.IndianaBall`)) (* (`self.ForceDirection`) (`self.ForceStrength`)) "None" false)
  (`/Game/Blueprint/Actors/LDElements/BP_IndianaJones_Ball.DestroyBall` _indianaball)
  (`AkGameObject.PostAkEvent` :`self` (`/Game/Blueprint/Actors/LDElements/BP_IndianaJones_Ball.Sound` _indianaball) :`AkEvent` "/Game/WwiseAudio/Events/Default_Work_Unit/Objets/Elements_de_LD/Boulder/Play_BoulderRoll.Play_BoulderRoll")
  (`KismetSystemLibrary.Delay` 0.5)
  (set `/Game/Blueprint/Actors/LDElements/BP_IndianaJones_Ball.hasStarted` true _indianaball)
  (`self.K2_DestroyActor`))

(fn `UserConstructionScript`)