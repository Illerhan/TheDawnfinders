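; BP_NoiseMaker is an interactible level element that makes a short burst of noise when a player interacts with it.
; On authority, each interaction finds the level's BP_Noise actor and raises its NoiseLocalAdder briefly, then resets it to zero after a short delay.
; It counts interactions and destroys itself once the required number is reached.
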(event `self.BP_OnInteraction`
  (params (Player :type "APlayerCharacter Object Reference"))
  (if (`self.HasAuthority` Player)
    (set `self.InteractionDone` (+ (`self.InteractionDone`) 1))
    (bind _returnvalue (`GameplayStatics.GetActorOfClass` "/Game/Blueprint/Actors/BP_Noise.BP_Noise_C"))
    (set `/Game/Blueprint/Actors/BP_Noise.NoiseLocalAdder` 10.0 _returnvalue)
    (`KismetSystemLibrary.Delay` 0.4)
    (set `/Game/Blueprint/Actors/BP_Noise.NoiseLocalAdder` 0.0 _returnvalue)
    (if (>= (`self.InteractionDone`) (`self.InteractionNeeded`))
      (`self.K2_DestroyActor`))))

(fn `UserConstructionScript`)