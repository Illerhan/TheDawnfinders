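; BP_ShootLine is a reusable shot tracer actor that flashes a line and an optional muzzle light along a firing direction.
; SetPosition centers the actor between the raised origin and range end, yaws it toward the origin, stretches Line to the range, and moves SpotLight to the origin.
; A next-tick loop counts down ShootEffectTimer, thinning the line and dimming the light, then hides both.
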(event `Show`
  (`SceneComponent.SetVisibility` (`self.Line`) true false))

(event `Hide`
  (`SceneComponent.SetVisibility` (`self.Line`) false false)
  (`LightComponent.SetIntensity` (`self.SpotLight`) 0.0))

(event `SetPosition`
  (params (Origin :type "Actor Object Reference") (Direction :type "Vector Structure") (Range :type "Float (double-precision)") (DoLight :type Boolean))
  (bind _line (`self.Line`))
  (bind _shooteffecttimer (`self.ShootEffectTimer`))
  (bind _returnvalue (+ (`self.K2_GetActorLocation` Origin) (0.0 0.0 50.0)))
  (bind _returnvalue_2 (* _shooteffecttimer 0.2))
  (`self.Show`)
  (`self.K2_SetActorLocation` (+ _returnvalue (* Direction (* Range 0.5))))
  (`self.K2_SetActorRotation` (`KismetMathLibrary.MakeRotator` 0.0 0.0 (`KismetMathLibrary.DegAtan2` (.y (- _returnvalue (`self.K2_GetActorLocation`))) (.x (- _returnvalue (`self.K2_GetActorLocation`))))))
  (`SceneComponent.K2_SetWorldLocation` (`self.SpotLight`) _returnvalue false false)
  (`SceneComponent.SetWorldScale3D` (`self.Line`) (`KismetMathLibrary.MakeVector` 0.1 0.1 (* Range 0.01)))
  (set `self.ShootEffectTimer` 0.8)
  (`SceneComponent.SetWorldScale3D` _line (`KismetMathLibrary.MakeVector` _returnvalue_2 _returnvalue_2 (.z (`SceneComponent.K2_GetComponentScale` _line))) :!label _label)
  (if DoLight
    (`LightComponent.SetIntensity` (`self.SpotLight`) (`KismetMathLibrary.Lerp` 0.0 3000.0 _shooteffecttimer)))
  (bind _output_get (set `self.ShootEffectTimer` (- (`self.ShootEffectTimer`) (* (`GameplayStatics.GetWorldDeltaSeconds`) 5.0))))
  (if (<= _output_get 0.0)
    (`KismetSystemLibrary.K2_ClearAndInvalidateTimerHandle` (`self.Timer Handle`))
    (`self.Hide`)
    (else
      (`KismetSystemLibrary.DelayUntilNextTick`)
      (goto _label))))

(fn `UserConstructionScript`)