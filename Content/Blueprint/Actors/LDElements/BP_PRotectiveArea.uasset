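; BP_PRotectiveArea is a level element that marks players as protected while they overlap its area, feeding the game's extraction check.
; Begin and end overlap toggle IsProtected on the player state, then run the check directly on authority or through a server event on remotes.
; The check loops all player characters, setting the game mode's AllSafe false if any living player is unprotected, then calls CheckExtraction.
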(event `Server_CheckProtectedPlayers`
  (bind _returnvalue (`GameplayStatics.GetGameMode`))
  (bind _outactors (`GameplayStatics.GetAllActorsOfClass` "/Game/Blueprint/Actors/Player/BP_PlayerCharacter.BP_PlayerCharacter_C" :!label _label))
  (for _array_element _outactors
    (bind _asps_custom (cast `/Game/Blueprint/GameFramework/PS_Custom` (`Pawn.PlayerState` _array_element)))
    (if (or (`CustomPlayerState.bIsProtected` _asps_custom) (`HealthComponent.bIsDead` (`APlayerCharacter.HealthComponent` _array_element)))
      (bind _asbp_custom_game_mode (cast `/Game/Blueprint/GameFramework/BP_CustomGameMode` _returnvalue))
      (set `/Game/Blueprint/GameFramework/BP_CustomGameMode.bAllSafe` true _asbp_custom_game_mode)
      (else
        (bind _asbp_custom_game_mode_2 (cast `/Game/Blueprint/GameFramework/BP_CustomGameMode` _returnvalue))
        (set `/Game/Blueprint/GameFramework/BP_CustomGameMode.bAllSafe` false _asbp_custom_game_mode_2)
        (break))))
  (bind _asbp_custom_game_mode_3 (cast `/Game/Blueprint/GameFramework/BP_CustomGameMode` (`GameplayStatics.GetGameMode`)))
  (`/Game/Blueprint/GameFramework/BP_CustomGameMode.CheckExtraction` _asbp_custom_game_mode_3))

(event `self.ProtectedArea.OnComponentBeginOverlap`
  (params (OverlappedComponent :type "PrimitiveComponent Object Reference") (OtherActor :type "Actor Object Reference") (OtherComp :type "PrimitiveComponent Object Reference") (OtherBodyIndex :type Integer) (bFromSweep :type Boolean) (SweepResult :type "HitResult Structure (by ref)"))
  (bind _asbp_player_character (cast `/Game/Blueprint/Actors/Player/BP_PlayerCharacter` OtherActor))
  (bind _ascustom_player_state (cast `CustomPlayerState` (`Pawn.PlayerState` _asbp_player_character)))
  (set `CustomPlayerState.bIsProtected` true _ascustom_player_state)
  (`/Engine/EditorBlueprintResources/ActorMacros.Switch Has Authority` :!label _label_2
    (:`Authority`
      (goto _label))
    (:`Remote`
      (`self.Server_CheckProtectedPlayers`))))

(event `self.ProtectedArea.OnComponentEndOverlap`
  (params (OverlappedComponent :type "PrimitiveComponent Object Reference") (OtherActor :type "Actor Object Reference") (OtherComp :type "PrimitiveComponent Object Reference") (OtherBodyIndex :type Integer))
  (bind _asbp_player_character (cast `/Game/Blueprint/Actors/Player/BP_PlayerCharacter` OtherActor))
  (bind _ascustom_player_state (cast `CustomPlayerState` (`Pawn.PlayerState` _asbp_player_character)))
  (set `CustomPlayerState.bIsProtected` false _ascustom_player_state)
  (goto _label_2))

(fn `UserConstructionScript`)