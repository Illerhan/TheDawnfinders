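; BP_CurseWall is a curse wall actor that dissolves away and destroys itself in response to the palanquin light event.
; On BeginPlay it creates a dynamic material on the CurseWall component and resets its dissolve parameter.
; PalanquinLighton fires only once, playing a timeline that animates the dissolve from start to end, then destroys the actor when finished.
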(event `self.ReceiveBeginPlay`
  (bind _returnvalue (`PrimitiveComponent.CreateDynamicMaterialInstance` (`self.CurseWall`) 0 null "None"))
  (bind _output_get (set `self.Mat` _returnvalue))
  (`MaterialInstanceDynamic.SetScalarParameterValue` _output_get "DissolveAmmount" -1.0))

(event `/Game/Blueprint/Actors/Others/IFogOfWar.Palanquin Light On`
  (if (not (`self.IsActivated`))
    (set `self.IsActivated` true)
    (bind (_direction _alpha) (`Timeline|Timeline` :!via `PlayFromStart`)
      (:`Update`
        (`MaterialInstanceDynamic.SetScalarParameterValue` (`self.Mat`) "DissolveAmmount" (`KismetMathLibrary.Lerp` -1.0 1.0 _alpha)))
      (:`Finished`
        (`self.K2_DestroyActor`)))))

(fn `UserConstructionScript`)