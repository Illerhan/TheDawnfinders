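; BP_Noise is an attachable actor that represents how much noise its parent actor makes while moving.
; Each tick it scales the NoiseRange component by the parent's speed times a general multiplier and a local modifier.
; NoiseRange overlaps all channels only when that scale exceeds one, and ignores them otherwise.
; PreviousVelocity is zeroed every tick and never read here.
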(event `self.ReceiveTick`
  (params (DeltaSeconds :type "Float (single-precision)"))
  (bind _noiserange (`self.NoiseRange`))
  (bind _returnvalue (* (* (/ (`KismetMathLibrary.VSize` (`self.GetVelocity` (`self.GetAttachParentActor`))) 100.0) (`self.NoiseMultiply`)) (`self.NoiseLocalModifier`)))
  (`SceneComponent.SetWorldScale3D` (`self.NoiseRange`) (`KismetMathLibrary.Conv_DoubleToVector` _returnvalue))
  (if (<= _returnvalue 1.0)
    (`PrimitiveComponent.SetCollisionResponseToAllChannels` _noiserange "ECR_Ignore")
    (else
      (`PrimitiveComponent.SetCollisionResponseToAllChannels` _noiserange "ECR_Overlap")))
  (set `self.PreviousVelocity` (0.0 0.0 0.0)))

(fn `UserConstructionScript`)