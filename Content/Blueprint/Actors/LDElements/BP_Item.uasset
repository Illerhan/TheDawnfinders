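; BP_Item is a world item actor that shows a details widget and a rarity effect chosen from its item data.
; On BeginPlay it makes dynamic materials for the mesh and hides them with zero opacity.
; Fadein and FadeOut count fog-of-war areas, driving an opacity Timeline forward for the first and backward after the last.
; The interact collider shows or hides the details widget only for the locally controlled player.
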(event `self.ReceiveBeginPlay`
  (`parent.ReceiveBeginPlay`)
  (bind _aswbp_world_details (cast `/Game/UI/Widgets/WBP_WorldDetails` (`WidgetComponent.GetWidget` (`self.DetailsWidget`))))
  (set `self.WBP_WorldDetails` _aswbp_world_details)
  (for (_array_element _array_index) (`MeshComponent.GetMaterials` (`self.ItemMesh`))
    (bind _returnvalue (`KismetMaterialLibrary.CreateDynamicMaterialInstance` _array_element))
    (`KismetArrayLibrary.Array_Add` (`self.Materials`) _returnvalue)
    (`MaterialInstanceDynamic.SetScalarParameterValue` _returnvalue "Opacity" 0.0)
    (`PrimitiveComponent.SetMaterial` (`self.ItemMesh`) _array_index _returnvalue)))

(event `self.FadeIn`
  (bind _result (`/Engine/EditorBlueprintResources/StandardMacros.IncrementInt` (`self.FogOfWarAreasCount`))
    (:`  `
      (if (== _result 1)
        (bind (_direction _newtrack_0) (`Timeline|Timeline` :!via `PlayFromStart` :!label _label)
          (:`Update`
            (for _array_element (`self.Materials`)
              (`MaterialInstanceDynamic.SetScalarParameterValue` _array_element "Opacity" _newtrack_0))))))))

(event `self.FadeOut`
  (bind _result (`/Engine/EditorBlueprintResources/StandardMacros.DecrementInt` (`self.FogOfWarAreasCount`))
    (:`  `
      (if (== _result 0)
        (goto _label :!via `ReverseFromEnd`)))))

(event `self.InteractCollider.OnComponentBeginOverlap`
  (params (OverlappedComponent :type "PrimitiveComponent Object Reference") (OtherActor :type "Actor Object Reference") (OtherComp :type "PrimitiveComponent Object Reference") (OtherBodyIndex :type Integer) (bFromSweep :type Boolean) (SweepResult :type "HitResult Structure (by ref)"))
  (if (`self.ActorHasTag` OtherActor "Player")
    (bind _ascharacter (cast `Character` OtherActor))
    (bind _returnvalue (`Pawn.GetController` _ascharacter))
    (`/Engine/EditorBlueprintResources/StandardMacros.IsValid` _returnvalue
      (:`Is Valid`
        (if (`Controller.IsLocalController` _returnvalue)
          (`WorldDetailsWidget.Show` (`self.WBP_WorldDetails`) (`self.ItemData`)))))))

(event `self.InteractCollider.OnComponentEndOverlap`
  (params (OverlappedComponent :type "PrimitiveComponent Object Reference") (OtherActor :type "Actor Object Reference") (OtherComp :type "PrimitiveComponent Object Reference") (OtherBodyIndex :type Integer))
  (if (`self.ActorHasTag` OtherActor "Player")
    (bind _ascharacter (cast `Character` OtherActor))
    (bind _returnvalue (`Pawn.GetController` _ascharacter))
    (`/Engine/EditorBlueprintResources/StandardMacros.IsValid` _returnvalue
      (:`Is Valid`
        (if (`Controller.IsLocalController` _returnvalue)
          (`WorldDetailsWidget.Hide` (`self.WBP_WorldDetails`)))))))

(event `self.Initialise`
  (params (Data :type "ItemInfos Structure"))
  (bind _itemdata (break `ItemInfos` Data))
  (`parent.Initialise` Data)
  (bind _aswbp_world_details (cast `/Game/UI/Widgets/WBP_WorldDetails` (`WidgetComponent.GetWidget` (`self.DetailsWidget`))))
  (set `self.WBP_WorldDetails` _aswbp_world_details)
  (`/Engine/EditorBlueprintResources/StandardMacros.IsValid` _itemdata
    (:`Is Valid`
      (`NiagaraComponent.SetAsset` (`self.RarityVFXComponent`) (`|GetArrayItem` (`self.RarityVFXs`) (`KismetMathLibrary.Conv_ByteToInt` (`ItemData.ItemRarity` _itemdata))) true))))

(fn `UserConstructionScript`)