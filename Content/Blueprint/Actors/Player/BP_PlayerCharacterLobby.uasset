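; Player character for the lobby, translating Enhanced Input into item, movement and interaction actions gated by the current player state.
; Item, interaction and stamina components do the work, with montage notifies driving repeated attack collision checks and movement emitting state-scaled noise.
; A predicted projectile path becomes spline meshes for throw previews, and auto-move arrival plays lever or chest interactions.
; Run and ranged-aim logic is partly disconnected.
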(event `EnhancedInput|/Game/Inputs/Actions/IA_LightAttack`
  (params (ActionValue :type Boolean) (ElapsedSeconds :type "Float (double-precision)") (TriggeredSeconds :type "Float (double-precision)") (InputAction :type "InputAction Object Reference" :default "/Game/Inputs/Actions/IA_LightAttack.IA_LightAttack"))
  ; Weapons Attacks
  (:`Triggered`
    (switch `EPlayerState` (`self.CurrentState`)
      (:`None`
        _)
      (:`Running`
        _)
      (:`Sneaking`
        _))
    (`ItemComponent.DoLightAttack` (`self.ItemComponent`))))

(event `EnhancedInput|/Game/Inputs/Actions/IA_ItemSecondaryAction`
  (params (ActionValue :type Boolean) (ElapsedSeconds :type "Float (double-precision)") (TriggeredSeconds :type "Float (double-precision)") (InputAction :type "InputAction Object Reference" :default "/Game/Inputs/Actions/IA_ItemSecondaryAction.IA_ItemSecondaryAction"))
  (bind _itemcomponent (`self.ItemComponent`))
  (bind _currentstate (`self.CurrentState`))
  ; Secondary Action
  (:`Started`
    (switch `EPlayerState` _currentstate
      (:`None`
        _)
      (:`Running`
        _)
      (:`Blocking`
        _)
      (:`Sneaking`
        _))
    (`ItemComponent.DoSecondaryAction` _itemcomponent))
  (:`Canceled`
    (switch `EPlayerState` _currentstate :!label _label
      (:`None`
        _)
      (:`Running`
        _)
      (:`UsingEquipment`
        _)
      (:`Blocking`
        _)
      (:`Sneaking`
        _))
    (`ItemComponent.StopSecondaryAction` _itemcomponent)
    (`self.ClearThrowPreview`))
  (:`Completed`
    (goto _label)))

(event `EnhancedInput|/Game/Inputs/Actions/IA_HeavyAttack`
  (params (ActionValue :type Boolean) (ElapsedSeconds :type "Float (double-precision)") (TriggeredSeconds :type "Float (double-precision)") (InputAction :type "InputAction Object Reference" :default "/Game/Inputs/Actions/IA_HeavyAttack.IA_HeavyAttack"))
  ; Weapons Attacks
  (:`Triggered`
    (switch `EPlayerState` (`self.CurrentState`)
      (:`None`
        _)
      (:`Running`
        _)
      (:`Sneaking`
        _))
    (`ItemComponent.DoHeavyAttack` (`self.ItemComponent`))))

(event `EnhancedInput|/Game/Inputs/Actions/IA_ItemMainAction`
  (params (ActionValue :type Boolean) (ElapsedSeconds :type "Float (double-precision)") (TriggeredSeconds :type "Float (double-precision)") (InputAction :type "InputAction Object Reference" :default "/Game/Inputs/Actions/IA_ItemMainAction.IA_ItemMainAction"))
  (bind _currentstate (`self.CurrentState`))
  (bind _itemcomponent (`self.ItemComponent`))
  ; Main Action
  (:`Started`
    (switch `EPlayerState` _currentstate
      (:`None`
        _)
      (:`Running`
        _)
      (:`UsingEquipment`
        _)
      (:`Sneaking`
        _))
    (`ItemComponent.DoMainAction` _itemcomponent)
    (`self.ClearThrowPreview`))
  (:`Canceled`
    (switch `EPlayerState` _currentstate :!label _label_2
      (:`None`
        _)
      (:`Running`
        _)
      (:`UsingEquipment`
        _)
      (:`Sneaking`
        _))
    (`ItemComponent.StopMainAction` _itemcomponent))
  (:`Completed`
    (goto _label_2)))

(event `self.BP_OnMontageNotifyBegin`
  (params (NotifyName :type Name))
  (bind _itemcomponent (`self.ItemComponent`))
  ; Do Attack Collision
  (`ItemComponent.DoAttackInertia` _itemcomponent)
  (set `self.TempInt` 0)
  (if (< (`self.TempInt`) 15) :!label _label_3
    (`ItemComponent.DoAttackCollision` _itemcomponent)
    (`/Engine/EditorBlueprintResources/StandardMacros.IncrementInt` (`self.TempInt`)
      (:`  `
        (`KismetSystemLibrary.Delay` 0.01)
        (goto _label_3)))))

(event `self.DisplayThrowPreview`
  (params (Direction :type "Vector Structure") (Strength :type "Float (single-precision)"))
  (bind _returnvalue (`self.K2_GetActorLocation`))
  (bind _splinemeshcomponents (`self.SplineMeshComponents`))
  (bind _spline (`self.Spline`))
  ; Throw Preview
  (`self.ClearThrowPreview`)
  (if (`self.bIsForcingRotation`)
    (bind _predictresult (`GameplayStatics.Blueprint_PredictProjectilePath_Advanced` (make `PredictProjectilePathParams` (`SceneComponent.K2_GetComponentLocation` (`self.ThrowStartPosRef`)) (* Direction Strength) true 5.0 1.5 true "ECC_PhysicsBody" _ _ 25.0)))
    (for _array_element (`.PathData` (break `PredictProjectilePathResult` _predictresult))
      (`SplineComponent.AddSplinePoint` _spline (`.Location` (break `PredictProjectilePathPointData` _array_element)) "World" true))
    (for _index (range 1 (+ (`SplineComponent.GetNumberOfSplinePoints` _spline) 1))
      (bind _returnvalue_2 (`AddComponent|NODE_AddSplineMeshComponent-0` :`RelativeTransform` (`KismetMathLibrary.MakeTransform` (0.0 0.0 0.0) (* (`self.CurrentForcedRotation`) -1.0))))
      (bind _returnvalue_3 (`KismetArrayLibrary.Array_Add` _splinemeshcomponents _returnvalue_2))
      (bind (_location _tangent) (`SplineComponent.GetLocationAndTangentAtSplinePoint` _spline _index "World"))
      (bind (_location_2 _tangent_2) (`SplineComponent.GetLocationAndTangentAtSplinePoint` _spline (+ _index 1) "World"))
      (`SplineMeshComponent.SetStartAndEnd` (`|GetArrayItem` _splinemeshcomponents _returnvalue_3) (- _location _returnvalue) _tangent (- (`KismetMathLibrary.VLerp` _location _location_2 0.5) _returnvalue) (`KismetMathLibrary.VLerp` _tangent _tangent_2 0.5) true))))

(event `EnhancedInput|/Game/Inputs/Actions/IA_Reload`
  (params (ActionValue :type Boolean) (ElapsedSeconds :type "Float (double-precision)") (TriggeredSeconds :type "Float (double-precision)") (InputAction :type "InputAction Object Reference" :default "/Game/Inputs/Actions/IA_Reload.IA_Reload"))
  (:`Triggered`
    (switch `EPlayerState` (`self.CurrentState`)
      (:`None`
        _)
      (:`UsingEquipment`
        _)
      (:`Sneaking`
        _))
    (`ItemComponent.Reload` (`self.ItemComponent`))))

(event `ClearThrowPreview`
  (bind _splinemeshcomponents (`self.SplineMeshComponents`))
  ; Throw Preview
  (`SplineComponent.ClearSplinePoints` (`self.Spline`) true)
  (`ActorComponent.K2_DestroyComponent` _splinemeshcomponents)
  (`KismetArrayLibrary.Array_Clear` _splinemeshcomponents))

(event `EnhancedInput|/Game/Inputs/Actions/IA_Move`
  (params (ActionValue :type "Vector2D Structure") (ElapsedSeconds :type "Float (double-precision)") (TriggeredSeconds :type "Float (double-precision)") (InputAction :type "InputAction Object Reference" :default "/Game/Inputs/Actions/IA_Move.IA_Move"))
  ; Main Movement Input
  (:`Triggered`
    (`self.MoveCharacter` ActionValue :!label _label)
    (if (> (`KismetMathLibrary.VSizeSquared` (`self.CurrentPlayerInput`)) 0.1)
      (switch `EPlayerState` (`self.CurrentState`)
        (:`None`
          (`PlayerInterface.PlaySoundOnServer` "Walk" (* (`PlayerData.WalkSoundRange` (`self.PlayerConfig`)) (`self.NoiseModifier`)) 0.3))
        (:`Running`
          (`PlayerInterface.PlaySoundOnServer` "Run" (* (`PlayerData.RunSoundRange` (`self.PlayerConfig`)) (`self.NoiseModifier`)) 0.8))
        (:`Sneaking`
          (`PlayerInterface.PlaySoundOnServer` "Sneak" (* (`PlayerData.SneakSoundRange` (`self.PlayerConfig`)) (`self.NoiseModifier`)) 0.1)))))
  (:`Ongoing`
    (goto _label))
  (:`Canceled`
    (goto _label))
  (:`Completed`
    (goto _label)))

(event `EnhancedInput|/Game/Inputs/Actions/IA_Run`
  (params (ActionValue :type Boolean) (ElapsedSeconds :type "Float (double-precision)") (TriggeredSeconds :type "Float (double-precision)") (InputAction :type "InputAction Object Reference" :default "/Game/Inputs/Actions/IA_Run.IA_Run"))
  (bind _currentstate (`self.CurrentState`))
  ; Run
  (:`Triggered`
    (if (> (`KismetMathLibrary.VSizeSquared` (`self.CurrentPlayerInput`)) 0.5)
      (switch `EPlayerState` _currentstate
        (:`None`
          _)
        (:`Running`
          _)
        (:`Blocking`)
        (:`Sneaking`
          _))
      (bind _returnvalue (`StaminaComponent.VerifyHasStamina` (`self.StaminaComponent`)))))
  (:`Canceled`
    (switch `EPlayerState` _currentstate :!label _label_2))
  (:`Completed`
    (goto _label_2)))

(event `EnhancedInput|/Game/Inputs/Actions/IA_Sneak`
  (params (ActionValue :type Boolean) (ElapsedSeconds :type "Float (double-precision)") (TriggeredSeconds :type "Float (double-precision)") (InputAction :type "InputAction Object Reference" :default "/Game/Inputs/Actions/IA_Sneak.IA_Sneak"))
  ; Sneak
  (:`Started`
    (switch `EPlayerState` (`self.CurrentState`)
      (:`None`
        (`PlayerInterface.RequestStateChange` "Sneaking" :!label _label_3))
      (:`Running`
        (goto _label_3))
      (:`Sneaking`
        (`PlayerInterface.SetCurrentPlayerState` "None")))))

(event `self.ReachAutoMoveDestination`
  (bind _interactioncomponent (`self.InteractionComponent`))
  (if (not (`HealthComponent.bIsFallen` (`self.HealthComponent`)))
    (`self.ForceRotationInstant` (`self.AutoMoveTargetRot`))
    (bind _asbp_lever_child_02 (cast `/Game/Blueprint/Actors/LDElements/Interactibles/Levers/BP_Lever_Child_02` (`self.AutoMoveTarget`))
      (:`then`
        (`InteractionComponent.DoInteractAnimation` (`self.InteractionComponent`) _asbp_lever_child_02)
        (message `Interactible.DoInteractionAnim` _asbp_lever_child_02 self)
        (`PlayerInterface.RequestStateChange` "Immobilized" true)
        (`KismetSystemLibrary.Delay` (`InteractibleObjects.InteractAnimDuration` _asbp_lever_child_02))
        (message `Interactible.Interact` _asbp_lever_child_02 self)
        (`self.StopForceRotation` 0.0)
        (`InteractionComponent.EndInteractAnimatiopn` _interactioncomponent)
        (`InteractionComponent.CancelInteraction` _interactioncomponent))
      (:`CastFailed`
        (bind _asbp_chest_base (cast `/Game/Blueprint/Actors/LDElements/Interactibles/Containers/Chests/BP_Chest_Base` (`self.AutoMoveTarget`))
          (:`then`
            (`InteractionComponent.DoInteractAnimation` (`self.InteractionComponent`) _asbp_chest_base)
            (message `Interactible.DoInteractionAnim` _asbp_chest_base self)
            (`PlayerInterface.SetCurrentPlayerState` "Immobilized" true)
            (`KismetSystemLibrary.Delay` (`InteractibleObjects.InteractAnimDuration` _asbp_chest_base))
            (`self.StopForceRotation` 0.0)
            (`InteractionComponent.EndInteractAnimatiopn` (`self.InteractionComponent`))
            (`PlayerInterface.SetCurrentPlayerState` "None" true)
            (message `Interactible.Interact` _asbp_chest_base self))
          (:`CastFailed`
            (bind _asbp_lever_child_01 (cast `/Game/Blueprint/Actors/LDElements/Interactibles/Levers/BP_Lever_Child_01` (`self.AutoMoveTarget`)))
            (`InteractionComponent.DoInteractAnimation` (`self.InteractionComponent`) _asbp_lever_child_01)
            (message `Interactible.DoInteractionAnim` _asbp_lever_child_01 self)
            (`PlayerInterface.SetCurrentPlayerState` "Immobilized" true)))))))

(event `AttachPlayerToActor`
  (params (Actor :type "SceneComponent Object Reference"))
  (set `self.AttachedActor` Actor))

(event `UnattachPlayerFromActor`
  (set `self.AttachedActor` null)
  (`self.StopForceRotation` 0.0))

(event `EnhancedInput|/Game/Inputs/Actions/IA_Interact`
  (params (ActionValue :type Boolean) (ElapsedSeconds :type "Float (double-precision)") (TriggeredSeconds :type "Float (double-precision)") (InputAction :type "InputAction Object Reference" :default "/Game/Inputs/Actions/IA_Interact.IA_Interact"))
  (bind _interactioncomponent (`self.InteractionComponent`))
  (bind _bisautomoving (`self.bIsAutoMoving`))
  (bind _currentstate (`self.CurrentState`))
  ; Interaction Inputs
  (:`Started`
    (if (not _bisautomoving)
      (switch `EPlayerState` _currentstate
        (:`None`
          _)
        (:`Running`
          _)
        (:`Carrying`
          _)
        (:`Immobilized`
          _)
        (:`Trapped`
          _)
        (:`Sneaking`
          _))
      (`InteractionComponent.StartInteract` _interactioncomponent)))
  (:`Completed`
    (if (not _bisautomoving)
      (switch `EPlayerState` _currentstate
        (:`None`
          _)
        (:`Running`
          _)
        (:`Carrying`
          _)
        (:`Immobilized`
          _)
        (:`Trapped`
          _)
        (:`Sneaking`
          _))
      (`InteractionComponent.StopInteract` _interactioncomponent))))

(event `EnhancedInput|/Game/Inputs/Actions/IA_Cancel`
  (params (ActionValue :type Boolean) (ElapsedSeconds :type "Float (double-precision)") (TriggeredSeconds :type "Float (double-precision)") (InputAction :type "InputAction Object Reference" :default "/Game/Inputs/Actions/IA_Cancel.IA_Cancel"))
  (bind _itemcomponent (`self.ItemComponent`))
  ; Interaction Inputs
  (:`Started`
    (if (not (`self.bIsAutoMoving`))
      (`KismetSystemLibrary.DelayUntilNextTick`)
      (switch `EPlayerState` (`self.CurrentState`)
        (:`None`
          (`InteractionComponent.CancelInteraction` (`self.InteractionComponent`) :!label _label))
        (:`Running`
          (goto _label))
        (:`Carrying`
          (goto _label))
        (:`UsingEquipment`
          (if (`ItemComponent.bIsReloading` _itemcomponent)
            (`ItemComponent.CancelReload` _itemcomponent)))
        (:`Immobilized`
          (goto _label))
        (:`Sneaking`
          (goto _label))))))

(event `self.SelectInteractible`
  (params (Interactor :type "Actor Object Reference"))
  (bind _returnvalue (`WidgetComponent.GetWidget` (`self.Interactible Widget Component`)))
  ; Select / Unselect Players
  (switch `EPlayerState` (`self.CurrentState`)
    (:`Fallen`
      (bind _aswbp_world_interactible (cast `/Game/UI/Widgets/WBP_WorldInteractible` _returnvalue))
      (`WorldInteractibleWidget.DisplayText` _aswbp_world_interactible "Help" "/Game/Art/PlaceHolder/Input/A_dark_color.A_dark_color"))
    (:`Dead`
      (bind _aswbp_world_interactible_2 (cast `/Game/UI/Widgets/WBP_WorldInteractible` _returnvalue))
      (`WorldInteractibleWidget.DisplayText` _aswbp_world_interactible_2 "Revive" "/Game/Art/PlaceHolder/Input/ButtonRT.ButtonRT"))))

(event `self.UnselectInteractible`
  (params (Interactor :type "Actor Object Reference"))
  ; Select / Unselect Players
  (bind _aswbp_world_interactible (cast `/Game/UI/Widgets/WBP_WorldInteractible` (`WidgetComponent.GetWidget` (`self.Interactible Widget Component`))))
  (`WorldInteractibleWidget.HideText` _aswbp_world_interactible))

(fn `OnRep_AttachedActor`
  (`self.StopForceRotation` 0.0))

(fn `OnRep_NumberOfLights`)

(fn `OnRep_PlayerColor`
  (bind _aswbp_player_name (cast `/Game/UI/Widgets/WBP_PlayerName` (`WidgetComponent.GetUserWidgetObject` (`self.Name`))))
  (`TextBlock.SetColorAndOpacity` (`/Game/UI/Widgets/WBP_PlayerName.TextBlock_30` _aswbp_player_name) (make `SlateColor` (`self.PlayerColor`))))

(fn `RegisterMapping`
  (params (Target :type "EnhancedInputSubsystemInterface Interface"))
  (bind _returnvalue (`EnhancedInputSubsystemInterface.GetUserSettings` Target))
  (if (not (`EnhancedInputUserSettings.IsMappingContextRegistered` _returnvalue "/Game/Inputs/IMC_Dawnfinders.IMC_Dawnfinders"))
    (`EnhancedInputUserSettings.RegisterInputMappingContext` _returnvalue "/Game/Inputs/IMC_Dawnfinders.IMC_Dawnfinders")))

(fn `UserConstructionScript`
  ; Get Position For Cam Cutout
  (`KismetMaterialLibrary.SetVectorParameterValue` "/Game/Art/Materials/CollectionParameter/MPC_CameraCutout.MPC_CameraCutout" "PlayerPosition" (`KismetMathLibrary.Conv_VectorToLinearColor` (`self.K2_GetActorLocation`))))