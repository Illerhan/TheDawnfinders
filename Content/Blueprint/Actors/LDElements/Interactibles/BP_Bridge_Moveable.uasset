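; BP_Bridge_Moveable is an interactible level element, a bridge that rotates between two orientations.
; RotateEvent toggles on IsActivate, lerping the root's world rotation between StartRotation and EndRotation through separate forward and return timelines, flipping the flag during updates.
; Timer sets the play rate only on the forward timeline, even in the return branch.
; Collider enable and disable logic is present but unconnected.
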(event `self.ReceiveBeginPlay`)

(event `RotateEvent`
  (if (`self.isActivate`)
    (`TimelineComponent.SetPlayRate` (`self.Timeline`) (`self.Timer`))
    (bind (_direction _track01) (`Timeline|Timeline_0` :!via `PlayFromStart`)
      (:`Update`
        (`SceneComponent.K2_SetWorldRotation` (`self.Rooot`) (`KismetMathLibrary.RLerp` (`self.EndRotation`) (`self.StartRotation`) _track01) false false)
        (set `self.isActivate` false)))
    (else
      (`TimelineComponent.SetPlayRate` (`self.Timeline`) (`self.Timer`))
      (bind (_direction_2 _track01_2) (`Timeline|Timeline` :!via `PlayFromStart`)
        (:`Update`
          (`SceneComponent.K2_SetWorldRotation` (`self.Rooot`) (`KismetMathLibrary.RLerp` (`self.StartRotation`) (`self.EndRotation`) _track01_2) false false)
          (set `self.isActivate` true))))))

(fn `UserConstructionScript`
  (`parent.UserConstructionScript`))