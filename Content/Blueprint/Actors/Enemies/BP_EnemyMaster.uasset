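; Base enemy character that senses players, attacks them and reveals itself through fog of war and light.
; State-sized hearing collider and capsule hits feed players and aggression to the AI controller; AlertEnemies spreads both to nearby enemies.
; Attacks use motion warping and repeated montage-notify collision checks, then snap back onto the navmesh.
; Dynamic materials drive hit flash, counted fog fades and light-based dissolve, while show/hide toggles ticking and AI.
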(event `self.HearCollider.OnComponentBeginOverlap`
  (params (OverlappedComponent :type "PrimitiveComponent Object Reference") (OtherActor :type "Actor Object Reference") (OtherComp :type "PrimitiveComponent Object Reference") (OtherBodyIndex :type Integer) (bFromSweep :type Boolean) (SweepResult :type "HitResult Structure (by ref)"))
  (bind _playersatrange (`/Game/Blueprint/AI/Controllers/AIC_BasicEnemy.PlayersAtRange` (`self.AIController`)))
  (bind _nearplayers (`BasicEnemyAIController.NearPlayers` (`self.AIController`)))
  (bind _playersatrange_2 (`/Game/Blueprint/AI/Controllers/AIC_BasicEnemy.PlayersAtRange` (`self.AIController`)))
  (bind _nearplayers_2 (`BasicEnemyAIController.NearPlayers` (`self.AIController`)))
  ; Near Player Aggressive trigger
  (`/Engine/EditorBlueprintResources/StandardMacros.IsValid` (`self.AIController`)
    (:`Is Valid`
      (if (and (`self.ActorHasTag` OtherActor "Player") (`ActorComponent.ComponentHasTag` OtherComp "Noise"))
        (bind _asbp_noise (cast `/Game/Blueprint/Actors/Player/BP_Noise` OtherActor)
          (:`then`
            (bind _noiseoriginactor (`Noise.NoiseOriginActor` _asbp_noise))
            (`/Engine/EditorBlueprintResources/StandardMacros.IsValid` _noiseoriginactor
              (:`Is Valid`
                (if (not (`KismetArrayLibrary.Array_Contains` _nearplayers _noiseoriginactor))
                  (`KismetArrayLibrary.Array_Add` _nearplayers _noiseoriginactor)
                  (if (not (`KismetArrayLibrary.Array_Contains` _playersatrange_2 _noiseoriginactor))
                    (`KismetArrayLibrary.Array_Add` _playersatrange_2 _noiseoriginactor))))))
          (:`CastFailed`
            (bind _returnvalue (message `PlayerInterface.GetCurrentPlayerState` OtherActor))
            (switch `EPlayerState` _returnvalue
              (:`None`
                _)
              (:`Running`
                _)
              (:`Carrying`
                _)
              (:`UsingEquipment`
                _)
              (:`Blocking`
                _)
              (:`Dodging`
                _)
              (:`Immobilized`
                _)
              (:`Trapped`
                _)
              (:`Sneaking`
                _))
            (if (not (`KismetArrayLibrary.Array_Contains` _nearplayers_2 OtherActor))
              (`KismetArrayLibrary.Array_Add` _nearplayers_2 OtherActor)
              (if (not (`KismetArrayLibrary.Array_Contains` _playersatrange OtherActor))
                (`KismetArrayLibrary.Array_Add` _playersatrange OtherActor)))))))))

(event `self.HearCollider.OnComponentEndOverlap`
  (params (OverlappedComponent :type "PrimitiveComponent Object Reference") (OtherActor :type "Actor Object Reference") (OtherComp :type "PrimitiveComponent Object Reference") (OtherBodyIndex :type Integer))
  (bind _nearplayers (`BasicEnemyAIController.NearPlayers` (`self.AIController`)))
  ; Near Player Aggressive trigger
  (`/Engine/EditorBlueprintResources/StandardMacros.IsValid` (`self.AIController`)
    (:`Is Valid`
      (if (and (`self.ActorHasTag` OtherActor "Player") (`ActorComponent.ComponentHasTag` OtherComp "Noise"))
        (if (`KismetArrayLibrary.Array_Contains` _nearplayers OtherActor)
          (`KismetArrayLibrary.Array_RemoveItem` _nearplayers OtherActor))))))

(event `self.CapsuleComponent.OnComponentHit`
  (params (HitComponent :type "PrimitiveComponent Object Reference") (OtherActor :type "Actor Object Reference") (OtherComp :type "PrimitiveComponent Object Reference") (NormalImpulse :type "Vector Structure") (Hit :type "HitResult Structure (by ref)"))
  (bind (_returnvalue_x _returnvalue_y) (`KismetMathLibrary.BreakVector` (* (`KismetMathLibrary.Normal` (- (`self.K2_GetActorLocation`) (`self.K2_GetActorLocation` OtherActor))) (/ 4000.0 (`self.PushMass`)))))
  ; Near Player Aggressive trigger
  (`self.K2_AddActorWorldOffset` (`KismetMathLibrary.MakeVector` _returnvalue_x _returnvalue_y))
  (`/Engine/EditorBlueprintResources/StandardMacros.IsValid` (`self.AIController`)
    (:`Is Valid`
      (if (and (`self.ActorHasTag` OtherActor "Player") (not (`self.bIsCrystallized`)))
        (bind _returnvalue (message `PlayerInterface.GetCurrentPlayerState` OtherActor))
        (switch `EPlayerState` _returnvalue
          (:`None`
            _)
          (:`Running`
            _)
          (:`Carrying`
            _)
          (:`UsingEquipment`
            _)
          (:`Blocking`
            _)
          (:`Dodging`
            _)
          (:`Immobilized`
            _)
          (:`Sneaking`
            _))
        (`BasicEnemyAIController.SetEnemyState` (`self.AIController`) "Aggressive")))))

(event `self.ReceiveBeginPlay`
  ; Initialisation
  (set `self.bIsInitialised` true)
  (`parent.ReceiveBeginPlay`)
  (`KismetSystemLibrary.Delay` 3.0)
  (set `self.InitialPos` (`self.K2_GetActorLocation`)))

(event `Initialise`
  ; Initialisation
  (`parent.ReceiveBeginPlay`)
  (`self.EnterIdleState`)
  (bind _asaic_basic_enemy (cast `/Game/Blueprint/AI/Controllers/AIC_BasicEnemy` (`self.GetController`))
    (:`then`
      (set `self.AIController` _asaic_basic_enemy))
    (:`CastFailed`
      _))
  (`SceneComponent.K2_AttachToComponent` (`self.AttackCollisionPosRef`) (`self.Mesh`) "LeftWeaponSocket" "SnapToTarget" "SnapToTarget" "KeepRelative" true)
  (for (_array_element _array_index) (`MeshComponent.GetMaterials` (`self.Mesh`))
    (bind _returnvalue (`KismetMaterialLibrary.CreateDynamicMaterialInstance` _array_element (`KismetStringLibrary.Conv_StringToName` (`KismetStringLibrary.Concat_StrStr` "Test " (`KismetStringLibrary.Conv_IntToString` _array_index)))))
    (`KismetArrayLibrary.Array_Add` (`self.EnemyMaterials`) _returnvalue)
    (`MaterialInstanceDynamic.SetScalarParameterValue` _returnvalue "Opacity" 0.0)
    (`PrimitiveComponent.SetMaterial` (`self.Mesh`) _array_index _returnvalue)))

(event `self.AtRangeCollider.OnComponentEndOverlap`
  (params (OverlappedComponent :type "PrimitiveComponent Object Reference") (OtherActor :type "Actor Object Reference") (OtherComp :type "PrimitiveComponent Object Reference") (OtherBodyIndex :type Integer))
  ; At Range Collider
  (`/Engine/EditorBlueprintResources/StandardMacros.IsValid` (`self.AIController`)
    (:`Is Valid`
      (if (and (`self.ActorHasTag` OtherActor "Player") (not (`ActorComponent.ComponentHasTag` OtherComp "Noise")))
        (`KismetArrayLibrary.Array_RemoveItem` (`/Game/Blueprint/AI/Controllers/AIC_BasicEnemy.PlayersAtRange` (`self.AIController`)) OtherActor)))))

(event `Server_DoHitEffect`
  ; Hit Effect
  (`self.HitEffectMulticast`))

(event `self.DoHitEffect`
  ; Hit Effect
  (`self.HitEffectMulticast`))

(event `HitEffectMulticast`
  ; Hit Effect
  (`|ExecutionSequence`
    (:`then_0`
      (bind (_direction _newtrack_0) (`Timeline|Timeline` :!via `PlayFromStart`)
        (:`Update`
          (for _array_element (`self.EnemyMaterials`)
            (`MaterialInstanceDynamic.SetVectorParameterValue` _array_element "L1Tint" (`KismetMathLibrary.LinearColorLerp` (struct :`R` 1.0 :`G` 1.0 :`B` 1.0 :`A` 1.0) (struct :`R` 1.0 :`B` 0.011963 :`A` 1.0) _newtrack_0))
            (`MaterialInstanceDynamic.SetScalarParameterValue` _array_element "L1Saturation" (+ (* _newtrack_0 10.0) 1.0))))))
    (:`then_1`
      ;;[0.15 0.04118 0.03982 0.5] Test blood vfx
      (switch `int` (`KismetMathLibrary.RandomIntegerInRange` 0 1)
        (:`0`
          (`ActorComponent.Activate` (`self.Blood2`) true))
        (:`1`
          (`ActorComponent.Activate` (`self.Blood1`) true))))))

(event `ResetTimeDilation`
  ; Hit Effect
  ;;[0.15 0.04118 0.03982 0.5] Test hit stop
  (`GameplayStatics.SetGlobalTimeDilation` 1.0))

(event `self.FadeIn`
  ; Fade Behavior
  (`self.FadeIn_Multicast`))

(event `self.StartAttack`
  (params (AttackData :type "EnemyActionData Structure") (Target :type "Actor Object Reference"))
  ; Attack (Motion Warping)
  (`parent.StartAttack` AttackData Target)
  (set `self.TargetPlayer` Target))

(event `self.FadeOut`
  ; Fade Behavior
  (`self.FadeOut_Multicast`))

(event `FadeIn_Multicast`
  ; Fade Behavior
  (bind _result (`/Engine/EditorBlueprintResources/StandardMacros.IncrementInt` (`self.FogOfWarAreasCount`))
    (:`  `
      (bind _output_get (set `self.FogOfWarAreasCount` (`KismetMathLibrary.Clamp` _result 0 100)))
      (if (== _output_get 1)
        (`parent.FadeIn`)
        (bind (_direction _newtrack_0) (`Timeline|FadeInTimeline` :!via `PlayFromStart` :!label _label)
          (:`Update`
            (for _array_element (`self.EnemyMaterials`)
              (`MaterialInstanceDynamic.SetScalarParameterValue` _array_element "Opacity" _newtrack_0))))))))

(event `/Game/Blueprint/Interface/BPI_EnemyAnimationController.UpdatePlayerLocation`
  (bind _targetplayer (`self.TargetPlayer`))
  ; Attack (Motion Warping)
  (`/Engine/EditorBlueprintResources/StandardMacros.IsValid` _targetplayer
    (:`Is Valid`
      (`MotionWarpingComponent.AddOrUpdateWarpTarget` (`self.MotionWarping`) (make `MotionWarpingTarget` "AttackTarget" (`self.K2_GetActorLocation` _targetplayer) (`self.K2_GetActorRotation`))))))

(event `FadeOut_Multicast`
  ; Fade Behavior
  (bind _result (`/Engine/EditorBlueprintResources/StandardMacros.DecrementInt` (`self.FogOfWarAreasCount`))
    (:`  `
      (bind _output_get (set `self.FogOfWarAreasCount` (`KismetMathLibrary.Clamp` _result 0 100)))
      (if (== _output_get 0)
        (`parent.FadeOut`)
        (goto _label :!via `ReverseFromEnd`)))))

(event `self.ReceiveTick`
  (params (DeltaSeconds :type "Float (single-precision)"))
  (bind _aicontroller (`self.AIController`))
  (bind _initialpos (`self.InitialPos`))
  ; Event Tick
  (`parent.ReceiveTick` DeltaSeconds)
  (if (`self.HasAuthority`)
    (`|ExecutionSequence`
      (:`then_0`
        (`/Engine/EditorBlueprintResources/StandardMacros.IsValid` _aicontroller
          (:`Is Valid`
            (set `self.CurrentEnemyState` (`BasicEnemyAIController.EnemyState` _aicontroller))
            (set `self.FollowingStatus` (`AIController.GetMoveStatus` _aicontroller))
            (if (not (`self.bLockRotation`))
              (`self.K2_SetActorRotation` (`KismetMathLibrary.RInterpTo` (`self.K2_GetActorRotation`) (`KismetMathLibrary.MakeRotator` 0.0 0.0 (.yaw (`KismetMathLibrary.FindLookAtRotation` (`self.K2_GetActorLocation`) (`AIController.GetImmediateMoveDestination` (`self.AIController`))))) DeltaSeconds 5.0))))))
      (:`then_1`
        (if (and (`self.bIsCrystallized`) (!= _initialpos (0.0 0.0 0.0)))
          (`self.K2_SetActorLocation` _initialpos))))))

(event `self.BP_OnMontageNotifyBegin`
  (params (NotifyName :type Name))
  ; Montages
  (set `self.TempInt` 0)
  (if (< (`self.TempInt`) 8) :!label _label_2
    (`self.DoAttackCollision`)
    (`/Engine/EditorBlueprintResources/StandardMacros.IncrementInt` (`self.TempInt`)
      (:`  `
        (`KismetSystemLibrary.Delay` 0.008)
        (goto _label_2)))))

(event `self.BP_OnMontageEnd`
  (params (bInterrupted :type Boolean))
  (bind _aicontroller (`self.AIController`))
  (bind (_projectedlocation _returnvalue) (`NavigationSystemV1.K2_ProjectPointToNavigation` (`self.K2_GetActorLocation`) null null (500.0 500.0 500.0)))
  ; Montages
  (`/Engine/EditorBlueprintResources/StandardMacros.IsValid` _aicontroller
    (:`Is Valid`
      (`/Game/Blueprint/AI/Controllers/AIC_BasicEnemy.EndAttack` _aicontroller)
      (if _returnvalue
        (`self.K2_SetActorLocation` _projectedlocation)))))

(event `self.EnterSuspicious`
  ; Enter / Exit Listning + Suspicious State
  (`SphereComponent.SetSphereRadius` (`self.HearCollider`) (`EnemyData.SuspiciousHearingRadius` (`self.EnemyData`)) true))

(event `ShowEnemyLocal`
  (bind _aicontroller (`self.AIController`))
  (`ActorComponent.SetComponentTickEnabled` (`self.Mesh`) true :!label _label_3)
  (`ActorComponent.SetComponentTickEnabled` (`self.CharacterMovement`) true)
  (`self.SetActorHiddenInGame` false)
  (`self.SetActorTickEnabled` true)
  (`/Engine/EditorBlueprintResources/StandardMacros.IsValid` _aicontroller
    (:`Is Valid`
      (`BasicEnemyAIController.EnableAIController` _aicontroller))))

(event `self.ShowEnemy`
  (goto _label_3))

(event `self.EnterIdleState`
  ; Enter / Exit Listning + Suspicious State
  (`SphereComponent.SetSphereRadius` (`self.HearCollider`) (`EnemyData.NormalHearingRadius` (`self.EnemyData`)) true))

(event `HideEnemyLocal`
  (bind _aicontroller (`self.AIController`))
  (`ActorComponent.SetComponentTickEnabled` (`self.Mesh`) false :!label _label_4)
  (`ActorComponent.SetComponentTickEnabled` (`self.CharacterMovement`) false)
  (`self.SetActorHiddenInGame` true)
  (`self.SetActorTickEnabled` false)
  (`/Engine/EditorBlueprintResources/StandardMacros.IsValid` _aicontroller
    (:`Is Valid`
      (`BasicEnemyAIController.DisableAIController` _aicontroller))))

(event `self.EnterListeningState`
  ; Enter / Exit Listning + Suspicious State
  (`SphereComponent.SetSphereRadius` (`self.HearCollider`) (`EnemyData.ListeningHearingRadius` (`self.EnemyData`)) true))

(event `/Game/Blueprint/Actors/Others/IFogOfWar.Light On`
  (params (isTorchLight :type Boolean))
  ;[0.4635 0.1823 0 0.5] Fog of War
  (bind _result (`/Engine/EditorBlueprintResources/StandardMacros.IncrementInt` (`self.NumberOfLights`) :!label _label_5)
    (:`  `
      (if (== _result 1)
        (`self.Appear`)))))

(event `self.HideEnemy`
  (goto _label_4))

(event `/Game/Blueprint/Actors/Others/IFogOfWar.Palanquin Light On`
  ;[0.4635 0.1823 0 0.5] Fog of War
  (goto _label_5))

(event `/Game/Blueprint/Actors/Others/IFogOfWar.Light Off`
  (params (isTorchLight :type Boolean))
  ;[0.4635 0.1823 0 0.5] Fog of War
  (bind _output_get (set `self.NumberOfLights` (`KismetMathLibrary.Max` (- (`self.NumberOfLights`) 1)) :!label _label_6))
  (if (<= _output_get 0)
    (`self.Disappear`)))

(event `/Game/Blueprint/Actors/Others/IFogOfWar.Palanquin Light Off`
  ;[0.4635 0.1823 0 0.5] Fog of War
  (goto _label_6))

(event `Appear`
  ;[0.4635 0.1823 0 0.5] Fog of War
  (bind (_direction _alpha) (`Timeline|Dissolve` :!label _label_7)
    (:`Update`
      (for _array_element (`self.EnemyMaterials`)
        (`MaterialInstanceDynamic.SetScalarParameterValue` _array_element "DissolveAmmount" (`KismetMathLibrary.Lerp` 1.0 -1.0 _alpha))))))

(event `Disappear`
  ;[0.4635 0.1823 0 0.5] Fog of War
  (goto _label_7 :!via `Reverse`))

(fn `AlertEnemies`
  (bind _returnvalue (`self.K2_GetActorLocation`))
  (bind _outhits (`KismetSystemLibrary.SphereTraceMulti` _returnvalue _returnvalue 1000.0 "TraceTypeQuery3"))
  (for _array_element _outhits
    (bind _asbp_enemy_master (cast `/Game/Blueprint/Actors/Enemies/BP_EnemyMaster` (`.HitActor` (`GameplayStatics.BreakHitResult` _array_element))))
    (bind _aicontroller (`BaseEnemy.AIController` _asbp_enemy_master))
    (set `BasicEnemyAIController.PlayersAtRange` (`BasicEnemyAIController.PlayersAtRange` (`self.AIController`)) _aicontroller)
    (`BasicEnemyAIController.SetEnemyState` _aicontroller "Aggressive")))

(fn `OnRep_bIsInitialised`
  (`self.Initialise`))

(fn `OnRep_NumberOfLights`)

(fn `UserConstructionScript`)