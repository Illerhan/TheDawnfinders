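; BP_CarriableVivianite is a carriable vivianite item that serves as light fuel for a BP_Litter.
; When put in a target actor that is a litter, it stores its FuelAmount in the litter's LightComponent.
; It then shows a French light-activation prompt and icon on the litter's world interactible widget.
; A Sequence runs the parent put-in handling afterward, even if the target is not a litter.
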(event `self.PutInTargetActor`
  (params (Actor :type "Actor Object Reference"))
  (`|ExecutionSequence`
    (:`then_0`
      (bind _asbp_litter (cast `/Game/Blueprint/Actors/LDElements/Interactibles/BP_Litter` Actor))
      ; Do effect on litter
      (`PlayerLightComponent.StoreFuel` (`Litter.LightComponent` _asbp_litter) (`self.FuelAmount`))
      (bind _aswbp_world_interactible (cast `/Game/UI/Widgets/WBP_WorldInteractible` (`WidgetComponent.GetWidget` (`InteractibleObjects.InteractibleWidgetComponent` _asbp_litter))))
      (`WorldInteractibleWidget.DisplayText` _aswbp_world_interactible "Activé la lumiere" "/Game/Art/PlaceHolder/Input/A_dark_color.A_dark_color"))
    (:`then_1`
      (`parent.PutInTargetActor` Actor))))

(fn `UserConstructionScript`
  (`parent.UserConstructionScript`))