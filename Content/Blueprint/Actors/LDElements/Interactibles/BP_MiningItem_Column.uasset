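; BP_MiningItem_Column is a minable column interactible that can topple and hurt the player.
; FallEvent pushes the physics mesh with a delayed force, enables the outline collider, then opens a short window where hits deal heavy damage to the player.
; Overlaps on that collider toggle a dynamic outline overlay material.
; The actor's location feeds a material parameter collection, and damage extends the parent logic with an audio-style PostEvent.
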(event `self.OutlineCollider.OnComponentBeginOverlap`
  (params (OverlappedComponent :type "PrimitiveComponent Object Reference") (OtherActor :type "Actor Object Reference") (OtherComp :type "PrimitiveComponent Object Reference") (OtherBodyIndex :type Integer) (bFromSweep :type Boolean) (SweepResult :type "HitResult Structure (by ref)"))
  ; OutlineOverlap
  (`MaterialInstanceDynamic.SetScalarParameterValue` (stale `self.ReceiveBeginPlay` _returnvalue) "IsVisible" 1.0))

(event `self.OutlineCollider.OnComponentEndOverlap`
  (params (OverlappedComponent :type "PrimitiveComponent Object Reference") (OtherActor :type "Actor Object Reference") (OtherComp :type "PrimitiveComponent Object Reference") (OtherBodyIndex :type Integer))
  ; OutlineOverlap
  (`MaterialInstanceDynamic.SetScalarParameterValue` (stale `self.ReceiveBeginPlay` _returnvalue) "IsVisible" 0.0))

(event `self.ReceiveBeginPlay`
  (`parent.ReceiveBeginPlay`)
  (`SceneComponent.K2_SetRelativeRotation` (`self.StaticMesh`) (`KismetMathLibrary.MakeRotator` 0.0 0.0 (`KismetMathLibrary.RandomFloatInRange` -10.0 10.0)) false false)
  (bind _returnvalue (`KismetMaterialLibrary.CreateDynamicMaterialInstance` "/Game/Art/Materials/Instances/Instances-FXs/MI_OutlineOverlay_02.MI_OutlineOverlay_02"))
  (`MeshComponent.SetOverlayMaterial` (`self.StaticMesh`) _returnvalue)
  (`KismetMaterialLibrary.SetVectorParameterValue` "/Game/Art/Materials/CollectionParameter/MPC_ColorModifiers.MPC_ColorModifiers" "DepositPosition" (`KismetMathLibrary.Conv_VectorToLinearColor` (`self.K2_GetActorLocation`)))
  (`PrimitiveComponent.SetCollisionEnabled` (`self.BoxCollider`) "NoCollision")
  (`PrimitiveComponent.SetCollisionEnabled` (`self.OutlineCollider`) "NoCollision")
  (`KismetSystemLibrary.Delay` (`self.delay`))
  (`SceneComponent.K2_SetWorldRotation` :`self` (`self.StaticMesh`)))

(event `self.ReceiveDamage`
  (params (Quantity :type "Float (single-precision)") (Origin :type "Actor Object Reference"))
  (`parent.ReceiveDamage` Quantity Origin)
  (`AkGameplayStatics.PostEvent` null Origin))

(event `FallEvent`
  ; FallEvent
  (`KismetSystemLibrary.Delay` (`self.delay`))
  (`PrimitiveComponent.AddForceAtLocation` (`self.StaticMesh`) (`self.DirectionFallForce`) (`SceneComponent.K2_GetComponentLocation` (`self.Sphere`)) "None")
  (`PrimitiveComponent.SetCollisionEnabled` (`self.OutlineCollider`) "QueryOnly")
  (`KismetSystemLibrary.Delay` 1.5)
  (set `self.IsFallen` true)
  (`KismetSystemLibrary.Delay` 1.3)
  (set `self.IsFallen` false))

(event `self.StaticMesh.OnComponentHit`
  (params (HitComponent :type "PrimitiveComponent Object Reference") (OtherActor :type "Actor Object Reference") (OtherComp :type "PrimitiveComponent Object Reference") (NormalImpulse :type "Vector Structure") (Hit :type "HitResult Structure (by ref)"))
  ; FallEvent
  (if (`self.IsFallen`)
    (bind _asbp_player_character (cast `/Game/Blueprint/Actors/Player/BP_PlayerCharacter` OtherActor))
    (`HealthComponent.TakeDamage` (`APlayerCharacter.HealthComponent` _asbp_player_character) 100.0 "Blood")
    (`KismetSystemLibrary.PrintString` "Die")))

(fn `UserConstructionScript`
  (`KismetMaterialLibrary.SetVectorParameterValue` "/Game/Art/Materials/CollectionParameter/MPC_ColorModifiers.MPC_ColorModifiers" "DepositPosition" (`KismetMathLibrary.Conv_VectorToLinearColor` (`self.K2_GetActorLocation`))))