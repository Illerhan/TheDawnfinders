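; Destructible column actor that topples on the first hit and is destroyed by further hits.
; The first TakeDamage calls the custom Destroy event, which sets IsDown and plays a timeline lerping the actor's rotation from zero to TargetRot.
; Once down, each hit decrements HealthPoints, printing a debug "CROUNCH" until it reaches zero and the actor is destroyed.
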(event `Destroy`
  (if (not (`self.isDown`))
    (set `self.isDown` true)
    (bind (_direction _newtrack_0) (`Timeline|Timeline` :!via `PlayFromStart`)
      (:`Update`
        (`self.K2_SetActorRotation` (`KismetMathLibrary.RLerp` (struct) (`self.TargetRot`) _newtrack_0))))))

(event `TakeDamage`
  (if (`self.isDown`)
    (bind _result (`/Engine/EditorBlueprintResources/StandardMacros.DecrementInt` (`self.healthPoints`))
      (:`  `
        (if (<= _result 0)
          (`self.K2_DestroyActor`)
          (else
            (`KismetSystemLibrary.PrintString` "CROUNCH")))))
    (else
      (`self.Destroy`))))

(fn `UserConstructionScript`)