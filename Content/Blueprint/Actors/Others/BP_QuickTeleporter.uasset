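; Quick-teleport actor that moves the first player's pawn to one of three preset locations with a key press.
; On BeginPlay it enables input for player controller 0, binding numpad 7, 8 and 9 to the matching Teleporter location variables.
; Each key passes its location and the pawn to Multicast_ServerTP, an event named for multicast replication, which teleports the pawn with zero rotation.
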(event `self.ReceiveBeginPlay`
  (`self.EnableInput` (`GameplayStatics.GetPlayerController` 0)))

(event `Key|NumPadSeven`
  (params (Key :type "Key Structure"))
  (:`Pressed`
    (if (== "NumPadSeven" Key)
      (`self.Multicast_ServerTP` (`self.Teleporter 7`) (`GameplayStatics.GetPlayerPawn` 0)))))

(event `Key|NumPadEight`
  (params (Key :type "Key Structure"))
  (:`Pressed`
    (if (== "NumPadEight" Key)
      (`self.Multicast_ServerTP` (`self.Teleporter 8`) (`GameplayStatics.GetPlayerPawn` 0)))))

(event `Key|NumPadNine`
  (params (Key :type "Key Structure"))
  (:`Pressed`
    (if (== "NumPadNine" Key)
      (`self.Multicast_ServerTP` (`self.Teleporter 9`) (`GameplayStatics.GetPlayerPawn` 0)))))

(event `Multicast_ServerTP`
  (params (Location :type "Vector Structure") (Pawn :type "Pawn Object Reference"))
  (`self.K2_TeleportTo` :`self` Pawn :`DestLocation` Location))

(fn `UserConstructionScript`)