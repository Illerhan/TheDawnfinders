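; BP_ExtractInteractible is a lever actor that starts extraction when interacted with.
; Interaction calls the BP_Mule to the extraction zone through its AI controller, flags the game mode as extracting, starts its timer and reveals a navigation VFX.
; A dynamic overlay material on the lever mesh, created at BeginPlay, toggles an outline's visibility as actors enter or leave the interact collider.
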(event `self.InteractCollider.OnComponentBeginOverlap`
  (params (OverlappedComponent :type "PrimitiveComponent Object Reference") (OtherActor :type "Actor Object Reference") (OtherComp :type "PrimitiveComponent Object Reference") (OtherBodyIndex :type Integer) (bFromSweep :type Boolean) (SweepResult :type "HitResult Structure (by ref)"))
  ; OutlineOverlap
  (`MaterialInstanceDynamic.SetScalarParameterValue` (stale `self.ReceiveBeginPlay` _returnvalue_2) "IsVisible" 1.0))

(event `self.InteractCollider.OnComponentEndOverlap`
  (params (OverlappedComponent :type "PrimitiveComponent Object Reference") (OtherActor :type "Actor Object Reference") (OtherComp :type "PrimitiveComponent Object Reference") (OtherBodyIndex :type Integer))
  ; OutlineOverlap
  (`MaterialInstanceDynamic.SetScalarParameterValue` (stale `self.ReceiveBeginPlay` _returnvalue_2) "IsVisible" 0.0))

(event `self.ReceiveBeginPlay`
  (bind _returnvalue (`GameplayStatics.GetActorOfClass` "/Game/Blueprint/Actors/Mule/BP_Mule.BP_Mule_C"))
  (set `self.Mule` _returnvalue)
  (bind _returnvalue_2 (`KismetMaterialLibrary.CreateDynamicMaterialInstance` "/Game/Art/Materials/Instances/Instances-FXs/MI_OutlineOverlay_03.MI_OutlineOverlay_03"))
  (`MeshComponent.SetOverlayMaterial` (`self.SkeletalMeshLever`) _returnvalue_2))

(event `ShowSpline`
  (`self.SetActorHiddenInGame` (`self.NavigationVFX`) false))

(event `self.BP_OnInteraction`
  (params (Player :type "APlayerCharacter Object Reference"))
  (bind _asaic_mule_controller (cast `/Game/Blueprint/Actors/Mule/AIC_MuleController` (`AIBlueprintHelperLibrary.GetAIController` (`self.Mule`))))
  (`MuleAIController.CallMule` _asaic_mule_controller (`self.Extraction Zone`))
  (bind _asbp_custom_game_mode (cast `/Game/Blueprint/GameFramework/BP_CustomGameMode` (`GameplayStatics.GetGameMode`)))
  (set `/Game/Blueprint/GameFramework/BP_CustomGameMode.bIsExtracting` true _asbp_custom_game_mode)
  (`/Game/Blueprint/GameFramework/BP_CustomGameMode.TimerExtraction` _asbp_custom_game_mode (`self.ExtractionTimer`))
  (`self.ShowSpline`))

(fn `UserConstructionScript`)