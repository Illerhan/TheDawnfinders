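; BP_Chest is an interactible level-design chest that zeroes the Opacity parameter of its materials at startup.
; On BeginPlay, after the parent logic, it creates a dynamic instance of each material on StaticMesh and Cube and assigns it back to its slot.
; Each instance is stored in the Materials array; this graph has no interaction or later opacity changes.
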(event `self.ReceiveBeginPlay`
  (`parent.ReceiveBeginPlay`)
  (`|ExecutionSequence`
    (:`then_0`
      (for (_array_element _array_index) (`MeshComponent.GetMaterials` (`self.StaticMesh`))
        (bind _returnvalue (`KismetMaterialLibrary.CreateDynamicMaterialInstance` _array_element))
        (`KismetArrayLibrary.Array_Add` (`self.Materials`) _returnvalue)
        (`MaterialInstanceDynamic.SetScalarParameterValue` _returnvalue "Opacity" 0.0)
        (`PrimitiveComponent.SetMaterial` (`self.StaticMesh`) _array_index _returnvalue)))
    (:`then_1`
      (for (_array_element_2 _array_index_2) (`MeshComponent.GetMaterials` (`self.Cube`))
        (bind _returnvalue_2 (`KismetMaterialLibrary.CreateDynamicMaterialInstance` _array_element_2))
        (`KismetArrayLibrary.Array_Add` (`self.Materials`) _returnvalue_2)
        (`MaterialInstanceDynamic.SetScalarParameterValue` _returnvalue_2 "Opacity" 0.0)
        (`PrimitiveComponent.SetMaterial` (`self.Cube`) _array_index_2 _returnvalue_2)))))

(fn `UserConstructionScript`)