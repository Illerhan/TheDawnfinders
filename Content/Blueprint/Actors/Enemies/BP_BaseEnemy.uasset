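; Base enemy actor with overlap-driven player detection, melee attacks and fog-of-war visibility.
; A replicated init flag's OnRep caches the AI controller and widget and creates transparent dynamic materials.
; Hearing overlaps set the controller Aggressive by player state, while a range collider maintains its players-at-range list.
; Montage notifies toggle the damage collider, and multicast fades use an area counter to drive an opacity timeline.
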(event `self.ReceiveBeginPlay`
  (set `self.bIsInitialised` true))

(event `Initialise`
  (bind _asaic_basic_enemy (cast `/Game/Blueprint/Actors/Enemies/AIC_BasicEnemy` (`self.GetController`))
    (:`then`
      (set `self.AIController` _asaic_basic_enemy))
    (:`CastFailed`
      _))
  (bind _aswbp_enemy (cast `/Game/UI/Widgets/WBP_Enemy` (`WidgetComponent.GetWidget` (`self.Widget`)))
    (:`then`
      (set `self.WBP_Enemy` _aswbp_enemy))
    (:`CastFailed`
      _))
  (`PrimitiveComponent.SetCollisionEnabled` (`self.AttackCollider`) "NoCollision")
  (for (_array_element _array_index) (`MeshComponent.GetMaterials` (`self.Mesh`))
    (bind _returnvalue (`KismetMaterialLibrary.CreateDynamicMaterialInstance` _array_element))
    (`KismetArrayLibrary.Array_Add` (`self.EnemyMaterials`) _returnvalue)
    (`MaterialInstanceDynamic.SetScalarParameterValue` _returnvalue "Opacity" 0.0)
    (`PrimitiveComponent.SetMaterial` (`self.Mesh`) _array_index _returnvalue)))

(event `self.HearCollider.OnComponentBeginOverlap`
  (params (OverlappedComponent :type "PrimitiveComponent Object Reference") (OtherActor :type "Actor Object Reference") (OtherComp :type "PrimitiveComponent Object Reference") (OtherBodyIndex :type Integer) (bFromSweep :type Boolean) (SweepResult :type "HitResult Structure (by ref)"))
  (`/Engine/EditorBlueprintResources/StandardMacros.IsValid` (`self.AIController`)
    (:`Is Valid`
      (if (`self.ActorHasTag` OtherActor "Player")
        (bind _returnvalue (message `PlayerInterface.GetCurrentPlayerState` OtherActor))
        (switch `EPlayerState` _returnvalue
          (:`None`
            _)
          (:`Running`
            _)
          (:`Crouching`
            _)
          (:`UsingEquipment`
            _)
          (:`Blocking`
            _)
          (:`Dodging`
            _)
          (:`Immobilized`
            _))
        (`/Game/Blueprint/Actors/Enemies/AIC_BasicEnemy.SetEnemyState` (`self.AIController`) "Aggressive")))))

(event `self.FadeIn`
  (`self.FadeIn_Multicast`))

(event `self.AtRangeCollider.OnComponentBeginOverlap`
  (params (OverlappedComponent :type "PrimitiveComponent Object Reference") (OtherActor :type "Actor Object Reference") (OtherComp :type "PrimitiveComponent Object Reference") (OtherBodyIndex :type Integer) (bFromSweep :type Boolean) (SweepResult :type "HitResult Structure (by ref)"))
  (`/Engine/EditorBlueprintResources/StandardMacros.IsValid` (`self.AIController`)
    (:`Is Valid`
      (if (`self.ActorHasTag` OtherActor "Player")
        (`KismetArrayLibrary.Array_Add` (`/Game/Blueprint/Actors/Enemies/AIC_BasicEnemy.PlayersAtRange` (`self.AIController`)) OtherActor)))))

(event `self.FadeOut`
  (`self.FadeOut_Multicast`))

(event `FadeIn_Multicast`
  (bind _result (`/Engine/EditorBlueprintResources/StandardMacros.IncrementInt` (`self.FogOfWarAreasCount`))
    (:`  `
      (if (== _result 1)
        (bind (_direction _newtrack_0) (`Timeline|FadeInTimeline` :!label _label)
          (:`Update`
            (for _array_element (`self.EnemyMaterials`)
              (`MaterialInstanceDynamic.SetScalarParameterValue` _array_element "Opacity" _newtrack_0))))))))

(event `FadeOut_Multicast`
  (bind _result (`/Engine/EditorBlueprintResources/StandardMacros.DecrementInt` (`self.FogOfWarAreasCount`))
    (:`  `
      (if (== _result 0)
        (goto _label :!via `ReverseFromEnd`)))))

(event `self.AtRangeCollider.OnComponentEndOverlap`
  (params (OverlappedComponent :type "PrimitiveComponent Object Reference") (OtherActor :type "Actor Object Reference") (OtherComp :type "PrimitiveComponent Object Reference") (OtherBodyIndex :type Integer))
  (`/Engine/EditorBlueprintResources/StandardMacros.IsValid` (`self.AIController`)
    (:`Is Valid`
      (if (`self.ActorHasTag` OtherActor "Player")
        (`KismetArrayLibrary.Array_RemoveItem` (`/Game/Blueprint/Actors/Enemies/AIC_BasicEnemy.PlayersAtRange` (`self.AIController`)) OtherActor)))))

(event `self.BP_OnMontageNotifyBegin`
  (params (NotifyName :type Name))
  (bind _attackcollider (`self.AttackCollider`))
  ; Attacks
  (`/Engine/EditorBlueprintResources/StandardMacros.FlipFlop`
    (:`A`
      (`PrimitiveComponent.SetCollisionEnabled` _attackcollider "QueryOnly"))
    (:`B`
      (`PrimitiveComponent.SetCollisionEnabled` _attackcollider "NoCollision"))))

(event `self.AttackCollider.OnComponentBeginOverlap`
  (params (OverlappedComponent :type "PrimitiveComponent Object Reference") (OtherActor :type "Actor Object Reference") (OtherComp :type "PrimitiveComponent Object Reference") (OtherBodyIndex :type Integer) (bFromSweep :type Boolean) (SweepResult :type "HitResult Structure (by ref)"))
  ; Attacks
  (if (`self.ActorHasTag` OtherActor "Enemy")
    _
    (elif (`KismetSystemLibrary.DoesImplementInterface` OtherActor "/Script/TheDawnfinders.Damageable")
      (message `Damageable.ReceiveDamage` OtherActor 5.0 self))))

(fn `OnRep_bIsInitialised`
  (`self.Initialise`))

(fn `UserConstructionScript`)