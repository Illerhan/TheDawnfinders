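; Game mode for an extraction game, handling player survival, end-of-run recaps and loot payout before seamless travel.
; Extraction checks and timers show each player's recap, as does an all-dead check with a failure flag.
; Before travel, the BP_Mule's inventory value is split per player; unprotected players lose their items and get gold scaled by DeathMult.
; Inventory is saved on the player state, and gold through the game instance's save.
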(event `CleanInventory`
  (params (Target :type "CustomPlayerState Object Reference"))
  ;[0.15 0.04923 0.000495 0.5] Clean Inventory
  (bind _asbp_player_character (cast `/Game/Blueprint/Actors/Player/BP_PlayerCharacter` (`PlayerState.GetPawn` Target)))
  (bind _inventorycomponent (`APlayerCharacter.InventoryComponent` _asbp_player_character))
  (bind (_arrayindex _arrayelement) (`/Engine/EditorBlueprintResources/StandardMacros.ReverseForEachLoop` (`InventoryComponent.InventorySlots` _inventorycomponent))
    (:`LoopBody`
      (`/Engine/EditorBlueprintResources/StandardMacros.IsValid` (break `ItemInfos` (break `InventorySlot` _arrayelement))
        (:`Is Valid`
          (`InventoryComponent.RemoveItemAtIndex` _inventorycomponent _arrayindex true false))))))

(event `AddPlayerAlive`
  (params (Player :type "APlayerCharacter Object Reference (by ref)"))
  (`KismetArrayLibrary.Array_Add` (`self.PlayersAlive`) Player))

(event `RemovePlayerAlive`
  (params (Player :type "APlayerCharacter Object Reference (by ref)"))
  (`KismetArrayLibrary.Array_RemoveItem` (`self.PlayersAlive`) Player))

(event `CheckIOfDead`
  (params (Target :type "CustomPlayerState Object Reference") (A :type Integer))
  ;[0.009147 0.15 0 0.5] Check if dead for loot gestion
  (bind _output_get (set `self.PS` Target))
  (if (`CustomPlayerState.bIsProtected` _output_get)
    (set `CustomPlayerState.SavedGold` (+ (`CustomPlayerState.SavedGold` (`self.PS`)) A) (`self.PS`))
    (else
      (`self.CleanInventory` (`self.PS`))
      (set `CustomPlayerState.SavedGold` (+ (`CustomPlayerState.SavedGold` (`self.PS`)) (* A (`self.DeathMult`))) (`self.PS`))))
  (`CustomPlayerState.SaveInventoryBeforeTravel` (`self.PS`)))

(event `self.OnPreSeamlessTravel`
  (params (PC :type "Controller Object Reference") (PS :type "CustomPlayerState Object Reference") (Players :type Integer))
  ;[0.15 0.1395 0 0.5] Pre Seemless travel item and gold global gestion
  (bind _returnvalue (`GameplayStatics.GetActorOfClass` "/Game/Blueprint/Actors/Mule/BP_Mule.BP_Mule_C"))
  (bind _inventorycomponent (`Mule.InventoryComponent` _returnvalue))
  (`InventoryComponent.UpdateValuable` _inventorycomponent)
  (bind _asps_custom (cast `/Game/Blueprint/GameFramework/PS_Custom` PS))
  (`self.CheckIOfDead` _asps_custom (/ (`InventoryComponent.CurrentValue` _inventorycomponent) Players))
  (bind _asgi_custom (cast `/Game/Blueprint/GameFramework/GI_Custom` (`GameplayStatics.GetGameInstance`)))
  (set `/Game/Blueprint/GameFramework/BP_LocalSave.Gold` (`CustomPlayerState.SavedGold` (`self.PS`)) (`/Game/Blueprint/GameFramework/GI_Custom.GameSave` _asgi_custom))
  (`/Game/Blueprint/GameFramework/GI_Custom.SavePlayerData` _asgi_custom))

(event `CheckExtraction`
  ;[0.03018 0.03496 0.15 0.5] Extraction Gestion
  (`self.bAllSafe`
    (:`then`
      (`self.bIsExtracting`
        (:`then`
          (`KismetSystemLibrary.K2_SetTimerDelegate` (delegate `Extract`) 5.0)
          (for _array_element (`GameStateBase.PlayerArray` (`GameplayStatics.GetGameState`))
            (bind _aspc_custom (cast `/Game/Blueprint/GameFramework/PC_Custom` (`PlayerState.GetPlayerController` _array_element)))
            (`/Game/Blueprint/GameFramework/PC_Custom.Client_SHowRecap` _aspc_custom true)))
        (:`else`)))
    (:`else`)))

(event `Extract`
  ;[0.03018 0.03496 0.15 0.5] Extraction Gestion
  (for _array_element (`GameStateBase.PlayerArray` (`GameplayStatics.GetGameState`))
    (bind _aspc_custom (cast `/Game/Blueprint/GameFramework/PC_Custom` (`PlayerState.GetPlayerController` _array_element)))
    (`/Game/Blueprint/GameFramework/PC_Custom.Client_SHowRecap` _aspc_custom true)))

(event `TimerExtraction`
  (params (Time :type "Float (single-precision)"))
  ;[0.03018 0.03496 0.15 0.5] Extraction Gestion
  (`KismetSystemLibrary.K2_SetTimerDelegate` (delegate `Extract`) Time)
  (bind _asbp_custom_game_state (cast `/Game/Blueprint/GameFramework/BP_CustomGameState` (`GameplayStatics.GetGameState`)))
  (`/Game/Blueprint/GameFramework/BP_CustomGameState.Multicast_TimerExtreaction` _asbp_custom_game_state Time))

(event `self.CheckAllDead`
  (bind _returnvalue (`GameplayStatics.GetGameState`))
  (cast `/Game/Blueprint/GameFramework/BP_CustomGameState` _returnvalue)
  (if (>= (`self.DeadPlayerCount`) (`KismetArrayLibrary.Array_Length` (`GameStateBase.PlayerArray` _returnvalue)))
    (for _array_element (`GameStateBase.PlayerArray` (`GameplayStatics.GetGameState`))
      (bind _aspc_custom (cast `/Game/Blueprint/GameFramework/PC_Custom` (`PlayerState.GetPlayerController` _array_element)))
      (`/Game/Blueprint/GameFramework/PC_Custom.Client_SHowRecap` _aspc_custom false))))

(fn `HandleSeamlessTravelPlayer`
  (returns (C :type "Controller Object Reference"))
  (return null))

(fn `UserConstructionScript`)