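; BP_CurseStatue is a trap that unleashes a curse when it catches a player moving while its eyes are open.
; Opening the eyes lights them and, after a brief grace delay, enables a sight collider until they close.
; Tick checks the velocity of tagged players inside that collider.
; The first detected movement stops Tick, multicast-enables the child-actor BP_CurseZone and activates the statue's Niagara effect.
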(event `self.ReceiveBeginPlay`
  (`self.CloseStatueEyes`)
  (`ActorComponent.SetActive` (`self.CurseZone`) false false)
  (bind _asbp_curse_zone (cast `/Game/Blueprint/Actors/LDElements/Traps/BP_CurseZone` (`ChildActorComponent.ChildActor` (`self.CurseZone`))))
  (`CurseZone.Multicast_SetEnabled` _asbp_curse_zone false))

(event `self.OpenStatueEyes`
  (params (Duration :type "Float (single-precision)"))
  ; Open / Close Eyes
  (if (not (and (`self.CurseDeployed`) (`self.HasAuthority`)))
    (`parent.OpenStatueEyes` Duration)
    (`LightComponent.SetIntensity` (`self.Eye1`) 1000.0)
    (`LightComponent.SetIntensity` (`self.Eye2`) 1000.0)
    (`KismetSystemLibrary.Delay` 0.5)
    (`PrimitiveComponent.SetCollisionEnabled` (`self.StatueEyesCollider`) "QueryOnly")
    (`KismetSystemLibrary.Delay` Duration)
    (`self.CloseStatueEyes`)))

(event `self.DeployCurse`
  (`/Engine/EditorBlueprintResources/StandardMacros.DoOnce` false
    (:`Completed`
      (`self.SetActorTickEnabled` false)
      (bind _asbp_curse_zone (cast `/Game/Blueprint/Actors/LDElements/Traps/BP_CurseZone` (`ChildActorComponent.ChildActor` (`self.CurseZone`))))
      (`CurseZone.Multicast_SetEnabled` _asbp_curse_zone true)
      (`ActorComponent.Activate` (`self.NS_CurseStatue`) true))))

(event `self.CloseStatueEyes`
  ; Open / Close Eyes
  (if (not (and (`self.CurseDeployed`) (`self.HasAuthority`)))
    (`parent.CloseStatueEyes`)
    (`LightComponent.SetIntensity` (`self.Eye1`) 0.0)
    (`LightComponent.SetIntensity` (`self.Eye2`) 0.0)
    (`PrimitiveComponent.SetCollisionEnabled` (`self.StatueEyesCollider`) "NoCollision")))

(event `self.StatueEyesCollider.OnComponentBeginOverlap`
  (params (OverlappedComponent :type "PrimitiveComponent Object Reference") (OtherActor :type "Actor Object Reference") (OtherComp :type "PrimitiveComponent Object Reference") (OtherBodyIndex :type Integer) (bFromSweep :type Boolean) (SweepResult :type "HitResult Structure (by ref)"))
  ; Collision
  (if (`self.ActorHasTag` OtherActor "Player")
    (`KismetArrayLibrary.Array_Add` (`self.PlayersInSight`) OtherActor)))

(event `self.ReceiveTick`
  (params (DeltaSeconds :type "Float (single-precision)"))
  (`parent.ReceiveTick` DeltaSeconds)
  (for _array_element (`self.PlayersInSight`)
    (if (> (`KismetMathLibrary.VSizeSquared` (`self.GetVelocity` _array_element)) 100.0)
      (`self.DeployCurse`))))

(event `self.StatueEyesCollider.OnComponentEndOverlap`
  (params (OverlappedComponent :type "PrimitiveComponent Object Reference") (OtherActor :type "Actor Object Reference") (OtherComp :type "PrimitiveComponent Object Reference") (OtherBodyIndex :type Integer))
  ; Collision
  (if (`self.ActorHasTag` OtherActor "Player")
    (`KismetArrayLibrary.Array_RemoveItem` (`self.PlayersInSight`) OtherActor)))

(fn `UserConstructionScript`)