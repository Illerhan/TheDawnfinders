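; Trap actor that can trigger a set of falling columns when the player character enters its overlap area.
; On overlap, a random roll against Probability decides whether it fires.
; When it fires, it destroys its Cube component, waits one second, then calls FallEvent on every column in ColumnList, printing a debug string for each.
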(event `self.ReceiveBeginPlay`)

(event `self.ReceiveActorBeginOverlap`
  (params (OtherActor :type "Actor Object Reference"))
  (cast `/Game/Blueprint/Actors/Player/BP_PlayerCharacter` OtherActor)
  (if (<= (`KismetMathLibrary.RandomFloatInRange` 0.0 100.0) (`self.Probability`))
    (`ActorComponent.K2_DestroyComponent` (`self.Cube`))
    (`KismetSystemLibrary.Delay` 1.0)
    (for _array_element (`self.ColumnList`)
      (`/Game/Blueprint/Actors/LDElements/Interactibles/BP_MiningItem_Child_Column.FallEvent` _array_element)
      (`KismetSystemLibrary.PrintString` "Hello"))))

(fn `UserConstructionScript`)