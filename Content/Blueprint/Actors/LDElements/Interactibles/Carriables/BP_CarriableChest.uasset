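; BP_CarriableChest is a carriable treasure chest that awards gold when put into a mule.
; On begin play it gives the mesh a slight random yaw and a dynamic outline overlay material, whose visibility toggles as the interact collider's overlaps begin and end.
; When put in a target that casts to BP_Mule, it adds its gold value through the mule's inventory component and triggers feedback, then calls the parent behavior.
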(event `self.InteractCollider.OnComponentBeginOverlap`
  (params (OverlappedComponent :type "PrimitiveComponent Object Reference") (OtherActor :type "Actor Object Reference") (OtherComp :type "PrimitiveComponent Object Reference") (OtherBodyIndex :type Integer) (bFromSweep :type Boolean) (SweepResult :type "HitResult Structure (by ref)"))
  ; OutlineOverlap
  (`/Engine/EditorBlueprintResources/StandardMacros.IsValid` (stale `self.ReceiveBeginPlay` _returnvalue)
    (:`Is Valid`
      (`MaterialInstanceDynamic.SetScalarParameterValue` (stale `self.ReceiveBeginPlay` _returnvalue) "IsVisible" 1.0))))

(event `self.InteractCollider.OnComponentEndOverlap`
  (params (OverlappedComponent :type "PrimitiveComponent Object Reference") (OtherActor :type "Actor Object Reference") (OtherComp :type "PrimitiveComponent Object Reference") (OtherBodyIndex :type Integer))
  ; OutlineOverlap
  (`/Engine/EditorBlueprintResources/StandardMacros.IsValid` (stale `self.ReceiveBeginPlay` _returnvalue)
    (:`Is Valid`
      (`MaterialInstanceDynamic.SetScalarParameterValue` (stale `self.ReceiveBeginPlay` _returnvalue) "IsVisible" 0.0))))

(event `self.ReceiveBeginPlay`
  (`SceneComponent.K2_SetRelativeRotation` (`self.StaticMesh`) (`KismetMathLibrary.MakeRotator` 0.0 0.0 (`KismetMathLibrary.RandomFloatInRange` -10.0 10.0)) false false)
  (bind _returnvalue (`KismetMaterialLibrary.CreateDynamicMaterialInstance` "/Game/Art/Materials/Instances/Instances-FXs/MI_OutlineOverlay_02.MI_OutlineOverlay_02"))
  (`MeshComponent.SetOverlayMaterial` (`self.StaticMesh`) _returnvalue))

(event `self.PutInTargetActor`
  (params (Actor :type "Actor Object Reference"))
  (bind _goldvalue (`self.GoldValue`))
  (`|ExecutionSequence`
    (:`then_0`
      (bind _asbp_mule (cast `/Game/Blueprint/Actors/Mule/BP_Mule` Actor))
      (`InventoryComponent.Server_AddGold` (`Mule.InventoryComponent` _asbp_mule) _goldvalue)
      (`/Game/Blueprint/Actors/Mule/BP_Mule.DoCarryableFeedback` _asbp_mule _goldvalue))
    (:`then_1`
      (`parent.PutInTargetActor` Actor))))

(fn `UserConstructionScript`
  (`parent.UserConstructionScript`))