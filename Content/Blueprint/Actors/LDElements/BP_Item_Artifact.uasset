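; Artifact level element that bobs in place until its chains are destroyed, then moves away and opens a gate.
; BeginPlay starts a ping-pong timeline that raises and lowers the root while balancing is enabled.
; CheckAllChainsState counts destroyed chains in ChainList, resetting on any intact one; a count of four triggers MoveArtifact and BPGate.
; MoveArtifact stops the bobbing and lerps the actor by the EndPosition offset on a second timeline.
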(event `self.ReceiveTick`
  (params (DeltaSeconds :type "Float (single-precision)")))

(event `CheckAllChainsState`
  (for _array_element (`self.ChainList`)
    (if (`/Game/Blueprint/Actors/LDElements/Interactibles/BP_DestuctibleChains.isDestroy` _array_element)
      (bind _result (`/Engine/EditorBlueprintResources/StandardMacros.IncrementInt` (`self.DestroyChainNumber`))
        (:`  `
          (if (== _result 4)
            (`self.MoveArtifact`)
            (`Doors.StartOpening` (`self.BP_Gate`)))))
      (else
        (set `self.DestroyChainNumber` 0)))))

(event `MoveArtifact`
  (set `self.isBalancingUpDown` false)
  (set `self.StartPosition` (`self.K2_GetActorLocation`))
  (set `self.EndPosition` (+ (`self.K2_GetActorLocation`) (`self.EndPosition`)))
  (`TimelineComponent.SetPlayRate` (`self.ArtifactTimeline`) (`self.SpeedMovement`))
  (bind (_direction _newtrack_0) (`Timeline|ArtifactTimeline`)
    (:`Update`
      (`self.K2_SetActorLocation` (`KismetMathLibrary.VLerp` (`self.StartPosition`) (`self.EndPosition`) _newtrack_0)))))

(event `self.ReceiveBeginPlay`
  (`parent.ReceiveBeginPlay`)
  (set `self.MeshPosStart` (`SceneComponent.K2_GetComponentLocation` (`self.Rooot`)))
  (set `self.MeshPosEnd` (+ (`SceneComponent.K2_GetComponentLocation` (`self.Rooot`)) (0.0 0.0 75.0)))
  (`TimelineComponent.SetPlayRate` (`self.ArtifactTimeline`) 0.001)
  (bind (_direction _newtrack_0) (`Timeline|Timeline_0` :!label _label)
    (:`Update`
      (if (`self.isBalancingUpDown`)
        (`SceneComponent.K2_SetWorldLocation` (`self.Rooot`) (`KismetMathLibrary.VLerp` (`self.MeshPosStart`) (`self.MeshPosEnd`) _newtrack_0) false false)))
    (:`Finished`
      (if (`self.isLooped`)
        (set `self.isLooped` false)
        (goto _label :!via `Reverse`)
        (else
          (set `self.isLooped` true)
          (goto _label))))))

(fn `UserConstructionScript`
  (`parent.UserConstructionScript`))