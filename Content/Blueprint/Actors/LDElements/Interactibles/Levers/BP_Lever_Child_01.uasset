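; Co-op lever interactible that fires once enough players hold it, with the required count derivable from living players.
; Players auto-move to the nearest free slot attached to the lever's socket, and an overlap toggles an outline overlay.
; Each new holder or death-count change rechecks the count, then multicasts the animation, attaches holders to slots and calls Interact.
; After a delay it releases them and disables the lever.
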(event `self.InteractCollider.OnComponentBeginOverlap`
  (params (OverlappedComponent :type "PrimitiveComponent Object Reference") (OtherActor :type "Actor Object Reference") (OtherComp :type "PrimitiveComponent Object Reference") (OtherBodyIndex :type Integer) (bFromSweep :type Boolean) (SweepResult :type "HitResult Structure (by ref)"))
  ; OutlineOverlap
  (`MaterialInstanceDynamic.SetScalarParameterValue` (stale `self.ReceiveBeginPlay` _returnvalue) "IsVisible" 1.0))

(event `self.InteractCollider.OnComponentEndOverlap`
  (params (OverlappedComponent :type "PrimitiveComponent Object Reference") (OtherActor :type "Actor Object Reference") (OtherComp :type "PrimitiveComponent Object Reference") (OtherBodyIndex :type Integer))
  ; OutlineOverlap
  (`MaterialInstanceDynamic.SetScalarParameterValue` (stale `self.ReceiveBeginPlay` _returnvalue) "IsVisible" 0.0))

(event `self.ReceiveBeginPlay`
  (bind _returnvalue (`KismetMaterialLibrary.CreateDynamicMaterialInstance` "/Game/Art/Materials/Instances/Instances-FXs/MI_OutlineOverlay_03.MI_OutlineOverlay_03"))
  (`MeshComponent.SetOverlayMaterial` (`self.Lever`) _returnvalue)
  (bind _output_get (set `self.PlayerPositions` (`|MakeArray` (`self.PlayerPos`) (`self.PlayerPos1`) (`self.PlayerPos2`) (`self.PlayerPos3`))))
  (for _ (range (`KismetArrayLibrary.Array_Length` _output_get))
    (`KismetArrayLibrary.Array_Add` (`self.UsedPositions`)))
  (`SceneComponent.K2_AttachToComponent` (`self.PlayerPos`) (`self.Lever`) "Socket" "KeepWorld" "KeepWorld" "KeepWorld" true)
  (`SceneComponent.K2_AttachToComponent` (`self.PlayerPos1`) (`self.Lever`) "Socket" "KeepWorld" "KeepWorld" "KeepWorld" true)
  (`SceneComponent.K2_AttachToComponent` (`self.PlayerPos2`) (`self.Lever`) "Socket" "KeepWorld" "KeepWorld" "KeepWorld" true)
  (`SceneComponent.K2_AttachToComponent` (`self.PlayerPos3`) (`self.Lever`) "Socket" "KeepWorld" "KeepWorld" "KeepWorld" true)
  (bind _asbp_custom_game_mode (cast `/Game/Blueprint/GameFramework/BP_CustomGameMode` (`GameplayStatics.GetGameMode`)))
  (add `/Game/Blueprint/GameFramework/BP_CustomGameMode.OnDeadCountChange` _asbp_custom_game_mode (delegate `VerifyUseLever`)))

(event `self.DoPlayerAutoMove`
  (params (Player :type "APlayerCharacter Object Reference"))
  (bind _usedpositions (`self.UsedPositions`))
  (bind _output (`|GetArrayItem` (`self.PlayerPositions`) (`self.PickedIndex`)))
  ; Go to lever
  (set `self.PickedIndex` 0)
  (set `self.MaxDist` 1000000.0)
  (for (_array_element _array_index) (`self.PlayerPositions`)
    (if (not (`|GetArrayItem` _usedpositions _array_index))
      (bind _returnvalue (`KismetMathLibrary.VSizeSquared` (- (`self.K2_GetActorLocation` Player) (`SceneComponent.K2_GetComponentLocation` _array_element))))
      (if (< _returnvalue (`self.MaxDist`))
        (set `self.PickedIndex` _array_index)
        (set `self.MaxDist` _returnvalue))))
  (`APlayerCharacter.StartAutoMoveCharacter` Player (`SceneComponent.K2_GetComponentLocation` _output) (`SceneComponent.K2_GetComponentRotation` _output) self)
  (`KismetArrayLibrary.Array_Set` _usedpositions (`self.PickedIndex`) true))

(event `VerifyUseLever`
  ; Reach lever + rotate lever
  (if (>= (`KismetArrayLibrary.Array_Length` (`self.PlayersHolding`)) (`self.NeededPlayerCount`)) :!label _label
    (`self.Multicast_PlayAnimation`)
    (for _array_element (`self.PlayersHolding`)
      (set `self.PickedIndex` 0)
      (set `self.MaxDist` 1000000.0)
      (for (_array_element_2 _array_index) (`self.PlayerPositions`)
        (bind _returnvalue (`KismetMathLibrary.VSizeSquared` (- (`self.K2_GetActorLocation` _array_element) (`SceneComponent.K2_GetComponentLocation` _array_element_2))))
        (if (< _returnvalue (`self.MaxDist`))
          (set `self.MaxDist` _returnvalue)
          (set `self.PickedIndex` _array_index)))
      (`/Game/Blueprint/Actors/Player/BP_PlayerCharacter.AttachPlayerToActor` _array_element (`|GetArrayItem` (`self.PlayerPositions`) (`self.PickedIndex`))))
    (`Interactible.Interact` (`|GetArrayItem` (`self.PlayersHolding`)))
    (`KismetSystemLibrary.Delay` (`self.InteractAnimDuration`))
    (for _array_element_3 (`self.PlayersHolding`)
      (`/Game/Blueprint/Actors/Player/BP_PlayerCharacter.UnattachPlayerFromActor` _array_element_3)
      (`APlayerCharacter.StopForceRotation` _array_element_3 0.0)
      (bind _interactioncomponent (`APlayerCharacter.InteractionComponent` _array_element_3))
      (`InteractionComponent.EndInteractAnimatiopn` _interactioncomponent)
      (`InteractionComponent.CancelInteraction` _interactioncomponent)
      (`PlayerInterface.SetCurrentPlayerState` _array_element_3 "None" true))
    (set `self.bCanBeUsed` false)))

(event `self.DoInteractionAnim`
  (params (Interactor :type "Actor Object Reference"))
  ; Reach lever + rotate lever
  (bind _asbp_player_character (cast `/Game/Blueprint/Actors/Player/BP_PlayerCharacter` Interactor))
  (`KismetArrayLibrary.Array_Add` (`self.PlayersHolding`) _asbp_player_character)
  (goto _label))

(event `Multicast_PlayAnimation`
  (bind _lever (`self.Lever`))
  (`SkeletalMeshComponent.SetPlayRate` _lever 1.0)
  (`SkeletalMeshComponent.Play` _lever false)
  (set `self.bAnimationIsActive` true))

(event `self.StopInteract`
  (params (Interactor :type "Actor Object Reference"))
  (if (not (`self.bAnimationIsActive`))
    (bind _asbp_player_character (cast `/Game/Blueprint/Actors/Player/BP_PlayerCharacter` Interactor))
    (`KismetArrayLibrary.Array_RemoveItem` (`self.PlayersHolding`) _asbp_player_character)
    (`/Engine/EditorBlueprintResources/StandardMacros.DecrementInt` (`self.CurrentInteractActorCount`)
      (:`  `
        (`InteractionComponent.EndInteractAnimatiopn` (`APlayerCharacter.InteractionComponent` _asbp_player_character))
        (set `self.PickedIndex` 0)
        (set `self.MaxDist` 1000000.0)
        (for (_array_element _array_index) (`self.PlayerPositions`)
          (bind _returnvalue (`KismetMathLibrary.VSizeSquared` (- (`self.K2_GetActorLocation` _asbp_player_character) (`SceneComponent.K2_GetComponentLocation` _array_element))))
          (if (< _returnvalue (`self.MaxDist`))
            (set `self.MaxDist` _returnvalue)
            (set `self.PickedIndex` _array_index)))
        (`KismetArrayLibrary.Array_Set` (`self.UsedPositions`) (`self.PickedIndex`))))))

(event `self.ActualiseNeededPlayerCount`
  (bind _asbp_custom_game_mode (cast `/Game/Blueprint/GameFramework/BP_CustomGameMode` (`GameplayStatics.GetGameMode`)))
  (set `self.NeededPlayerCount` (- (`KismetArrayLibrary.Array_Length` (`GameStateBase.PlayerArray` (`GameplayStatics.GetGameState`))) (`CustomGameMode.DeadPlayerCount` _asbp_custom_game_mode))))

(fn `UserConstructionScript`
  (`parent.UserConstructionScript`))