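; Player character for a multiplayer game: handles local setup, player name and color, spectating when dead, and damage feedback.
; Enhanced Input events, mostly gated by character state, drive movement, dodge and the interaction, inventory, item and stamina components.
; Actions emit server-side noise, shown through a loudness material; non-torch lights are counted to toggle health protection zones.
; Tick feeds position to a camera-cutout parameter collection; aimed throws preview with predicted-path spline meshes.
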(event `EnhancedInput|/Game/Inputs/Actions/IA_ClosePalanquin`
  (params (ActionValue :type Boolean) (ElapsedSeconds :type "Float (double-precision)") (TriggeredSeconds :type "Float (double-precision)") (InputAction :type "InputAction Object Reference" :default "/Game/Inputs/Actions/IA_ClosePalanquin.IA_ClosePalanquin"))
  (:`Triggered`
    (`KismetSystemLibrary.DelayUntilNextTick`)
    (bind _ashud_custom (cast `/Game/Blueprint/GameFramework/HUD_Custom` (`PlayerController.GetHUD` (`GameplayStatics.GetPlayerController` 0))))
    (bind _mainwidgetref (`/Game/Blueprint/GameFramework/HUD_Custom.MainWidgetRef` _ashud_custom))
    (bind _returnvalue (`MainWidget.GetIsInContainer` _mainwidgetref))
    (if _returnvalue
      (`MainWidget.CloseContainerInventory` _mainwidgetref))))

(event `PlayerInterface.DoCameraShake`
  (params (Intensity :type "Float (single-precision)"))
  (bind _returnvalue (`self.GetController`))
  ; Feedbacks
  (`/Engine/EditorBlueprintResources/StandardMacros.IsValid` _returnvalue
    (:`Is Valid`
      (if (`Controller.IsLocalController` _returnvalue)
        (switch `EPlayerState` (`self.CurrentState`)
          (:`None`
            _)
          (:`Running`
            _)
          (:`Carrying`
            _)
          (:`UsingEquipment`
            _)
          (:`Blocking`
            _)
          (:`Dodging`
            _)
          (:`Immobilized`
            _))
        (`LegacyCameraShake.StartLegacyCameraShake` (`PlayerController.PlayerCameraManager` (`GameplayStatics.GetPlayerController` 0)) "/Game/Blueprint/Others/BP_CameraShake.BP_CameraShake_C" Intensity)))))

(event `SpectateNext`
  (bind _returnvalue (+ (`self.CurrentSpectatingPlayer`) 1))
  (bind _playersarray (`/Game/Blueprint/GameFramework/BP_CustomGameState.PlayersArray` (`self.GameStateREF`)))
  ; Spectate Mode
  (if (> _returnvalue (+ (`KismetArrayLibrary.Array_Length` _playersarray) -1))
    (set `self.CurrentSpectatingPlayer` 0)
    (else
      (set `self.CurrentSpectatingPlayer` _returnvalue)))
  (`PlayerController.SetViewTargetWithBlend` (`GameplayStatics.GetPlayerController` 0) (`|GetArrayItem` _playersarray (`self.CurrentSpectatingPlayer`)) 0.0 "VTBlend_Linear" 0.0 false))

(event `self.OnLanded`
  (params (Hit :type "HitResult Structure (by ref)")))

(event `PlayerInterface.DoDamagePostProcess`
  (params (Speed :type "Float (single-precision)"))
  (bind _returnvalue (`self.GetController`))
  ; Feedbacks
  (`/Engine/EditorBlueprintResources/StandardMacros.IsValid` _returnvalue
    (:`Is Valid`
      (if (`Controller.IsLocalController` _returnvalue)
        (bind _outactors (`GameplayStatics.GetAllActorsWithTag` "PPDamage"))
        (if (> (`KismetArrayLibrary.Array_Length` _outactors) 0)
          ;;[0.15 0.04118 0.03982 0.5] Test vfx blood
          (bind _aspost_process_volume (cast `PostProcessVolume` (`|GetArrayItem` _outactors)))
          (switch `int` (`KismetMathLibrary.RandomIntegerInRange` 0 1)
            (:`0`
              (`ActorComponent.Activate` (`self.Blood1`) true)
              (bind (_direction _newtrack_0) (`Timeline|DamageTimeline` :!via `PlayFromStart` :!label _label)
                (:`Update`
                  (set `PostProcessVolume.BlendWeight` _newtrack_0 _aspost_process_volume))))
            (:`1`
              (`ActorComponent.Activate` (`self.Blood2`) true)
              (goto _label :!via `PlayFromStart`))))))))

(event `EnhancedInput|/Game/Inputs/Actions/IA_SpectateNext`
  (params (ActionValue :type Boolean) (ElapsedSeconds :type "Float (double-precision)") (TriggeredSeconds :type "Float (double-precision)") (InputAction :type "InputAction Object Reference" :default "/Game/Inputs/Actions/IA_SpectateNext.IA_SpectateNext"))
  ; Spectate
  (:`Started`
    (if (`|EnumEquality` (`self.CurrentState`) "Dead")
      (`self.SpectateNext`))))

(event `SpectatePrevious`
  (bind _returnvalue (- (`self.CurrentSpectatingPlayer`) 1))
  (bind _playersarray (`/Game/Blueprint/GameFramework/BP_CustomGameState.PlayersArray` (`self.GameStateREF`)))
  ; Spectate Mode
  (if (< _returnvalue 0)
    (set `self.CurrentSpectatingPlayer` (+ (`KismetArrayLibrary.Array_Length` _playersarray) -1))
    (else
      (set `self.CurrentSpectatingPlayer` _returnvalue)))
  (`PlayerController.SetViewTargetWithBlend` (`GameplayStatics.GetPlayerController` 0) (`|GetArrayItem` _playersarray (`self.CurrentSpectatingPlayer`)) 0.0 "VTBlend_Linear" 0.0 false))

(event `EnhancedInput|/Game/Inputs/Actions/IA_SpectatePrevious`
  (params (ActionValue :type Boolean) (ElapsedSeconds :type "Float (double-precision)") (TriggeredSeconds :type "Float (double-precision)") (InputAction :type "InputAction Object Reference" :default "/Game/Inputs/Actions/IA_SpectatePrevious.IA_SpectatePrevious"))
  ; Spectate
  (:`Started`
    (if (`|EnumEquality` (`self.CurrentState`) "Dead")
      (`self.SpectatePrevious`))))

(event `self.ReceiveBeginPlay`
  (bind _returnvalue (`GameplayStatics.GetPlayerController` 0))
  (bind _returnvalue_2 (`self.GetController`))
  (bind _returnvalue_3 (`self.GetController`))
  (bind _returnvalue_4 (`PlayerController.GetHUD` _returnvalue))
  ; Begin Play
  (`WidgetBlueprintLibrary.SetInputMode_GameOnly` (`GameplayStatics.GetPlayerController` 0))
  (`PlayerCameraComponent.InitialiseComponent` (`self.Camera Component`) (`self.SpringArm`))
  (`|ExecutionSequence`
    (:`then_0`
      (bind _asplayer_controller (cast `PlayerController` (`self.GetController`))
        (:`then`
          (bind _returnvalue_5 (pcsubsystem `EnhancedInputLocalPlayerSubsystem` _asplayer_controller))
          (`EnhancedInputSubsystemInterface.RemoveMappingContext` _returnvalue_5 "/Game/TopDown/Input/IMC_Default.IMC_Default" (struct))
          (`EnhancedInputSubsystemInterface.AddMappingContext` _returnvalue_5 "/Game/Inputs/IMC_Dawnfinders.IMC_Dawnfinders" 0 (struct)))
        (:`CastFailed`
          _))
      (cast `PlayerController` _returnvalue_2
        (:`then`
          (if (`Controller.IsLocalPlayerController` _returnvalue)
            (bind _ashud_custom (cast `/Game/Blueprint/GameFramework/HUD_Custom` _returnvalue_4))
            (`/Game/Blueprint/GameFramework/HUD_Custom.AddMainwidget` _ashud_custom)
            (`/Game/Blueprint/GameFramework/HUD_Custom.AddMuleWidget` _ashud_custom)
            (else
              (if (`self.HasAuthority`) :!label _label_2
                (bind _ashud_custom_2 (cast `/Game/Blueprint/GameFramework/HUD_Custom` _returnvalue_4))
                (`KismetSystemLibrary.Delay` 0.5)
                (`/Game/Blueprint/GameFramework/HUD_Custom.AddPlayerState` _ashud_custom_2 (`Controller.PlayerState` _returnvalue_2))))))
        (:`CastFailed`
          (goto _label_2))))
    (:`then_1`
      (bind _asbp_custom_game_state (cast `/Game/Blueprint/GameFramework/BP_CustomGameState` (`GameplayStatics.GetGameState`)))
      (bind _output_get (set `self.GameStateREF` _asbp_custom_game_state))
      (`/Game/Blueprint/GameFramework/BP_CustomGameState.AddPlayer` _output_get self))
    (:`then_2`
      (`parent.ReceiveBeginPlay`)
      (`SceneComponent.K2_AttachToComponent` (`self.WeaponMeshComponent`) (`self.Mesh`) "RightHandSocket" "SnapToTarget" "KeepRelative" "KeepRelative" true)
      (`SceneComponent.K2_AttachToComponent` (`self.WeaponCollisionPosRef`) (`self.Mesh`) "RightHandSocket" "SnapToTarget" "KeepRelative" "SnapToTarget" true)
      (`ActorComponent.Deactivate` (`self.NS_Poison`)))
    (:`then_3`
      (`/Engine/EditorBlueprintResources/StandardMacros.IsValid` _returnvalue_3
        (:`Is Valid`
          (if (not (`Controller.IsLocalController` _returnvalue_3))
            (`self.DisableInput` null :!label _label_3)
            (set `CharacterMovementComponent.bOrientRotationToMovement` true (`self.CharacterMovement`))))
        (:`Is Not Valid`
          (goto _label_3))))
    (:`then_4`
      (`self.SetupDynamicMaterials`))))

(event `RetryInitNames`
  (bind _playerstate (`self.PlayerState`))
  (bind _playerid (`PlayerState.PlayerId` _playerstate))
  (bind _aswbp_player_name (cast `/Game/UI/Widgets/WBP_PlayerName` (`WidgetComponent.GetUserWidgetObject` (`self.Name`)) :!label _label_4))
  (`/Engine/EditorBlueprintResources/StandardMacros.IsValid` _playerstate
    (:`Is Valid`
      (set `/Game/UI/Widgets/WBP_PlayerName.OwnerCharacter` self _aswbp_player_name)
      (set `TextBlock.Text` (`|FormatText` "Player {id}" _playerid) (`/Game/UI/Widgets/WBP_PlayerName.TextBlock_30` _aswbp_player_name))
      (switch `int` (mod _playerid 4)
        (:`0`
          (set `self.PlayerColor` (struct :`G` 1.0 :`B` 0.223508 :`A` 1.0)))
        (:`1`
          (set `self.PlayerColor` (struct :`G` 0.234899 :`B` 1.0 :`A` 1.0)))
        (:`2`
          (set `self.PlayerColor` (struct :`R` 1.0 :`B` 0.589239 :`A` 1.0)))
        (:`3`
          (set `self.PlayerColor` (struct :`R` 1.0 :`G` 0.933884 :`A` 1.0)))))
    (:`Is Not Valid`
      (`KismetSystemLibrary.K2_SetTimerDelegate` (delegate `RetryInitNames`) 0.2))))

(event `self.InitPlayerNames`
  (goto _label_4))

(event `EnhancedInput|/Game/Inputs/Actions/IA_Rotate`
  (params (ActionValue :type "Vector2D Structure") (ElapsedSeconds :type "Float (double-precision)") (TriggeredSeconds :type "Float (double-precision)") (InputAction :type "InputAction Object Reference" :default "/Game/Inputs/Actions/IA_Rotate.IA_Rotate"))
  (:`Triggered`
    (if (> (`KismetMathLibrary.VSize2D` ActionValue) 0.1)
      (`self.ForceRotation` (`KismetMathLibrary.Conv_Vector2DToVector` ActionValue))
      (else
        (set `self.bIsForcingRotation` false :!label _label_5))))
  (:`Canceled`
    (goto _label_5))
  (:`Completed`
    (goto _label_5)))

(event `EnhancedInput|/Game/Inputs/Actions/IA_Interact`
  (params (ActionValue :type Boolean) (ElapsedSeconds :type "Float (double-precision)") (TriggeredSeconds :type "Float (double-precision)") (InputAction :type "InputAction Object Reference" :default "/Game/Inputs/Actions/IA_Interact.IA_Interact"))
  (bind _interactioncomponent (`self.InteractionComponent`))
  (bind _currentstate (`self.CurrentState`))
  ; Interaction Input
  (:`Started`
    (switch `EPlayerState` _currentstate
      (:`None`
        _)
      (:`Running`
        _)
      (:`Carrying`
        _)
      (:`Immobilized`
        _)
      (:`Trapped`
        _)
      (:`Sneaking`
        _))
    (`InteractionComponent.StartInteract` _interactioncomponent))
  (:`Completed`
    (switch `EPlayerState` _currentstate
      (:`None`
        _)
      (:`Running`
        _)
      (:`Carrying`
        _)
      (:`Immobilized`
        _)
      (:`Trapped`
        _)
      (:`Sneaking`
        _))
    (`InteractionComponent.StopInteract` _interactioncomponent)))

(event `EnhancedInput|/Game/Inputs/Actions/IA_ChangeInventorySlot`
  (params (ActionValue :type "Float (double-precision)") (ElapsedSeconds :type "Float (double-precision)") (TriggeredSeconds :type "Float (double-precision)") (InputAction :type "InputAction Object Reference" :default "/Game/Inputs/Actions/IA_ChangeInventorySlot.IA_ChangeInventorySlot"))
  ; Inventory
  (:`Triggered`
    (`InventoryComponent.ChangeCurrentSlot` (`self.InventoryComponent`) (< ActionValue 0.0) -1)))

(event `EnhancedInput|/Game/Inputs/Actions/IA_Inventory`
  (params (ActionValue :type Boolean) (ElapsedSeconds :type "Float (double-precision)") (TriggeredSeconds :type "Float (double-precision)") (InputAction :type "InputAction Object Reference" :default "/Game/Inputs/Actions/IA_Inventory.IA_Inventory"))
  ; Inventory
  (:`Started`
    (switch `EPlayerState` (`self.CurrentState`)
      (:`None`
        _)
      (:`Running`
        _)
      (:`Carrying`
        _)
      (:`Fallen`
        _)
      (:`Sneaking`
        _))
    (`InventoryComponent.OpenInventory` (`self.InventoryComponent`)))
  (:`Canceled`
    (`InventoryComponent.CloseInventory` (`self.InventoryComponent`) :!label _label_6))
  (:`Completed`
    (goto _label_6)))

(event `EnhancedInput|/Game/Inputs/Actions/IA_Cancel`
  (params (ActionValue :type Boolean) (ElapsedSeconds :type "Float (double-precision)") (TriggeredSeconds :type "Float (double-precision)") (InputAction :type "InputAction Object Reference" :default "/Game/Inputs/Actions/IA_Cancel.IA_Cancel"))
  ; Interaction Input
  (:`Triggered`
    (`KismetSystemLibrary.DelayUntilNextTick`)
    (`InteractionComponent.CancelInteraction` (`self.InteractionComponent`))))

(event `EnhancedInput|/Game/Inputs/Actions/IA_Dodge`
  (params (ActionValue :type Boolean) (ElapsedSeconds :type "Float (double-precision)") (TriggeredSeconds :type "Float (double-precision)") (InputAction :type "InputAction Object Reference" :default "/Game/Inputs/Actions/IA_Dodge.IA_Dodge"))
  (bind _staminacomponent (`self.StaminaComponent`))
  ; Dodge
  (:`Triggered`
    (switch `EPlayerState` (`self.CurrentState`)
      (:`None`
        _)
      (:`Running`
        _)
      (:`Sneaking`
        _))
    (bind _returnvalue (`StaminaComponent.VerifyHasStamina` (`self.StaminaComponent`)))
    (if _returnvalue
      (`StaminaComponent.UseStamina` _staminacomponent (`StaminaComponent.StaminaConsumptionDodge` _staminacomponent))
      (`self.StartDodge`)
      (`self.PlayMontage` "/Game/Art/Animations/Players/Montages/AM_Dawnfinder_Male_Dodge.AM_Dawnfinder_Male_Dodge" 1.0)
      (`PlayerInterface.PlaySoundOnServer` "Dodge" (`PlayerData.DodgeSoundRange` (`self.PlayerConfig`)) 0.8)
      (`HealthComponent.StartInvincibilityFrames` (`self.HealthComponent`) (`PlayerData.DodgeInvincibilityDuration` (`self.PlayerConfig`))))))

(event `EnhancedInput|/Game/Inputs/Actions/IA_Drop`
  (params (ActionValue :type Boolean) (ElapsedSeconds :type "Float (double-precision)") (TriggeredSeconds :type "Float (double-precision)") (InputAction :type "InputAction Object Reference" :default "/Game/Inputs/Actions/IA_Drop.IA_Drop"))
  ; Inventory
  (:`Started`
    (switch `EPlayerState` (`self.CurrentState`)
      (:`None`
        (bind _returnvalue (`InventoryComponent.GetIsOpened` (`self.InventoryComponent`) :!label _label_7))
        (if _returnvalue
          (`InventoryComponent.Throw` (`self.InventoryComponent`))))
      (:`Running`
        (goto _label_7))
      (:`Carrying`
        (`PlayerInterface.EndCarryHeavyItem` null))
      (:`Fallen`
        (goto _label_7))
      (:`Sneaking`
        (goto _label_7)))))

(event `self.BP_OnMontageEnded`
  (params (Montage :type "AnimMontage Object Reference") (bInterrupted :type Boolean))
  ; Dodge
  (switch `EPlayerState` (`self.CurrentState`)
    (:`Dodging`
      (`self.EndDodge`))))

(event `EnhancedInput|/Game/Inputs/Actions/IA_InventorySelect`
  (params (ActionValue :type "Vector2D Structure") (ElapsedSeconds :type "Float (double-precision)") (TriggeredSeconds :type "Float (double-precision)") (InputAction :type "InputAction Object Reference" :default "/Game/Inputs/Actions/IA_InventorySelect.IA_InventorySelect"))
  (bind (_x _y) (`KismetMathLibrary.BreakVector2D` ActionValue))
  ; Inventory
  (:`Triggered`
    (if (> (`KismetMathLibrary.VSize2D` ActionValue) 0.9)
      (`InventoryComponent.SelectSlotByAngle` (`self.InventoryComponent`) (`KismetMathLibrary.FTrunc` (mod (+ (`KismetMathLibrary.DegAtan2` _y _x) 450.0) 360.0))))))

(event `EnhancedInput|/Game/Inputs/Actions/IA_QuickChangeLeft`
  (params (ActionValue :type "Float (double-precision)") (ElapsedSeconds :type "Float (double-precision)") (TriggeredSeconds :type "Float (double-precision)") (InputAction :type "InputAction Object Reference" :default "/Game/Inputs/Actions/IA_QuickChangeLeft.IA_QuickChangeLeft"))
  ; Inventory
  (:`Started`
    (switch `EPlayerState` (`self.CurrentState`)
      (:`None`
        _)
      (:`Running`
        _)
      (:`Fallen`
        _))
    (`InventoryComponent.QuickChange` (`self.InventoryComponent`) false)))

(event `EnhancedInput|/Game/Inputs/Actions/IA_QuickChangeRight`
  (params (ActionValue :type "Float (double-precision)") (ElapsedSeconds :type "Float (double-precision)") (TriggeredSeconds :type "Float (double-precision)") (InputAction :type "InputAction Object Reference" :default "/Game/Inputs/Actions/IA_QuickChangeRight.IA_QuickChangeRight"))
  ; Inventory
  (:`Started`
    (switch `EPlayerState` (`self.CurrentState`)
      (:`None`
        _)
      (:`Running`
        _)
      (:`Fallen`
        _))
    (`InventoryComponent.QuickChange` (`self.InventoryComponent`) true)))

(event `SetupDynamicMaterials`
  (bind _returnvalue (`KismetMaterialLibrary.CreateDynamicMaterialInstance` "/Game/Art/Materials/Masters/MM_VFXSoundPlayer.MM_VFXSoundPlayer"))
  (bind _output_get (set `self.Dyn Mat Soundwave` _returnvalue))
  (`PrimitiveComponent.SetMaterial` (`self.SM_Circle_SoundPlayer`) 0 _output_get)
  (bind _returnvalue_2 (`KismetMaterialLibrary.CreateDynamicMaterialInstance` (`PrimitiveComponent.GetMaterial` (`self.Mesh`) 0)))
  (set `self.DynMatChara` _returnvalue_2)
  (`PrimitiveComponent.SetMaterial` (`self.Mesh`) 0 (`self.DynMatChara`))
  (`MaterialInstanceDynamic.SetScalarParameterValue` (`self.DynMatChara`) "Color Intensity" 0.0))

(event `self.ReceiveTick`
  (params (DeltaSeconds :type "Float (single-precision)"))
  ; Get Position For Cam Cutout
  (`KismetMaterialLibrary.SetVectorParameterValue` "/Game/Art/Materials/CollectionParameter/MPC_CameraCutout.MPC_CameraCutout" "PlayerPosition" (`KismetMathLibrary.Conv_VectorToLinearColor` (`self.K2_GetActorLocation`)))
  ; Soundwave
  (`parent.ReceiveTick` DeltaSeconds)
  (bind _output_get (set `self.Smoothed Loudness` (`KismetMathLibrary.FInterpTo` (`self.Smoothed Loudness`) (`self.UILoudness`) DeltaSeconds 2.0)))
  (`MaterialInstanceDynamic.SetScalarParameterValue` (`self.Dyn Mat Soundwave`) "Loudness" _output_get)
  (`/Engine/EditorBlueprintResources/ActorMacros.Switch Has Authority`
    (:`Authority`
      (if (not (> (`KismetMathLibrary.VSizeSquared` (`self.CurrentPlayerInput`)) 0.1))
        (`PlayerInterface.PlaySoundOnServer` "None" (`KismetMathLibrary.FClamp` (- (`SphereComponent.SphereRadius` (`self.NoiseZone`)) (* (`GameplayStatics.GetWorldDeltaSeconds`) 1500.0)) 0.0 5000.0))))))

(event `EnhancedInput|/Game/Inputs/Actions/IA_Lantern`
  (params (ActionValue :type Boolean) (ElapsedSeconds :type "Float (double-precision)") (TriggeredSeconds :type "Float (double-precision)") (InputAction :type "InputAction Object Reference" :default "/Game/Inputs/Actions/IA_Lantern.IA_Lantern"))
  ; Mule
  (:`Started`
    (bind _aspc_custom (cast `/Game/Blueprint/GameFramework/PC_Custom` (`self.GetController`)))
    (`CustomPlayerController.Server_CallMule` _aspc_custom self)))

(event `self.Light On`
  (params (isTorchLight :type Boolean))
  ;[0.4844 0.1852 0 0.5] Fog of War / Curse
  (if (not isTorchLight)
    (bind _result (`/Engine/EditorBlueprintResources/StandardMacros.IncrementInt` (`self.NumberOfLights`) :!label _label_8)
      (:`  `
        (if (== _result 1)
          (`HealthComponent.AddProtectionZone` (`self.HealthComponent`)))))))

(event `self.Palanquin Light On`
  ;[0.4844 0.1852 0 0.5] Fog of War / Curse
  (goto _label_8))

(event `self.Light Off`
  (params (isTorchLight :type Boolean))
  ;[0.4844 0.1852 0 0.5] Fog of War / Curse
  (if (not isTorchLight)
    (bind _output_get (set `self.NumberOfLights` (`KismetMathLibrary.Max` (- (`self.NumberOfLights`) 1)) :!label _label_9))
    (if (<= _output_get 0)
      (`HealthComponent.RemoveProtectionZone` (`self.HealthComponent`)))))

(event `self.Palanquin Light Off`
  ;[0.4844 0.1852 0 0.5] Fog of War / Curse
  (goto _label_9))

(event `EnhancedInput|/Game/Inputs/Actions/IA_LightAttack`
  (params (ActionValue :type Boolean) (ElapsedSeconds :type "Float (double-precision)") (TriggeredSeconds :type "Float (double-precision)") (InputAction :type "InputAction Object Reference" :default "/Game/Inputs/Actions/IA_LightAttack.IA_LightAttack"))
  ; Weapons Attacks
  (:`Triggered`
    (switch `EPlayerState` (`self.CurrentState`)
      (:`None`
        _)
      (:`Running`
        _)
      (:`Sneaking`
        _))
    (`ItemComponent.DoLightAttack` (`self.ItemComponent`))))

(event `EnhancedInput|/Game/Inputs/Actions/IA_ItemSecondaryAction`
  (params (ActionValue :type Boolean) (ElapsedSeconds :type "Float (double-precision)") (TriggeredSeconds :type "Float (double-precision)") (InputAction :type "InputAction Object Reference" :default "/Game/Inputs/Actions/IA_ItemSecondaryAction.IA_ItemSecondaryAction"))
  (bind _itemcomponent (`self.ItemComponent`))
  (bind _currentstate (`self.CurrentState`))
  ; Secondary Action
  (:`Started`
    (switch `EPlayerState` _currentstate
      (:`None`
        _)
      (:`Running`
        _)
      (:`Blocking`
        _)
      (:`Sneaking`
        _))
    (`ItemComponent.DoSecondaryAction` _itemcomponent))
  (:`Canceled`
    (switch `EPlayerState` _currentstate :!label _label
      (:`None`
        _)
      (:`Running`
        _)
      (:`UsingEquipment`
        _)
      (:`Blocking`
        _)
      (:`Sneaking`
        _))
    (`ItemComponent.StopSecondaryAction` _itemcomponent)
    (`self.ClearThrowPreview`))
  (:`Completed`
    (goto _label)))

(event `EnhancedInput|/Game/Inputs/Actions/IA_HeavyAttack`
  (params (ActionValue :type Boolean) (ElapsedSeconds :type "Float (double-precision)") (TriggeredSeconds :type "Float (double-precision)") (InputAction :type "InputAction Object Reference" :default "/Game/Inputs/Actions/IA_HeavyAttack.IA_HeavyAttack"))
  ; Weapons Attacks
  (:`Triggered`
    (switch `EPlayerState` (`self.CurrentState`)
      (:`None`
        _)
      (:`Running`
        _)
      (:`Sneaking`
        _))
    (`ItemComponent.DoHeavyAttack` (`self.ItemComponent`))))

(event `EnhancedInput|/Game/Inputs/Actions/IA_ItemMainAction`
  (params (ActionValue :type Boolean) (ElapsedSeconds :type "Float (double-precision)") (TriggeredSeconds :type "Float (double-precision)") (InputAction :type "InputAction Object Reference" :default "/Game/Inputs/Actions/IA_ItemMainAction.IA_ItemMainAction"))
  (bind _currentstate (`self.CurrentState`))
  (bind _itemcomponent (`self.ItemComponent`))
  ; Main Action
  (:`Started`
    (switch `EPlayerState` _currentstate
      (:`None`
        _)
      (:`Running`
        _)
      (:`UsingEquipment`
        _)
      (:`Sneaking`
        _))
    (`ItemComponent.DoMainAction` _itemcomponent)
    (`self.ClearThrowPreview`))
  (:`Canceled`
    (switch `EPlayerState` _currentstate :!label _label_2
      (:`None`
        _)
      (:`Running`
        _)
      (:`UsingEquipment`
        _)
      (:`Sneaking`
        _))
    (`ItemComponent.StopMainAction` _itemcomponent))
  (:`Completed`
    (goto _label_2)))

(event `self.BP_OnMontageNotifyBegin`
  (params (NotifyName :type Name))
  (bind _itemcomponent (`self.ItemComponent`))
  ; Do Attack Collision
  (`ItemComponent.DoAttackInertia` _itemcomponent)
  (set `self.TempInt` 0)
  (if (< (`self.TempInt`) 10) :!label _label_3
    (`ItemComponent.DoAttackCollision` _itemcomponent)
    (`/Engine/EditorBlueprintResources/StandardMacros.IncrementInt` (`self.TempInt`)
      (:`  `
        (`KismetSystemLibrary.Delay` 0.01)
        (goto _label_3)))))

(event `self.DisplayThrowPreview`
  (params (Direction :type "Vector Structure") (Strength :type "Float (single-precision)"))
  (bind _returnvalue (`self.K2_GetActorLocation`))
  (bind _splinemeshcomponents (`self.SplineMeshComponents`))
  (bind _spline (`self.Spline`))
  ; Throw Preview
  (`self.ClearThrowPreview`)
  (if (`self.bIsForcingRotation`)
    (bind _predictresult (`GameplayStatics.Blueprint_PredictProjectilePath_Advanced` (make `PredictProjectilePathParams` (`SceneComponent.K2_GetComponentLocation` (`self.ThrowStartPosRef`)) (* Direction Strength) true 5.0 1.5 true "ECC_PhysicsBody" _ _ 25.0)))
    (for _array_element (`.PathData` (break `PredictProjectilePathResult` _predictresult))
      (`SplineComponent.AddSplinePoint` _spline (`.Location` (break `PredictProjectilePathPointData` _array_element)) "World" true))
    (for _index (range 1 (+ (`SplineComponent.GetNumberOfSplinePoints` _spline) 1))
      (bind _returnvalue_2 (`AddComponent|NODE_AddSplineMeshComponent-0` :`RelativeTransform` (`KismetMathLibrary.MakeTransform` (0.0 0.0 0.0) (* (`self.CurrentForcedRotation`) -1.0))))
      (bind _returnvalue_3 (`KismetArrayLibrary.Array_Add` _splinemeshcomponents _returnvalue_2))
      (bind (_location _tangent) (`SplineComponent.GetLocationAndTangentAtSplinePoint` _spline _index "World"))
      (bind (_location_2 _tangent_2) (`SplineComponent.GetLocationAndTangentAtSplinePoint` _spline (+ _index 1) "World"))
      (`SplineMeshComponent.SetStartAndEnd` (`|GetArrayItem` _splinemeshcomponents _returnvalue_3) (- _location _returnvalue) _tangent (- (`KismetMathLibrary.VLerp` _location _location_2 0.5) _returnvalue) (`KismetMathLibrary.VLerp` _tangent _tangent_2 0.5) true))))

(event `EnhancedInput|/Game/Inputs/Actions/IA_Reload`
  (params (ActionValue :type Boolean) (ElapsedSeconds :type "Float (double-precision)") (TriggeredSeconds :type "Float (double-precision)") (InputAction :type "InputAction Object Reference" :default "/Game/Inputs/Actions/IA_Reload.IA_Reload"))
  (:`Triggered`
    (`ItemComponent.Reload` (`self.ItemComponent`))))

(event `ClearThrowPreview`
  (bind _splinemeshcomponents (`self.SplineMeshComponents`))
  ; Throw Preview
  (`SplineComponent.ClearSplinePoints` (`self.Spline`) true)
  (`ActorComponent.K2_DestroyComponent` _splinemeshcomponents)
  (`KismetArrayLibrary.Array_Clear` _splinemeshcomponents))

(event `EnhancedInput|/Game/Inputs/Actions/IA_Move`
  (params (ActionValue :type "Vector2D Structure") (ElapsedSeconds :type "Float (double-precision)") (TriggeredSeconds :type "Float (double-precision)") (InputAction :type "InputAction Object Reference" :default "/Game/Inputs/Actions/IA_Move.IA_Move"))
  ; Main Movement Input
  (:`Triggered`
    (`self.MoveCharacter` ActionValue :!label _label)
    (if (> (`KismetMathLibrary.VSizeSquared` (`self.CurrentPlayerInput`)) 0.1)
      (switch `EPlayerState` (`self.CurrentState`)
        (:`None`
          (`PlayerInterface.PlaySoundOnServer` "Walk" (`PlayerData.WalkSoundRange` (`self.PlayerConfig`)) 0.3))
        (:`Running`
          (`PlayerInterface.PlaySoundOnServer` "Run" (`PlayerData.RunSoundRange` (`self.PlayerConfig`)) 0.8))
        (:`Sneaking`
          (`PlayerInterface.PlaySoundOnServer` "Sneak" (`PlayerData.SneakSoundRange` (`self.PlayerConfig`)) 0.1)))))
  (:`Ongoing`
    (goto _label))
  (:`Canceled`
    (goto _label))
  (:`Completed`
    (goto _label)))

(event `EnhancedInput|/Game/Inputs/Actions/IA_Run`
  (params (ActionValue :type Boolean) (ElapsedSeconds :type "Float (double-precision)") (TriggeredSeconds :type "Float (double-precision)") (InputAction :type "InputAction Object Reference" :default "/Game/Inputs/Actions/IA_Run.IA_Run"))
  (bind _staminacomponent (`self.StaminaComponent`))
  (bind _currentstate (`self.CurrentState`))
  ; Run
  (:`Triggered`
    (if (> (`KismetMathLibrary.VSizeSquared` (`self.CurrentPlayerInput`)) 0.5)
      (switch `EPlayerState` _currentstate
        (:`None`
          (bind _returnvalue (`StaminaComponent.VerifyHasStamina` (`self.StaminaComponent`) :!label _label_2))
          (if _returnvalue
            (`self.ManageRun` true)
            (`StaminaComponent.UseStamina` _staminacomponent (* (`GameplayStatics.GetWorldDeltaSeconds`) (`StaminaComponent.StaminaConsumptionRun` _staminacomponent)))
            (`StaminaComponent.UseStamina` (`self.StaminaComponent`) (* (`GameplayStatics.GetWorldDeltaSeconds`) (`StaminaComponent.StaminaConsumptionRun` _staminacomponent)))
            (else
              (`self.ManageRun` false :!label _label_3))))
        (:`Running`
          (goto _label_2))
        (:`Blocking`
          (goto _label_3))
        (:`Sneaking`
          (goto _label_2)))))
  (:`Canceled`
    (switch `EPlayerState` _currentstate :!label _label_4
      (:`None`
        (goto _label_3))
      (:`Running`
        (goto _label_3))))
  (:`Completed`
    (goto _label_4)))

(event `EnhancedInput|/Game/Inputs/Actions/IA_Sneak`
  (params (ActionValue :type Boolean) (ElapsedSeconds :type "Float (double-precision)") (TriggeredSeconds :type "Float (double-precision)") (InputAction :type "InputAction Object Reference" :default "/Game/Inputs/Actions/IA_Sneak.IA_Sneak"))
  ; Sneak
  (:`Started`
    (switch `EPlayerState` (`self.CurrentState`)
      (:`None`
        (`PlayerInterface.RequestStateChange` "Sneaking" :!label _label_5))
      (:`Running`
        (goto _label_5))
      (:`Sneaking`
        (`PlayerInterface.SetCurrentPlayerState` "None")))))

(fn `OnRep_NumberOfLights`)

(fn `OnRep_PlayerColor`
  (bind _aswbp_player_name (cast `/Game/UI/Widgets/WBP_PlayerName` (`WidgetComponent.GetUserWidgetObject` (`self.Name`))))
  (`TextBlock.SetColorAndOpacity` (`/Game/UI/Widgets/WBP_PlayerName.TextBlock_30` _aswbp_player_name) (make `SlateColor` (`self.PlayerColor`))))

(fn `UserConstructionScript`
  ; Get Position For Cam Cutout
  (`KismetMaterialLibrary.SetVectorParameterValue` "/Game/Art/Materials/CollectionParameter/MPC_CameraCutout.MPC_CameraCutout" "PlayerPosition" (`KismetMathLibrary.Conv_VectorToLinearColor` (`self.K2_GetActorLocation`))))