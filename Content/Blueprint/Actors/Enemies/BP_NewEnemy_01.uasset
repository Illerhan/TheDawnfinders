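; Enemy that wanders around its spawn point, randomly pauses to search with an enlarged detection range, and reacts to BP_Noise overlaps.
; A first noise makes it suspicious, turning it to search; another during the suspicion timer triggers combat and alerts nearby enemies and crystallized ones.
; Timelines drive wandering and search feedback, Tick lerps toward the noise target, and materials show state.
; Hallucinated instances vanish near the player; player damage logic is unconnected.
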(event `self.ReceiveBeginPlay`
  (bind _returnvalue (`GameplayStatics.GetActorOfClass` "/Game/Blueprint/Actors/Player/BP_PlayerCharacter.BP_PlayerCharacter_C"))
  (set `self.Player` _returnvalue)
  (set `self.StartPos` (`self.K2_GetActorLocation`))
  (`self.Move`)
  (`SceneComponent.SetRelativeScale3D` (`self.DetectionRange`) (`KismetMathLibrary.Conv_DoubleToVector` (`self.BaseDetectionRadius`))))

(event `SelectRandomAction`
  (`KismetSystemLibrary.Delay` (`KismetMathLibrary.RandomFloatInRange` (`self.MinWaitingTime`) (`self.MaxWaitingTime`)))
  (if (`self.IsInCombat`)
    _
    (elif (<= (`KismetMathLibrary.RandomFloat`) (`self.SearchProba`))
      (`self.Search`)
      (else
        (`self.Move`)))))

(event `Move`
  (bind (_movetarget_x _movetarget_y) (`KismetMathLibrary.BreakVector` (`self.MoveTarget`)))
  (bind (_startmovepos_x _startmovepos_y) (`KismetMathLibrary.BreakVector` (`self.StartMovePos`)))
  (if (> (`self.SuspiciousTimer`) 0.0)
    _
    (else
      _))
  (`self.Change Material` 0)
  (set `self.MoveTarget` (+ (`self.StartPos`) (`KismetMathLibrary.ClampVectorSize` (* (+ (* (`self.GetActorForwardVector`) (`KismetMathLibrary.RandomFloatInRange` -1.0 1.0)) (* (`KismetMathLibrary.RandomFloatInRange` -1.0 1.0) (`self.GetActorRightVector`))) (`self.MaxDistanceMove`)) (`self.MinDistanceMove`) (`self.MaxDistanceMove`))))
  (set `self.StartMovePos` (`self.K2_GetActorLocation`))
  (`TimelineComponent.SetPlayRate` (`self.MoveTimeline`) (/ 1.0 (* (/ 1.0 (`self.MoveSpeed`)) (`KismetMathLibrary.Vector_Distance` (`self.StartMovePos`) (`self.MoveTarget`)))))
  (`self.K2_SetActorRotation` (`KismetMathLibrary.ComposeRotators` (`KismetMathLibrary.FindLookAtRotation` (`KismetMathLibrary.MakeVector` _startmovepos_x _startmovepos_y) (`KismetMathLibrary.MakeVector` _movetarget_x _movetarget_y)) (struct :`Yaw` -90.0)))
  (bind (_direction _alpha) (`Timeline|MoveTimeline` :!via `PlayFromStart`)
    (:`Update`
      (`self.K2_SetActorLocation` (`KismetMathLibrary.VLerp` (`self.StartMovePos`) (`self.MoveTarget`) _alpha)))
    (:`Finished`
      (`self.SelectRandomAction`))))

(event `SearchFeedback`
  (bind (_direction _alpha) (`Timeline|Timeline` :!via `PlayFromStart`)
    (:`Update`
      (`SceneComponent.SetWorldScale3D` (`self.Plane`) (`KismetMathLibrary.Conv_DoubleToVector` (* _alpha (`self.SearchDetectionRadius`)))))))

(event `Search`
  (if (> (`self.SuspiciousTimer`) 0.0)
    _
    (else
      _))
  (`self.Change Material` 1)
  (`KismetSystemLibrary.Delay` 1.0)
  (`SceneComponent.SetRelativeScale3D` (`self.DetectionRange`) (`KismetMathLibrary.Conv_DoubleToVector` (`self.SearchDetectionRadius`)))
  (`self.SearchFeedback`)
  (`KismetSystemLibrary.Delay` (`self.SearchTime`))
  (`SceneComponent.SetRelativeScale3D` (`self.DetectionRange`) (`KismetMathLibrary.Conv_DoubleToVector` (`self.BaseDetectionRadius`)))
  (if (not (`self.IsInCombat`))
    (`self.Move`)))

(event `self.ReceiveActorBeginOverlap`
  (params (OtherActor :type "Actor Object Reference"))
  (bind _asbp_noise (cast `/Game/Blueprint/Actors/BP_Noise` OtherActor))
  (if (<= (`self.SuspiciousCooldown`) 0.0)
    (`TimelineComponent.Stop` (`self.MoveTimeline`))
    (if (> (`self.SuspiciousTimer`) 0.0)
      (`self.Alert` _asbp_noise)
      (else
        (`self.Suspect` (`self.K2_GetActorLocation` _asbp_noise))
        (set `self.SuspiciousCooldown` 1.5)))))

(event `self.ReceiveTick`
  (params (DeltaSeconds :type "Float (single-precision)"))
  (bind (_returnvalue_x _returnvalue_y) (`KismetMathLibrary.BreakVector` (`self.K2_GetActorLocation`)))
  (bind (_returnvalue_x_2 _returnvalue_y_2) (`KismetMathLibrary.BreakVector` (`self.K2_GetActorLocation` (`self.Target`))))
  (`self.CheckForHallucination`)
  (set `self.SuspiciousCooldown` (- (`self.SuspiciousCooldown`) DeltaSeconds))
  (bind _output_get (set `self.SuspiciousTimer` (- (`self.SuspiciousTimer`) DeltaSeconds)))
  (if (<= _output_get 0.0)
    (if (`self.isSuspicious`)
      (set `self.isSuspicious` false)
      (set `self.SearchProba` (/ (`self.SearchProba`) 2.0))
      (`self.Change Suspect Material` false)
      (if (`self.IsInCombat`) :!label _label
        (`self.K2_SetActorLocation` (`KismetMathLibrary.VLerp` (`self.K2_GetActorLocation`) (`self.K2_GetActorLocation` (`self.Target`)) 0.01))
        (`self.K2_SetActorRotation` (`KismetMathLibrary.ComposeRotators` (`KismetMathLibrary.FindLookAtRotation` (`KismetMathLibrary.MakeVector` _returnvalue_x _returnvalue_y) (`KismetMathLibrary.MakeVector` _returnvalue_x_2 _returnvalue_y_2)) (struct :`Yaw` -90.0)))))
    (else
      (goto _label))))

(event `Suspect`
  (params (DetectedNoiseLocation :type "Vector Structure"))
  (bind (_returnvalue_x _returnvalue_y) (`KismetMathLibrary.BreakVector` (`self.K2_GetActorLocation`)))
  (set `self.isSuspicious` true)
  (`self.Change Material` 2)
  (`self.Change Suspect Material` true)
  (`self.K2_SetActorRotation` (`KismetMathLibrary.ComposeRotators` (`KismetMathLibrary.FindLookAtRotation` (`KismetMathLibrary.MakeVector` _returnvalue_x _returnvalue_y) (`KismetMathLibrary.MakeVector` DetectedNoiseLocation_X DetectedNoiseLocation_Y)) (struct :`Yaw` -90.0)))
  (set `self.SuspiciousTimer` (`self.SuspiciousTime`))
  (`self.Search`)
  (set `self.SearchProba` (* (`self.SearchProba`) 2.0)))

(event `Alert`
  (params (TargetActor :type "Actor Object Reference") (IsAlertedByOther :type Boolean))
  (`self.Change Material` 3)
  (set `self.IsInCombat` true)
  (bind _output_get (set `self.Target` TargetActor))
  (if (not IsAlertedByOther)
    (`KismetSystemLibrary.Delay` 1.0)
    (`|ExecutionSequence`
      (:`then_0`
        (bind _outactors (`GameplayStatics.GetAllActorsOfClass` "BP_NewEnemy_01_C"))
        (for _array_element _outactors
          (if (<= (`KismetMathLibrary.Vector_Distance` (`self.K2_GetActorLocation` _array_element) (`self.K2_GetActorLocation`)) (`self.AlertRadius`))
            (`self.Alert` _array_element _output_get true))))
      (:`then_1`
        (bind _outactors_2 (`GameplayStatics.GetAllActorsOfClass` "/Game/Blueprint/Actors/Enemies/BP_NewCrystallized_02.BP_NewCrystallized_02_C"))
        (for _array_element_2 _outactors_2
          (if (<= (`KismetMathLibrary.Vector_Distance` (`self.K2_GetActorLocation` _array_element_2) (`self.K2_GetActorLocation`)) (`self.AlertRadius`))
            (`/Game/Blueprint/Actors/Enemies/BP_NewCrystallized_02.Alert` _array_element_2 _output_get true)))))))

(event `CheckForHallucination`
  (if (`self.isHallucinated`)
    (if (<= (`KismetMathLibrary.Vector_Distance` (`self.K2_GetActorLocation`) (`self.K2_GetActorLocation` (`self.Player`))) 500.0)
      (`self.K2_DestroyActor`))))

(fn `Change Material`
  (params (Index :type Integer))
  (`PrimitiveComponent.SetMaterial` (`self.Cube`) 0 (`|GetArrayItem` (`self.Materials`) Index)))

(fn `Change Suspect Material`
  (params (Activate :type Boolean))
  (bind _returnvalue (select `bool` Activate :`false` "/Game/Art/PlaceHolder/Materials/M_EnemyMove.M_EnemyMove" :`true` "/Game/Art/PlaceHolder/Materials/M_EnemySuspect.M_EnemySuspect" :!type "MaterialInterface Object Reference"))
  (`PrimitiveComponent.SetMaterial` (`self.Cube1`) 0 _returnvalue)
  (`PrimitiveComponent.SetMaterial` (`self.Cube2`) 0 _returnvalue))

(fn `UserConstructionScript`)