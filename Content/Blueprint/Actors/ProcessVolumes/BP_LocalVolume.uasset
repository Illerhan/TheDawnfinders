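; BP_LocalVolume is a spherical proximity volume that reports a weight, based on the player's distance, to a handler actor.
; SetHandler assigns the handler and index, and BeginPlay finds the player pawn with delayed retries.
; Each Tick maps normalized squared distance through a curve into a clamped weight, forcing zero at exactly zero distance.
; The construction script scales the sphere to MaxDistance, which BeginPlay squares to avoid square roots.
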(event `SetHandler`
  (params (Actor :type "/Game/Blueprint/Actors/ProcessVolumes/BP_LocalVolumeHandler Object Reference") (Index :type Integer))
  (set `self.Handler` Actor)
  (set `self.Index` Index))

(event `self.ReceiveBeginPlay`
  (`self.TryGetPawn`)
  (set `self.MaxDistance` (`KismetMathLibrary.Square` (`self.MaxDistance`))))

(event `TryGetPawn`
  (set `self.Player` (`GameplayStatics.GetPlayerPawn` 0))
  (if (`KismetSystemLibrary.IsValid` (`self.Player`))
    (`KismetSystemLibrary.PrintString` "Player found")
    (elif (> (`self.maxTries`) 0)
      (`KismetSystemLibrary.PrintString` "Retry")
      (`KismetSystemLibrary.Delay` 0.5)
      (`/Engine/EditorBlueprintResources/StandardMacros.DecrementInt` (`self.maxTries`)
        (:`  `
          (`self.TryGetPawn`)))
      (else
        (`KismetSystemLibrary.PrintString` "Pawn not found after 5 tries")))))

(event `self.ReceiveTick`
  (params (DeltaSeconds :type "Float (single-precision)"))
  (bind _returnvalue (`KismetMathLibrary.FClamp` (`KismetMathLibrary.VSizeSquared` (- (`self.K2_GetActorLocation`) (`self.K2_GetActorLocation` (`self.Player`)))) 0.0 (`self.MaxDistance`)))
  (if (`KismetSystemLibrary.IsValid` (`self.Player`))
    (if (== _returnvalue 0.0)
      (`/Game/Blueprint/Actors/ProcessVolumes/BP_LocalVolumeHandler.SetWeight` (`self.Handler`) 0.0 (`self.Index`))
      (else
        (`/Game/Blueprint/Actors/ProcessVolumes/BP_LocalVolumeHandler.SetWeight` (`self.Handler`) (`KismetMathLibrary.FClamp` (`CurveFloat.GetFloatValue` (`self.Curve`) (- 1.0 (/ _returnvalue (`KismetMathLibrary.FMax` (`self.MaxDistance`) 0.01))))) (`self.Index`))))))

(fn `UserConstructionScript`
  (`SceneComponent.SetWorldScale3D` (`self.Sphere`) (`KismetMathLibrary.Conv_DoubleToVector` (/ (`self.MaxDistance`) 50.0))))