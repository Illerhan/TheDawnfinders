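; BP_TopDoorVivianite is a vivianite architecture level element whose emissive glow toggles on activation.
; BeginPlay creates a dynamic material instance on the wall mesh's vivianite material slot.
; Each Activate call alternates a timeline forward or reverse through a FlipFlop, with a debug print, and the update lerps the material's emissive opacity between dim and bright.
; IsActive always returns false, whatever the glow state.
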(event `self.ReceiveBeginPlay`
  (bind _returnvalue (`PrimitiveComponent.CreateDynamicMaterialInstance` (`self.SM_ApophisDecorationWallBottom_001`) 2 "/Game/Art/Materials/Instances/Instances_Tileable/MI_VivianiteArchitecture_01.MI_VivianiteArchitecture_01" "None"))
  (set `self.Mat` _returnvalue))

(event `self.Activate`
  (`self.ShowHideLights`))

(event `ShowHideLights`
  (`KismetSystemLibrary.PrintString` "LIGHTS")
  (`/Engine/EditorBlueprintResources/StandardMacros.FlipFlop`
    (:`A`
      (bind (_direction _alpha) (`Timeline|Timeline` :!label _label)
        (:`Update`
          (`MaterialInstanceDynamic.SetScalarParameterValue` (`self.Mat`) "Emissive_OverallOpacity" (`KismetMathLibrary.Lerp` 0.3 5.0 _alpha)))))
    (:`B`
      (goto _label :!via `Reverse`))))

(fn `IsActive`
  (returns (ReturnValue :type Boolean))
  (return false))

(fn `UserConstructionScript`)