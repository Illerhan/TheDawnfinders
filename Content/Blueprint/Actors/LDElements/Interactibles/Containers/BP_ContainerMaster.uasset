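; BP_ContainerMaster is an interactible container, apparently a base class, that highlights itself and its interest-point VFX.
; Overlapping InteractCollider toggles a dynamic outline overlay material on the mesh.
; Light and palanquin-light events share authority-only logic that adjusts a NumberOfLights counter while the inventory has items.
; The VFX turns on while that count is positive and off when it drops to zero.
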(event `self.InteractCollider.OnComponentBeginOverlap`
  (params (OverlappedComponent :type "PrimitiveComponent Object Reference") (OtherActor :type "Actor Object Reference") (OtherComp :type "PrimitiveComponent Object Reference") (OtherBodyIndex :type Integer) (bFromSweep :type Boolean) (SweepResult :type "HitResult Structure (by ref)"))
  ; OutlineOverlap
  (`MaterialInstanceDynamic.SetScalarParameterValue` (stale `self.ReceiveBeginPlay` _returnvalue) "IsVisible" 1.0))

(event `self.InteractCollider.OnComponentEndOverlap`
  (params (OverlappedComponent :type "PrimitiveComponent Object Reference") (OtherActor :type "Actor Object Reference") (OtherComp :type "PrimitiveComponent Object Reference") (OtherBodyIndex :type Integer))
  ; OutlineOverlap
  (`MaterialInstanceDynamic.SetScalarParameterValue` (stale `self.ReceiveBeginPlay` _returnvalue) "IsVisible" 0.0))

(event `self.ReceiveBeginPlay`
  (bind _returnvalue (`KismetMaterialLibrary.CreateDynamicMaterialInstance` "/Game/Art/Materials/Instances/Instances-FXs/MI_OutlineOverlay_01.MI_OutlineOverlay_01"))
  (`MeshComponent.SetOverlayMaterial` (`self.StaticMesh`) _returnvalue)
  (`ActorComponent.Deactivate` (`self.InterestPointVFXComponent`)))

(event `/Game/Blueprint/Interface/BPI_FogOfWar.Light On`
  (params (isTorchLight :type Boolean))
  (`/Engine/EditorBlueprintResources/ActorMacros.Switch Has Authority` :!label _label
    (:`Authority`
      (bind _returnvalue (`InventoryComponent.GetIsEmpty` (`self.InventoryComponent`)))
      (if (not _returnvalue)
        (bind _result (`/Engine/EditorBlueprintResources/StandardMacros.IncrementInt` (`self.NumberOfLights`))
          (:`  `
            (if (> _result 0)
              (`self.Activate`))))))))

(event `/Game/Blueprint/Interface/BPI_FogOfWar.Palanquin Light On`
  (goto _label))

(event `/Game/Blueprint/Interface/BPI_FogOfWar.Light Off`
  (params (isTorchLight :type Boolean))
  (`/Engine/EditorBlueprintResources/ActorMacros.Switch Has Authority` :!label _label_2
    (:`Authority`
      (bind _returnvalue (`InventoryComponent.GetIsEmpty` (`self.InventoryComponent`)))
      (if (not _returnvalue)
        (bind _output_get (set `self.NumberOfLights` (`KismetMathLibrary.Clamp` (- (`self.NumberOfLights`) 1) 0 100)))
        (if (<= _output_get 0)
          (`self.Deactivate`))))))

(event `/Game/Blueprint/Interface/BPI_FogOfWar.Palanquin Light Off`
  (goto _label_2))

(event `Activate`
  (`ActorComponent.Activate` (`self.InterestPointVFXComponent`) false))

(event `Deactivate`
  (`ActorComponent.Deactivate` (`self.InterestPointVFXComponent`)))

(fn `OnRep_NumberOfLights`)

(fn `UserConstructionScript`)