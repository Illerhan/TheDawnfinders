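; Fog of war actor that reveals enemies while they overlap it, acting as a light or vision area.
; Each BP_EnemyMaster entering increments its NumberOfLights counter and unhides its mesh.
; Leaving decrements the counter and hides the mesh only when it reaches zero or below, so overlapping areas keep shared enemies visible.
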(event `self.ReceiveActorBeginOverlap`
  (params (OtherActor :type "Actor Object Reference"))
  (bind _asbp_enemy_master (cast `/Game/Blueprint/Actors/Enemies/BP_EnemyMaster` OtherActor))
  (`/Engine/EditorBlueprintResources/StandardMacros.IncrementInt` (`/Game/Blueprint/Actors/Enemies/BP_EnemyMaster.NumberOfLights` _asbp_enemy_master)
    (:`  `
      (`SceneComponent.SetHiddenInGame` (`Character.Mesh` _asbp_enemy_master) false false))))

(event `self.ReceiveActorEndOverlap`
  (params (OtherActor :type "Actor Object Reference"))
  (bind _asbp_enemy_master (cast `/Game/Blueprint/Actors/Enemies/BP_EnemyMaster` OtherActor))
  (bind _result (`/Engine/EditorBlueprintResources/StandardMacros.DecrementInt` (`/Game/Blueprint/Actors/Enemies/BP_EnemyMaster.NumberOfLights` _asbp_enemy_master))
    (:`  `
      (if (<= _result 0)
        (`SceneComponent.SetHiddenInGame` (`Character.Mesh` _asbp_enemy_master) true false)))))

(fn `UserConstructionScript`)