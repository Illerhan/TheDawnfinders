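; BP_LevelInstantiator is an actor that streams lists of sublevels in and out, triggered on overlap or at BeginPlay when BaseSpawner is set.
; Load steps through LevelsToLoad by recursing after short delays, making each level visible without blocking, then resets the shared Index and starts Unload.
; Unload works through LevelsToUnload the same way with longer delays, and both print each level name.
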(event `self.ReceiveBeginPlay`
  (if (`self.BaseSpawner`)
    (`self.Load`)))

(event `self.ReceiveActorBeginOverlap`
  (params (OtherActor :type "Actor Object Reference"))
  (set `self.Index` 0)
  (`self.Load`))

(event `Unload`
  (bind _index (`self.Index`))
  (bind _levelstounload (`self.LevelsToUnload`))
  (bind _output (`|GetArrayItem` _levelstounload _index))
  (if (< _index (`KismetArrayLibrary.Array_Length` _levelstounload))
    (`GameplayStatics.UnloadStreamLevel` _output)
    (`KismetSystemLibrary.PrintString` (`KismetStringLibrary.Concat_StrStr` "Unloaded " (`KismetStringLibrary.Conv_NameToString` _output)))
    (`/Engine/EditorBlueprintResources/StandardMacros.IncrementInt` (`self.Index`)
      (:`  `
        (`KismetSystemLibrary.Delay` 0.5)
        (`self.Unload`)))))

(event `Load`
  (bind _index (`self.Index`))
  (bind _levelstoload (`self.LevelsToLoad`))
  (bind _output (`|GetArrayItem` _levelstoload _index))
  (if (< _index (`KismetArrayLibrary.Array_Length` _levelstoload))
    (`GameplayStatics.LoadStreamLevel` _output true)
    (`KismetSystemLibrary.PrintString` (`KismetStringLibrary.Concat_StrStr` "Loaded" (`KismetStringLibrary.Conv_NameToString` _output)))
    (`/Engine/EditorBlueprintResources/StandardMacros.IncrementInt` (`self.Index`)
      (:`  `
        (`KismetSystemLibrary.Delay` 0.1)
        (`self.Load`)))
    (else
      (set `self.Index` 0)
      (`self.Unload`))))

(fn `UserConstructionScript`)