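; Base hallucination enemy that may appear to the local player according to a probability roll and their curse-derived sanity.
; Replicated initialization hides the mesh, creates dynamic materials and schedules display checks, which also require a clear surrounding sphere trace.
; A fog-of-war area counter drives a timeline fading material opacity.
; Tick mirrors AI controller state and smooths yaw toward movement, while montage notifies run repeated attack collision checks.
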(event `self.ReceiveBeginPlay`
  ; Initialisation
  (set `self.bIsInitialised` true)
  (`parent.ReceiveBeginPlay`))

(event `Initialise`
  ; Initialisation
  (bind _asaic_hallucination (cast `/Game/Blueprint/AI/Controllers/AIC_Hallucination` (`self.GetController`))
    (:`then`
      (set `self.AIController` _asaic_hallucination))
    (:`CastFailed`
      _))
  (for (_array_element _array_index) (`MeshComponent.GetMaterials` (`self.Mesh`))
    (bind _returnvalue (`KismetMaterialLibrary.CreateDynamicMaterialInstance` _array_element))
    (`KismetArrayLibrary.Array_Add` (`self.EnemyMaterials`) _returnvalue)
    (`MaterialInstanceDynamic.SetScalarParameterValue` _returnvalue "Opacity" 0.0)
    (`PrimitiveComponent.SetMaterial` (`self.Mesh`) _array_index _returnvalue))
  (`SceneComponent.SetVisibility` (`self.Mesh`) false true)
  (set `self.bIsDisplayed` true)
  (bind _asps_custom (cast `/Game/Blueprint/GameFramework/PS_Custom` (`Controller.PlayerState` (`GameplayStatics.GetPlayerController` 0))))
  (if (<= (`KismetMathLibrary.RandomFloatInRange` 0.0 100.0) (`self.AppearProbability`))
    (add `CustomPlayerState.OnCurseInfoChange` _asps_custom (delegate `TryDisplayOnClient`))
    (`self.TryDisplayOnClient`)
    (`KismetSystemLibrary.K2_SetTimerDelegate` (delegate `TryDisplayOnClient`) 5.0 true)))

(event `TryDisplayOnClient`
  (bind _returnvalue (`self.K2_GetActorLocation`))
  ; Fade Behavior
  (if (not (`self.IsDisplayed`))
    (bind (_outhits _returnvalue_2) (`KismetSystemLibrary.SphereTraceMulti` _returnvalue _returnvalue 1500.0 "TraceTypeQuery4"))
    (if (not _returnvalue_2)
      (bind _asps_custom (cast `/Game/Blueprint/GameFramework/PS_Custom` (`Controller.PlayerState` (`GameplayStatics.GetPlayerController` 0))))
      (if (>= (`self.SanityThreshold`) (* (- 1.0 (`CustomPlayerState.GetCurseRatio` _asps_custom)) 100.0))
        (`SceneComponent.SetVisibility` (`self.Mesh`) true true)
        (set `self.bIsDisplayed` true)))))

(event `self.FadeIn`
  ; Fade Behavior
  (if (`self.bIsDisplayed`)
    (`self.FadeOut_Multicast`)
    (`SceneComponent.SetVisibility` (`self.Mesh`) false true)
    (set `self.bIsDisplayed` false)))

(event `self.FadeOut`
  ; Fade Behavior
  (if (`self.bIsDisplayed`)
    _))

(event `FadeIn_Multicast`
  ; Fade Behavior
  (bind _result (`/Engine/EditorBlueprintResources/StandardMacros.IncrementInt` (`self.FogOfWarAreasCount`))
    (:`  `
      (bind _output_get (set `self.FogOfWarAreasCount` (`KismetMathLibrary.Clamp` _result 0 100)))
      (if (== _output_get 1)
        (`parent.FadeIn`)
        (bind (_direction _newtrack_0) (`Timeline|FadeInTimeline` :!via `PlayFromStart` :!label _label)
          (:`Update`
            (for _array_element (`self.EnemyMaterials`)
              (`MaterialInstanceDynamic.SetScalarParameterValue` _array_element "Opacity" _newtrack_0))))))))

(event `FadeOut_Multicast`
  ; Fade Behavior
  (bind _result (`/Engine/EditorBlueprintResources/StandardMacros.DecrementInt` (`self.FogOfWarAreasCount`))
    (:`  `
      (bind _output_get (set `self.FogOfWarAreasCount` (`KismetMathLibrary.Clamp` _result 0 100)))
      (if (== _output_get 0)
        (`parent.FadeOut`)
        (goto _label :!via `ReverseFromEnd`)))))

(event `self.ReceiveTick`
  (params (DeltaSeconds :type "Float (single-precision)"))
  (bind _aicontroller (`self.AIController`))
  ; Event Tick
  (`parent.ReceiveTick` DeltaSeconds)
  (`/Engine/EditorBlueprintResources/StandardMacros.IsValid` _aicontroller
    (:`Is Valid`
      (set `self.CurrentEnemyState` (`BasicEnemyAIController.EnemyState` _aicontroller))
      (set `self.FollowingStatus` (`AIController.GetMoveStatus` _aicontroller))
      (if (not (`self.bLockRotation`))
        (`self.K2_SetActorRotation` (`KismetMathLibrary.RInterpTo` (`self.K2_GetActorRotation`) (`KismetMathLibrary.MakeRotator` 0.0 0.0 (.yaw (`KismetMathLibrary.FindLookAtRotation` (`self.K2_GetActorLocation`) (`AIController.GetImmediateMoveDestination` (`self.AIController`))))) DeltaSeconds 5.0))))))

(event `self.BP_OnMontageNotifyBegin`
  (params (NotifyName :type Name))
  ; Montages
  (set `self.TempInt` 0)
  (if (< (`self.TempInt`) 8) :!label _label_2
    (`self.DoAttackCollision`)
    (`/Engine/EditorBlueprintResources/StandardMacros.IncrementInt` (`self.TempInt`)
      (:`  `
        (`KismetSystemLibrary.Delay` 0.008)
        (goto _label_2)))))

(event `self.BP_OnMontageEnd`
  (params (bInterrupted :type Boolean))
  (bind _aicontroller (`self.AIController`))
  ; Montages
  (`/Engine/EditorBlueprintResources/StandardMacros.IsValid` _aicontroller
    (:`Is Valid`
      (`/Game/Blueprint/AI/Controllers/AIC_BasicEnemy.EndAttack` _aicontroller))))

(fn `OnRep_bIsInitialised`
  (`self.Initialise`))

(fn `UserConstructionScript`)