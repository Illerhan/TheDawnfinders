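; BP_IndianaJones_Ball is a level-design hazard actor, a ball that damages the player on contact.
; It starts hidden with Sphere collision disabled, and nothing in this Blueprint re-enables either.
; Overlapping a BP_PlayerCharacter applies heavy Blood damage through its HealthComponent and destroys the ball immediately.
; A DestroyBall event offers removal after a configurable Delay.
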(event `self.ReceiveBeginPlay`
  (`self.SetActorHiddenInGame` true)
  (`PrimitiveComponent.SetCollisionEnabled` (`self.Sphere`) "NoCollision"))

(event `self.ReceiveActorBeginOverlap`
  (params (OtherActor :type "Actor Object Reference"))
  (bind _asbp_player_character (cast `/Game/Blueprint/Actors/Player/BP_PlayerCharacter` OtherActor))
  (`HealthComponent.TakeDamage` (`APlayerCharacter.HealthComponent` _asbp_player_character) 100.0 "Blood")
  (`self.K2_DestroyActor`))

(event `DestroyBall`
  (`KismetSystemLibrary.Delay` (`self.delay`))
  (`self.K2_DestroyActor`))

(fn `UserConstructionScript`)