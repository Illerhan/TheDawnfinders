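; BP_Plane_Rocks is a level element: a collision plane paired with a list of rock actors that it releases as falling rubble.
; DeactivatePlane turns off the plane's collision, clears IsActivate, then unhides each rock in RocksLists and enables physics on its rubble mesh.
; A Delay inside the loop body later restores the plane's query and physics collision and sets IsActivate again.
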(event `DeactivatePlane`
  (`PrimitiveComponent.SetCollisionEnabled` (`self.Plane`) "NoCollision")
  (set `self.isActivate` false)
  (for _array_element (`self.RocksLists`)
    (`PrimitiveComponent.SetSimulatePhysics` (`/Game/Blueprint/Actors/LDElements/BP_Physics_Rocks.SM_StoneRubble_001` _array_element) true)
    (`self.SetActorHiddenInGame` _array_element false)
    (`KismetSystemLibrary.Delay` 5.0)
    (`PrimitiveComponent.SetCollisionEnabled` (`self.Plane`) "QueryAndPhysics")
    (set `self.isActivate` true)))

(event `self.ReceiveBeginPlay`)

(fn `UserConstructionScript`)