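; Extraction platform Blueprint, a movable level element that sounds a loud warning before it moves.
; DoMovement plays a networked placeholder sine-tone ping at the Cylinder component, repeats it on a looping timer, and starts a ten-second delay.
; When the delay ends, StartExtraction calls the parent DoMovement to run the inherited movement and clears the noise timer.
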(event `self.ReceiveTick`
  (params (DeltaSeconds :type "Float (single-precision)")))

(event `self.DoMovement`
  (`self.MakeNoiseElevator`)
  (`KismetSystemLibrary.K2_SetTimerDelegate` (delegate `StartExtraction`) 10.0)
  (bind _returnvalue (`KismetSystemLibrary.K2_SetTimerDelegate` (delegate `MakeNoiseElevator`) 2.0 true)))

(event `StartExtraction`
  (`parent.DoMovement`)
  (`KismetSystemLibrary.K2_ClearAndInvalidateTimerHandle` (stale `self.DoMovement` _returnvalue)))

(event `MakeNoiseElevator`
  (`GameplaySoundHelper.PlaySoundNetworked` self "/Engine/EngineSounds/1kSineTonePing.1kSineTonePing" (`SceneComponent.K2_GetComponentLocation` (`self.Cylinder`)) 1000.0))

(fn `UserConstructionScript`)