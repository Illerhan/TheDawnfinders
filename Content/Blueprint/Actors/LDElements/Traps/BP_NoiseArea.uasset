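; BP_NoiseArea is a level-design trap volume that scales the player character's noise while they are inside it.
; Overlap begin multiplies BP_PlayerCharacter's NoiseModifier by NoiseMultiplier, and overlap end divides it back out.
; The construction script sets the cylinder's material according to whether the multiplier is above one, visually marking amplifying areas apart from the others.
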(event `self.ReceiveActorBeginOverlap`
  (params (OtherActor :type "Actor Object Reference"))
  (bind _asbp_player_character (cast `/Game/Blueprint/Actors/Player/BP_PlayerCharacter` OtherActor))
  (set `APlayerCharacter.NoiseModifier` (* (`APlayerCharacter.NoiseModifier` _asbp_player_character) (`self.NoiseMultiplier`)) _asbp_player_character))

(event `self.ReceiveActorEndOverlap`
  (params (OtherActor :type "Actor Object Reference"))
  (bind _asbp_player_character (cast `/Game/Blueprint/Actors/Player/BP_PlayerCharacter` OtherActor))
  (set `APlayerCharacter.NoiseModifier` (/ (`APlayerCharacter.NoiseModifier` _asbp_player_character) (`self.NoiseMultiplier`)) _asbp_player_character))

(fn `UserConstructionScript`
  (`PrimitiveComponent.SetMaterial` (`self.Cylinder`) 0 (select `bool` (> (`self.NoiseMultiplier`) 1.0) :`false` "/Game/Materials/LevelDesign_Builder/M_Noise_01.M_Noise_01" :`true` "/Game/Materials/LevelDesign_Builder/M_Noise_02.M_Noise_02" :!type "MaterialInterface Object Reference")))