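; BP_MiningItem is an interactible mining item actor whose outline highlights while something overlaps its OutlineCollider.
; On BeginPlay it gives the mesh a slight random yaw and applies a dynamic outline overlay material, whose IsVisible parameter the overlap events toggle.
; It writes its location to DepositPosition in the shared MPC_ColorModifiers collection during construction and BeginPlay, so that global value holds only the last writer's position.
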(event `self.OutlineCollider.OnComponentBeginOverlap`
  (params (OverlappedComponent :type "PrimitiveComponent Object Reference") (OtherActor :type "Actor Object Reference") (OtherComp :type "PrimitiveComponent Object Reference") (OtherBodyIndex :type Integer) (bFromSweep :type Boolean) (SweepResult :type "HitResult Structure (by ref)"))
  ; OutlineOverlap
  (`MaterialInstanceDynamic.SetScalarParameterValue` (stale `self.ReceiveBeginPlay` _returnvalue) "IsVisible" 1.0))

(event `self.OutlineCollider.OnComponentEndOverlap`
  (params (OverlappedComponent :type "PrimitiveComponent Object Reference") (OtherActor :type "Actor Object Reference") (OtherComp :type "PrimitiveComponent Object Reference") (OtherBodyIndex :type Integer))
  ; OutlineOverlap
  (`MaterialInstanceDynamic.SetScalarParameterValue` (stale `self.ReceiveBeginPlay` _returnvalue) "IsVisible" 0.0))

(event `self.ReceiveBeginPlay`
  (`parent.ReceiveBeginPlay`)
  (`SceneComponent.K2_SetRelativeRotation` (`self.StaticMesh`) (`KismetMathLibrary.MakeRotator` 0.0 0.0 (`KismetMathLibrary.RandomFloatInRange` -10.0 10.0)) false false)
  (bind _returnvalue (`KismetMaterialLibrary.CreateDynamicMaterialInstance` "/Game/Art/Materials/Instances/Instances-FXs/MI_OutlineOverlay_02.MI_OutlineOverlay_02"))
  (`MeshComponent.SetOverlayMaterial` (`self.StaticMesh`) _returnvalue)
  (`KismetMaterialLibrary.SetVectorParameterValue` "/Game/Art/Materials/CollectionParameter/MPC_ColorModifiers.MPC_ColorModifiers" "DepositPosition" (`KismetMathLibrary.Conv_VectorToLinearColor` (`self.K2_GetActorLocation`))))

(fn `UserConstructionScript`
  (`KismetMaterialLibrary.SetVectorParameterValue` "/Game/Art/Materials/CollectionParameter/MPC_ColorModifiers.MPC_ColorModifiers" "DepositPosition" (`KismetMathLibrary.Conv_VectorToLinearColor` (`self.K2_GetActorLocation`))))