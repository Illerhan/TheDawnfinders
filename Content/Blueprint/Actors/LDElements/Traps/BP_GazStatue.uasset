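; Gas statue trap that poisons any player character overlapping it, switched via Activate/Deactivate and not directly usable by interactors.
; One Timeline animates head pitch and two light intensities: Activate reverses it through OpenMouth, Deactivate plays it through CloseMouth.
; CloseMouth first disables PoisonZone and shows small gas puffs, then enables the zone and main gas when forward playback finishes.
; OpenMouth leaves gas and collision untouched.
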(event `self.ReceiveActorBeginOverlap`
  (params (OtherActor :type "Actor Object Reference"))
  (bind _asbp_player_character (cast `/Game/Blueprint/Actors/Player/BP_PlayerCharacter` OtherActor))
  (`HealthComponent.SetIsPoisoned` (`APlayerCharacter.HealthComponent` _asbp_player_character) true))

(event `self.Activate`
  (set `self.Activated` true)
  (`self.Open Mouth`))

(event `self.Deactivate`
  (set `self.Activated` false)
  (`self.Close Mouth`))

(event `Key|O`
  (params (Key :type "Key Structure")))

(event `Close Mouth`
  (`self.Deactivate Hitbox`)
  (bind (_direction _alpha) (`Timeline|Timeline` :!label _label)
    (:`Update`
      (`SceneComponent.K2_SetRelativeRotation` (`self.SM_PoisonTrapHead_01`) (`KismetMathLibrary.RLerp` (struct :`Roll` 25.0) (struct :`Roll` -15.0) _alpha true) false false)
      (bind _returnvalue (`KismetMathLibrary.Lerp` 0.0 300.0 _alpha))
      (`LightComponent.SetIntensity` (`self.PointLight`) _returnvalue)
      (`LightComponent.SetIntensity` (`self.PointLight1`) _returnvalue))
    (:`Finished`
      (if (>= _alpha 1.0)
        (`self.Activate Hitbox`)))))

(event `Open Mouth`
  (goto _label :!via `Reverse`))

(event `Activate Hitbox`
  (`ActorComponent.Activate` (`self.NS_Gaz`) true)
  (`ActorComponent.Deactivate` (`self.NS_SmallGaz`))
  (`ActorComponent.Deactivate` (`self.NS_SmallGaz1`))
  (`PrimitiveComponent.SetCollisionEnabled` (`self.Poison Zone`) "QueryAndPhysics"))

(event `Deactivate Hitbox`
  (`ActorComponent.Deactivate` (`self.NS_Gaz`))
  (`ActorComponent.Activate` (`self.NS_SmallGaz`) true)
  (`ActorComponent.Activate` (`self.NS_SmallGaz1`) true)
  (`PrimitiveComponent.SetCollisionEnabled` (`self.Poison Zone`) "NoCollision"))

(fn `GetCanBeUsed`
  (params (Interactor :type "Actor Object Reference"))
  (returns (ReturnValue :type Boolean))
  (return false))

(fn `GetNeededQTE`
  (returns (ReturnValue :type "EQTEType Enum"))
  (return "NoQTE"))

(fn `IsActive`
  (returns (ReturnValue :type Boolean))
  (return (`self.Activated`)))

(fn `UserConstructionScript`)