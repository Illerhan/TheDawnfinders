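; BP_Litter is the palanquin actor, an interactible that carries a protection zone and can be extracted.
; Each tick feeds its position and zone radius into MPC_Fog for a fog cutout.
; A Niagara protection effect scales with that radius while the light is on and hides once when it goes off.
; It spawns an off-screen indicator widget, and extraction starts a looping timer that broadcasts distraction noise through the player pawn.
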(event `self.ReceiveTick`
  (params (DeltaSeconds :type "Float (single-precision)"))
  (bind (_returnvalue_x _returnvalue_y) (`KismetMathLibrary.BreakVector` (`self.K2_GetActorLocation`)))
  (bind _ns_palanquinprotection (`self.NS_PalanquinProtection`))
  (bind _sphereradius (`SphereComponent.SphereRadius` (`self.ProtectionZone`)))
  (`KismetMaterialLibrary.SetScalarParameterValue` "/Game/Materials/MPC_Fog.MPC_Fog" "PalanquinX" _returnvalue_x)
  (`KismetMaterialLibrary.SetScalarParameterValue` "/Game/Materials/MPC_Fog.MPC_Fog" "PalanquinY" _returnvalue_y)
  (`KismetMaterialLibrary.SetScalarParameterValue` "/Game/Materials/MPC_Fog.MPC_Fog" "CutoutRadius" (/ _sphereradius 50.0))
  (if (`PlayerLightComponent.bLightOn` (`self.LightComponent`))
    (if (not (`SceneComponent.IsVisible` _ns_palanquinprotection))
      (`SceneComponent.SetVisibility` (`self.NS_PalanquinProtection`) true false))
    (`SceneComponent.SetWorldScale3D` _ns_palanquinprotection (`KismetMathLibrary.Conv_DoubleToVector` (/ _sphereradius 2000.0)))
    (goto _label :!via `Reset`)
    (else
      (`/Engine/EditorBlueprintResources/StandardMacros.DoOnce` false :!label _label
        (:`Completed`
          (`SceneComponent.SetVisibility` (`self.NS_PalanquinProtection`) false false))))))

(event `self.ReceiveBeginPlay`
  (bind _returnvalue (`|CreateWidget` "/Game/UI/Widgets/WBP_OffScreenPalanquin.WBP_OffScreenPalanquin_C"))
  (set `/Game/UI/Widgets/WBP_OffScreenPalanquin.Palanquin` self _returnvalue)
  (`UserWidget.AddToViewport` _returnvalue 0))

(event `self.StartExtraction`
  (`parent.StartExtraction`)
  (`KismetSystemLibrary.K2_SetTimerDelegate` (delegate `MakeNoiseElevator`) 2.0 true))

(event `MakeNoiseElevator`
  (`self.PlayNoise` self)
  (message `PlayerInterface.PlaySoundOnServer` (`GameplayStatics.GetPlayerPawn` 0) "Distraction" 10000.0 1.0 (`SceneComponent.K2_GetComponentLocation` (`self.RootCollision`))))

(fn `UserConstructionScript`)