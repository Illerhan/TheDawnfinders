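; BP_Land_Mine is a land mine trap actor that deals area damage when its Explose event is called.
; Explose runs a debug-drawn multi-sphere trace at its location and sends each hit actor a damage message.
; A multicast event then plays the explosion effect, hides the mesh and disables the trap collider, and the actor is destroyed after a short delay.
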(event `self.Explose`
  (bind _returnvalue (`self.K2_GetActorLocation`))
  (bind _outhits (`KismetSystemLibrary.SphereTraceMulti` :`Start` _returnvalue :`End` _returnvalue :`Radius` (`self.ExplosionRange`) :`TraceChannel` "TraceTypeQuery3" :`DrawDebugType` "ForDuration" :`DrawTime` 2.0))
  (for _array_element _outhits
    (message `Damageable.ReceiveDamage` (`.HitActor` (`GameplayStatics.BreakHitResult` _array_element)) (`KismetMathLibrary.Conv_IntToDouble` (`self.DamagesEnemies`)) self))
  (`self.Multicast_PlayExplosionVFX`)
  (`KismetSystemLibrary.Delay` 3.0)
  (`self.K2_DestroyActor`))

(event `Multicast_PlayExplosionVFX`
  (`ActorComponent.Activate` (`self.Explosion`) false)
  (`SceneComponent.SetVisibility` (`self.StaticMesh`) false false)
  (`PrimitiveComponent.SetCollisionEnabled` (`self.TrapCollider`) "NoCollision"))

(fn `UserConstructionScript`)