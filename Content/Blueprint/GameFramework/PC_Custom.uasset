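; Custom player controller covering lobby menu and camera, ready-up, end-of-game recap and player save data.
; Ready toggles go through the server to the game state, starting or ending the PlayerState countdown and refreshing squad widgets.
; A client recap event shows success only for protected winners.
; Inventory, stash and gold move between character, PlayerState and GameInstance save, using delayed cast retries; the inventory restore calls are disconnected.
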(event `LobbyCamera`
  (params (Target :type "PlayerController Object Reference"))
  (`KismetSystemLibrary.Delay` 0.2 :!label _label)
  (bind _returnvalue (`GameplayStatics.GetActorOfClass` "/Script/Engine.CameraActor"))
  (`/Engine/EditorBlueprintResources/StandardMacros.IsValid` _returnvalue
    (:`Is Valid`
      (`KismetSystemLibrary.Delay` 0.5)
      (`self.SetViewTargetWithBlend` _returnvalue))))

(event `self.ReceiveBeginPlay`
  (`|ExecutionSequence`
    (:`then_0`
      (bind _returnvalue (`GameplayStatics.GetActorOfClass` "/Game/Blueprint/Actors/Mule/BP_Mule.BP_Mule_C"))
      (set `self.Mule` _returnvalue)
      (bind _returnvalue_2 (`GameplayStatics.GetActorOfClass` "/Script/Engine.PlayerStart"))
      (set `self.SpawnPoint` _returnvalue_2))
    (:`then_1`
      (bind _returnvalue_3 (`GameplayStatics.GetCurrentLevelName` true))
      (if (`KismetStringLibrary.Contains` _returnvalue_3 "Main")
        (goto _label)))))

(event `Multi_PlayMultiSound`
  (params (AkEvent :type "AkAudioEvent Object Reference") (Actor :type "Actor Object Reference"))
  (`AkGameplayStatics.PostEvent` AkEvent Actor))

(event `Client_SHowRecap`
  (params (`bWin?` :type Boolean))
  ; Show Recap Client
  (set `self.GameEnded` true)
  (bind _ashud_custom (cast `/Game/Blueprint/GameFramework/HUD_Custom` (`self.GetHUD` self)))
  (bind _wbp_gamerecapwidget (`/Game/UI/Widgets/WBP_MainWidget.WBP_GameRecapWidget` (`/Game/Blueprint/GameFramework/HUD_Custom.MainWidgetRef` _ashud_custom)))
  (if (not (`GameRecapWidget.bIsDisplayed` _wbp_gamerecapwidget))
    (bind _asps_custom (cast `/Game/Blueprint/GameFramework/PS_Custom` (`self.PlayerState`)))
    (if (`CustomPlayerState.bIsProtected` _asps_custom)
      (if `bWin?`
        (`GameRecapWidget.DisplaySuccessRecap` _wbp_gamerecapwidget)
        (else
          (`GameRecapWidget.DisplayFailRecap` _wbp_gamerecapwidget :!label _label_2)))
      (else
        (goto _label_2)))
    (`WidgetBlueprintLibrary.SetInputMode_UIOnlyEx` self _wbp_gamerecapwidget)
    (`KismetSystemLibrary.Delay` 1.2)
    (`Widget.SetKeyboardFocus` (`/Game/UI/Widgets/MainMenu/WBP_ExpeditionButton.Button` (`/Game/UI/Widgets/WBP_GameRecapWidget.ReadyButton` _wbp_gamerecapwidget)))))

(event `Client_ResetMusique`
  (`MusicManager.ResetState` (subsystem `MusicManager`)))

(event `CreateLobbyWidget`
  (bind _returnvalue (`|CreateWidget` "/Game/UI/Widgets/MainMenu/WBP_MainMenuLobby.WBP_MainMenuLobby_C"))
  (`UserWidget.AddToViewport` _returnvalue 0)
  (set `self.MenuWidget` _returnvalue)
  (set `self.bShowMouseCursor` false)
  (`self.DisableInput` (`GameplayStatics.GetPlayerPawn` 0) null)
  (`KismetSystemLibrary.Delay` 0.5)
  (`WidgetBlueprintLibrary.SetInputMode_GameAndUIEx` self null "LockOnCapture")
  (set `self.bEnableClickEvents` false)
  (set `self.bEnableMouseOverEvents` false)
  (set `self.bEnableTouchOverEvents` false)
  (set `self.bEnableTouchEvents` false))

(event `Server_ApplyData`
  (params (PS :type "PlayerState Object Reference") (`Inventory Items` :type "Array of InventorySlot Structure") (`Stash Items` :type "Array of InventorySlot Structure") (`Saved Gold` :type Integer))
  (bind _asps_custom (cast `/Game/Blueprint/GameFramework/PS_Custom` PS :!label _label_3)
    (:`then`
      (set `CustomPlayerState.InventoryItems` `Inventory Items` _asps_custom)
      (set `CustomPlayerState.StashItems` `Stash Items` _asps_custom)
      (set `CustomPlayerState.SavedGold` `Saved Gold` _asps_custom))
    (:`CastFailed`
      (`KismetSystemLibrary.Delay` 0.1)
      (goto _label_3))))

(event `self.SwitchPanelBP`
  (params (PanelIndex :type Integer))
  (bind _menuwidget (`self.MenuWidget`))
  (switch `int` PanelIndex
    (:`0`
      (`/Game/UI/Widgets/MainMenu/WBP_MainMenuLobby.SwitchMenu` _menuwidget "NewEnumerator0"))
    (:`1`
      (`/Game/UI/Widgets/MainMenu/WBP_MainMenuLobby.SwitchMenu` _menuwidget "NewEnumerator1"))
    (:`2`
      (`/Game/UI/Widgets/MainMenu/WBP_MainMenuLobby.SwitchMenu` _menuwidget "NewEnumerator2"))))

(event `RequestLoadSave`
  (params (PS :type "PlayerState Object Reference"))
  (bind _asgi_custom (cast `/Game/Blueprint/GameFramework/GI_Custom` (`GameplayStatics.GetGameInstance`) :!label _label_4)
    (:`then`
      (bind _asps_custom (cast `/Game/Blueprint/GameFramework/PS_Custom` PS :!label _label_5)
        (:`then`
          (bind _gamesave (`/Game/Blueprint/GameFramework/GI_Custom.GameSave` _asgi_custom))
          (set `CustomPlayerState.InventoryItems` (`/Game/Blueprint/GameFramework/BP_LocalSave.PlayerInventory` _gamesave) _asps_custom)
          (set `CustomPlayerState.StashItems` (`/Game/Blueprint/GameFramework/BP_LocalSave.StashInventory` _gamesave) _asps_custom)
          (set `CustomPlayerState.SavedGold` (`/Game/Blueprint/GameFramework/BP_LocalSave.Gold` _gamesave) _asps_custom)
          (`KismetSystemLibrary.PrintString` (`KismetTextLibrary.Conv_TextToString` (`|FormatText` "Save Loaded")) true true (struct :`G` 0.66 :`B` 1.0 :`A` 1.0) 10.0))
        (:`CastFailed`
          (`KismetSystemLibrary.Delay` 0.1)
          (goto _label_5))))
    (:`CastFailed`
      (`KismetSystemLibrary.Delay` 0.1)
      (goto _label_4))))

(event `Client_SaveInventories`
  (`self.SaveInventories`))

(event `Server_ApplySaveData`
  (params (Inventory :type "Array of InventorySlot Structure") (SteshInv :type "Array of InventorySlot Structure") (Golds :type Integer))
  (bind _asps_custom (cast `/Game/Blueprint/GameFramework/PS_Custom` (`self.PlayerState`)))
  (bind _output_get (set `CustomPlayerState.InventoryItems` Inventory _asps_custom))
  (bind _output_get_2 (set `CustomPlayerState.StashItems` SteshInv _asps_custom))
  (set `CustomPlayerState.SavedGold` Golds _asps_custom))

(event `ToggleReady`
  (bind _output_get (set `self.bIsReady?` (not (`self.bIsReady?`))))
  (`self.Server_SetReady` (`self.PlayerState`) _output_get))

(event `Server_SetReady`
  (params (PlayerState :type "PlayerState Object Reference") (bReady :type Boolean))
  (bind _asbp_custom_game_state (cast `/Game/Blueprint/GameFramework/BP_CustomGameState` (`GameplayStatics.GetGameState`)))
  (`/Game/Blueprint/GameFramework/BP_CustomGameState.SetReadyLobby` _asbp_custom_game_state PlayerState bReady)
  (if (`/Game/Blueprint/GameFramework/BP_CustomGameState.AreAllLobbyReady?` _asbp_custom_game_state)
    (bind _asps_custom (cast `/Game/Blueprint/GameFramework/PS_Custom` PlayerState))
    (`/Game/Blueprint/GameFramework/PS_Custom.CountdownStart` _asps_custom)
    (else
      (bind _asps_custom_2 (cast `/Game/Blueprint/GameFramework/PS_Custom` PlayerState))
      (`/Game/Blueprint/GameFramework/PS_Custom.CountdownEnd` _asps_custom_2)))
  (bind _foundwidgets (`WidgetBlueprintLibrary.GetAllWidgetsOfClass` "/Game/UI/Widgets/MainMenu/WBP_ExpeditionButtons.WBP_ExpeditionButtons_C" false))
  (for _array_element _foundwidgets
    (`/Game/UI/Widgets/MainMenu/WBP_ExpeditionButtons.ActualiseSquad` _array_element)))

(fn `RestoreInventories`
  (params (self3 :type "/Game/Blueprint/Actors/Player/BP_PlayerCharacter Object Reference"))
  (bind _asgi_custom (cast `/Game/Blueprint/GameFramework/GI_Custom` (`GameplayStatics.GetGameInstance`)))
  (bind _gamesave (`/Game/Blueprint/GameFramework/GI_Custom.GameSave` _asgi_custom))
  (for _array_element (`/Game/Blueprint/GameFramework/BP_LocalSave.StashInventory` _gamesave)
    (`InventoryComponent.AddNewItem` (`/Game/Blueprint/Actors/Player/BP_PlayerCharacter.StashInventory` self3) (break `InventorySlot` _array_element) (`.Quantity` (break `InventorySlot` _array_element))))
  (for _array_element_2 (`/Game/Blueprint/GameFramework/BP_LocalSave.PlayerInventory` _gamesave)
    (`InventoryComponent.AddNewItem` (`APlayerCharacter.InventoryComponent` self3) (break `InventorySlot` _array_element_2) (`.Quantity` (break `InventorySlot` _array_element_2)))))

(fn `SaveInventories`
  (bind _asbp_player_character (cast `/Game/Blueprint/Actors/Player/BP_PlayerCharacter` (`self.K2_GetPawn`)))
  (bind _asgi_custom (cast `/Game/Blueprint/GameFramework/GI_Custom` (`GameplayStatics.GetGameInstance`)))
  (bind _gamesave (`/Game/Blueprint/GameFramework/GI_Custom.GameSave` _asgi_custom))
  (set `/Game/Blueprint/GameFramework/BP_LocalSave.PlayerInventory` (`InventoryComponent.InventorySlots` (`APlayerCharacter.InventoryComponent` _asbp_player_character)) _gamesave)
  (set `/Game/Blueprint/GameFramework/BP_LocalSave.StashInventory` (`InventoryComponent.InventorySlots` (`/Game/Blueprint/Actors/Player/BP_PlayerCharacter.StashInventory` _asbp_player_character)) _gamesave)
  (bind _asps_custom (cast `/Game/Blueprint/GameFramework/PS_Custom` (`Pawn.PlayerState` _asbp_player_character)))
  (set `/Game/Blueprint/GameFramework/BP_LocalSave.Gold` (`CustomPlayerState.SavedGold` _asps_custom) _gamesave)
  (`/Game/Blueprint/GameFramework/GI_Custom.SavePlayerData` _asgi_custom))

(fn `UserConstructionScript`)