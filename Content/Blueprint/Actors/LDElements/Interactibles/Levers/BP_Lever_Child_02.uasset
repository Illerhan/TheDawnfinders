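; BP_Lever_Child_02 is an interactible lever variant with an outline highlight and a skeletal mesh animation.
; A dynamic overlay material shows the outline on collider overlap, gated by SingleUse, which also gates disabling the lever and removing its prompt widget after interaction.
; A multicast event plays the animation forward or in reverse by on/off state.
; The player auto-moves to the nearer of two stand points, chosen by squared distance.
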(event `self.InteractCollider.OnComponentBeginOverlap`
  (params (OverlappedComponent :type "PrimitiveComponent Object Reference") (OtherActor :type "Actor Object Reference") (OtherComp :type "PrimitiveComponent Object Reference") (OtherBodyIndex :type Integer) (bFromSweep :type Boolean) (SweepResult :type "HitResult Structure (by ref)"))
  ; OutlineOverlap
  (`self.bSingleUse`
    (:`then`
      (`MaterialInstanceDynamic.SetScalarParameterValue` (stale `self.ReceiveBeginPlay` _returnvalue) "IsVisible" 1.0))
    (:`else`)))

(event `self.InteractCollider.OnComponentEndOverlap`
  (params (OverlappedComponent :type "PrimitiveComponent Object Reference") (OtherActor :type "Actor Object Reference") (OtherComp :type "PrimitiveComponent Object Reference") (OtherBodyIndex :type Integer))
  ; OutlineOverlap
  (`MaterialInstanceDynamic.SetScalarParameterValue` (stale `self.ReceiveBeginPlay` _returnvalue) "IsVisible" 0.0))

(event `self.ReceiveBeginPlay`
  (bind _returnvalue (`KismetMaterialLibrary.CreateDynamicMaterialInstance` "/Game/Art/Materials/Instances/Instances-FXs/MI_OutlineOverlay_03.MI_OutlineOverlay_03"))
  (`MeshComponent.SetOverlayMaterial` (`self.SkeletalMeshLever`) _returnvalue))

(event `self.BP_OnInteraction`
  (params (Player :type "APlayerCharacter Object Reference"))
  (`self.bSingleUse` :!label _label
    (:`then`
      (set `self.bCanBeUsed` false)
      (`MaterialInstanceDynamic.SetScalarParameterValue` (stale `self.ReceiveBeginPlay` _returnvalue) "IsVisible" 0.0)
      (`ActorComponent.K2_DestroyComponent` (`self.InteractibleWidgetComponent`)))
    (:`else`)))

(event `self.BP_OnInteractionFinished`
  (goto _label))

(event `self.DoInteractionAnim`
  (params (Interactor :type "Actor Object Reference"))
  (`self.Multicast_PlayAnimation` (not (`self.bIsOn`))))

(event `Multicast_PlayAnimation`
  (params (IsOn :type Boolean))
  (if IsOn
    (`SkeletalMeshComponent.SetPlayRate` (`self.SkeletalMeshLever`) 1.0)
    (`SkeletalMeshComponent.Play` (`self.SkeletalMeshLever`) false)
    (else
      (`SkeletalMeshComponent.SetPlayRate` (`self.SkeletalMeshLever`) -1.0)
      (`SkeletalMeshComponent.Play` (`self.SkeletalMeshLever`) false))))

(event `self.DoPlayerAutoMove`
  (params (Player :type "APlayerCharacter Object Reference"))
  (if (< (`KismetMathLibrary.VSizeSquared` (- (`self.K2_GetActorLocation` Player) (`SceneComponent.K2_GetComponentLocation` (`self.PlayerPos`)))) (`KismetMathLibrary.VSizeSquared` (- (`self.K2_GetActorLocation` Player) (`SceneComponent.K2_GetComponentLocation` (`self.PlayerPos1`)))))
    (`APlayerCharacter.StartAutoMoveCharacter` Player (`SceneComponent.K2_GetComponentLocation` (`self.PlayerPos`)) (`SceneComponent.K2_GetComponentRotation` (`self.PlayerPos`)) self)
    (else
      (`APlayerCharacter.StartAutoMoveCharacter` Player (`SceneComponent.K2_GetComponentLocation` (`self.PlayerPos1`)) (`SceneComponent.K2_GetComponentRotation` (`self.PlayerPos1`)) self))))

(fn `UserConstructionScript`
  (`parent.UserConstructionScript`))