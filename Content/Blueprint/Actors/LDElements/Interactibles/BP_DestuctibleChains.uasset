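; Destructible chain interactible that reports to its linked artifact when broken.
; At BeginPlay it pins both ends of the skeletal chain with constraints, slightly randomizes the static mesh yaw and adds an outline overlay material, shown on collider overlap.
; Damage breaks the end-link bone constraint, enables physics, destroys the static mesh and has BPArtifact check all chains.
; Its location is written to the color-modifier parameter collection as DepositPosition.
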(event `self.OutlineCollider.OnComponentBeginOverlap`
  (params (OverlappedComponent :type "PrimitiveComponent Object Reference") (OtherActor :type "Actor Object Reference") (OtherComp :type "PrimitiveComponent Object Reference") (OtherBodyIndex :type Integer) (bFromSweep :type Boolean) (SweepResult :type "HitResult Structure (by ref)"))
  ; OutlineOverlap
  (`MaterialInstanceDynamic.SetScalarParameterValue` (stale `self.ReceiveBeginPlay` _returnvalue) "IsVisible" 1.0))

(event `self.OutlineCollider.OnComponentEndOverlap`
  (params (OverlappedComponent :type "PrimitiveComponent Object Reference") (OtherActor :type "Actor Object Reference") (OtherComp :type "PrimitiveComponent Object Reference") (OtherBodyIndex :type Integer))
  ; OutlineOverlap
  (`MaterialInstanceDynamic.SetScalarParameterValue` (stale `self.ReceiveBeginPlay` _returnvalue) "IsVisible" 0.0))

(event `self.ReceiveBeginPlay`
  (`parent.ReceiveBeginPlay`)
  (`SceneComponent.K2_SetRelativeRotation` (`self.StaticMesh`) (`KismetMathLibrary.MakeRotator` 0.0 0.0 (`KismetMathLibrary.RandomFloatInRange` -10.0 10.0)) false false)
  (bind _returnvalue (`KismetMaterialLibrary.CreateDynamicMaterialInstance` "/Game/Art/Materials/Instances/Instances-FXs/MI_OutlineOverlay_02.MI_OutlineOverlay_02"))
  (`MeshComponent.SetOverlayMaterial` (`self.StaticMesh`) _returnvalue)
  (`KismetMaterialLibrary.SetVectorParameterValue` "/Game/Art/Materials/CollectionParameter/MPC_ColorModifiers.MPC_ColorModifiers" "DepositPosition" (`KismetMathLibrary.Conv_VectorToLinearColor` (`self.K2_GetActorLocation`)))
  (`self.Set Constraints`))

(event `self.ReceiveDamage`
  (params (Quantity :type "Float (single-precision)") (Origin :type "Actor Object Reference"))
  (`SkeletalMeshComponent.BreakConstraint` (`self.SkeletalMesh`) (0.0 0.0 0.0) (0.0 0.0 0.0) "Rig_Chain_Link_20")
  (`PrimitiveComponent.SetSimulatePhysics` (`self.SkeletalMesh`) true)
  (`PrimitiveComponent.SetSimulatePhysics` (`self.SkeletalMesh`) true)
  (`ActorComponent.K2_DestroyComponent` (`self.StaticMesh`))
  (set `self.isDestroy` true)
  (`/Game/Blueprint/Actors/LDElements/BP_Item_Artifact.CheckAllChainsState` (`self.BP_Artifact`)))

(event `Set Constraints`
  (bind _skeletalmesh (`self.SkeletalMesh`))
  (`PhysicsConstraintComponent.SetConstrainedComponents` (`self.StartConstraint`) _skeletalmesh "Rig_Chain_Root" null "None")
  (`PhysicsConstraintComponent.SetConstrainedComponents` (`self.EndConstraint`) _skeletalmesh "Rig_Chain_Link_20" null "None"))

(fn `UserConstructionScript`
  (`KismetMaterialLibrary.SetVectorParameterValue` "/Game/Art/Materials/CollectionParameter/MPC_ColorModifiers.MPC_ColorModifiers" "DepositPosition" (`KismetMathLibrary.Conv_VectorToLinearColor` (`self.K2_GetActorLocation`))))