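; Crushing-wall trap actor whose two walls close in on each other once the player enters it.
; The first player overlap starts a Timeline that lerps each wall toward the other's starting position and removes the first trigger.
; While active, Tick scales playback speed by player distance to a Target, slowing the walls as the player nears it.
; The next overlap ends that scaling, speeds the Timeline up sharply and removes the second trigger.
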(event `self.ReceiveBeginPlay`
  (set `self.MaxDistance` (`KismetMathLibrary.Vector_Distance` (`SceneComponent.K2_GetComponentLocation` (`self.Trigger Zone`)) (`SceneComponent.K2_GetComponentLocation` (`self.Target`)))))

(event `self.ReceiveActorBeginOverlap`
  (params (OtherActor :type "Actor Object Reference"))
  (bind _asbp_player_character (cast `/Game/Blueprint/Actors/Player/BP_PlayerCharacter` OtherActor))
  (set `self.Player` _asbp_player_character)
  (`/Engine/EditorBlueprintResources/StandardMacros.FlipFlop`
    (:`A`
      (`self.Activate`)
      (`ActorComponent.K2_DestroyComponent` (`self.Trigger Zone`)))
    (:`B`
      (set `self.isActivated` false)
      (`TimelineComponent.SetPlayRate` (`self.Timeline`) 5.0)
      (`ActorComponent.K2_DestroyComponent` (`self.Trigger Zone1`)))))

(event `Activate`
  (bind _startpos (`self.StartPos`))
  (bind _endpos (`self.EndPos`))
  (set `self.isActivated` true)
  (set `self.StartPos` (`SceneComponent.K2_GetComponentLocation` (`self.Wall 1`)))
  (set `self.EndPos` (`SceneComponent.K2_GetComponentLocation` (`self.Wall 2`)))
  (bind (_direction _alpha) (`Timeline|Timeline` :!via `PlayFromStart`)
    (:`Update`
      (`SceneComponent.K2_SetWorldLocation` (`self.Wall 1`) (`KismetMathLibrary.VLerp` _startpos _endpos _alpha) false false)
      (`SceneComponent.K2_SetWorldLocation` (`self.Wall 2`) (`KismetMathLibrary.VLerp` _endpos _startpos _alpha) false false))))

(event `self.ReceiveTick`
  (params (DeltaSeconds :type "Float (single-precision)"))
  (bind _maxdistance (`self.MaxDistance`))
  (if (`self.isActivated`)
    (`TimelineComponent.SetPlayRate` (`self.Timeline`) (`KismetMathLibrary.Lerp` 0.5 1.5 (/ (`KismetMathLibrary.FClamp` (`KismetMathLibrary.Vector_Distance` (`self.K2_GetActorLocation` (`self.Player`)) (`SceneComponent.K2_GetComponentLocation` (`self.Target`))) 0.0 _maxdistance) _maxdistance)))))

(fn `UserConstructionScript`)