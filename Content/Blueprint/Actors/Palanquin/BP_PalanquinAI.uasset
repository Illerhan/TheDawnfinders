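; AI controller for the palanquin that moves it to the location of the calling actor.
; CallPalanquin succeeds only when the cooldown is over and a resource remains, then spends one and restarts both timers.
; Tick counts down the cooldown and, only while resources are depleted, the recharge timer that restores one resource.
; A WBP_NewPalanquin widget created on BeginPlay displays cooldown, recharge progress and resource count.
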(event `self.ReceiveBeginPlay`
  (bind _returnvalue (`|CreateWidget` "/Game/UI/Widgets/WBP_NewPalanquin.WBP_NewPalanquin_C"))
  (bind _output_get (set `self.Widget` _returnvalue))
  (`UserWidget.AddToViewport` _output_get 0)
  (`self.Set Widget Chrono`)
  (`self.Set Widget Progress`)
  (`self.Set Widget Resource`))

(event `Call Palanquin`
  (params (Actor :type "/Game/Blueprint/Actors/Player/BP_PlayerCharacter Object Reference"))
  (bind _canmove (`self.CheckIfCanMove`))
  (if _canmove
    (`self.MoveToLocation` (`self.K2_GetActorLocation` Actor) -1.0 true true false true null)
    (set `self.CooldownTimer` (`self.Cooldown`))
    (`/Engine/EditorBlueprintResources/StandardMacros.DecrementInt` (`self.CurrentResources`)
      (:`  `
        (set `self.ResourceTimer` (`self.ResourceCooldown`))
        (`self.Set Widget Resource`)))
    (else
      (`KismetSystemLibrary.PrintString` "Can not move"))))

(event `self.ReceiveTick`
  (params (DeltaSeconds :type "Float (single-precision)"))
  (`self.Set Widget Chrono`)
  (`self.Set Widget Progress`)
  (set `self.CooldownTimer` (`KismetMathLibrary.FClamp` (- (`self.CooldownTimer`) DeltaSeconds) 0.0 (`self.Cooldown`)))
  (if (<= (`self.CurrentResources`) 0)
    (bind _output_get (set `self.ResourceTimer` (`KismetMathLibrary.FClamp` (- (`self.ResourceTimer`) DeltaSeconds) 0.0 (`self.ResourceCooldown`))))
    (if (<= _output_get 0.0)
      (`/Engine/EditorBlueprintResources/StandardMacros.IncrementInt` (`self.CurrentResources`)
        (:`  `
          (set `self.ResourceTimer` (`self.ResourceCooldown`))
          (`self.Set Widget Resource`))))))

(event `Set Widget Resource`
  (`/Game/UI/Widgets/WBP_NewPalanquin.Set Resource` (`self.Widget`) (`self.CurrentResources`)))

(event `Set Widget Progress`
  (`/Game/UI/Widgets/WBP_NewPalanquin.Set Progress` (`self.Widget`) (- 1.0 (/ (`self.ResourceTimer`) (`self.ResourceCooldown`)))))

(event `Set Widget Chrono`
  (`/Game/UI/Widgets/WBP_NewPalanquin.Set Chrono` (`self.Widget`) (`self.CooldownTimer`)))

(fn `CheckIfCanMove`
  (returns (CanMove :type Boolean))
  (return (and (<= (`self.CooldownTimer`) 0.0) (> (`self.CurrentResources`) 0))))

(fn `UserConstructionScript`)