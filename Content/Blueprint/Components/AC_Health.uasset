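; AC_Health is the player character's health component, extending parent health logic with visual feedback for damage and poison.
; Poison start and end call the parent, then multicast to toggle the player's poison Niagara effect and material color intensity.
; Ending poison also applies zero poison damage after a short delay.
; Tick writes the current hurt and poison strengths into a post-process material parameter collection to drive screen overlay opacity.
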(event `self.ReceiveBeginPlay`
  (bind _asbp_player_character (cast `/Game/Blueprint/Actors/Player/BP_PlayerCharacter` (`self.GetOwner`)))
  (set `self.Player` _asbp_player_character))

(event `self.StartPoisonEffects`
  ; Poison
  (`parent.StartPoisonEffects`)
  (`self.Multicast_StartPoison`))

(event `Multicast_StartPoison`
  ; Poison
  (`self.Activate` (`/Game/Blueprint/Actors/Player/BP_PlayerCharacter.NS_Poison` (`self.Player`)) false)
  (`MaterialInstanceDynamic.SetScalarParameterValue` (`/Game/Blueprint/Actors/Player/BP_PlayerCharacter.DynMatChara` (`self.Player`)) "Color Intensity" 2.0))

(event `self.EndPoisonEffects`
  ; Poison
  (`parent.EndPoisonEffects`)
  (`self.Multicast_EndPoison`))

(event `Multicast_EndPoison`
  ; Poison
  (`self.Deactivate` (`/Game/Blueprint/Actors/Player/BP_PlayerCharacter.NS_Poison` (`self.Player`)))
  (`MaterialInstanceDynamic.SetScalarParameterValue` (`/Game/Blueprint/Actors/Player/BP_PlayerCharacter.DynMatChara` (`self.Player`)) "Color Intensity" 0.0)
  (`KismetSystemLibrary.Delay` 0.1)
  (`self.TakeDamage` 0.0 "Poison"))

(event `self.ReceiveTick`
  (params (DeltaSeconds :type "Float (single-precision)"))
  (`parent.ReceiveTick` DeltaSeconds)
  (`KismetMaterialLibrary.SetScalarParameterValue` "/Game/Art/Materials/CollectionParameter/MPC_PostProcessEffects.MPC_PostProcessEffects" "DAMAGE-GeneralOpacity" (`self.CurrentHurtVolumeStrength`))
  (`KismetMaterialLibrary.SetScalarParameterValue` "/Game/Art/Materials/CollectionParameter/MPC_PostProcessEffects.MPC_PostProcessEffects" "POISON-GeneralOpacity" (`self.CurrentPoisonVolumeStrength`)))