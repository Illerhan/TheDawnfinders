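; Child Blueprint of a rotating bridge interactable that adds collision toggling to two cube components, Cube2 and Cube3.
; RotateEvent runs the parent rotation, then, unless IsFinalBridge is set, disables both cubes' collision when IsActivate is true and restores it otherwise.
; For the final bridge, BeginPlay only disables Cube3's collision and RotateEvent leaves collision untouched.
; BeginPlay overrides the parent without calling it.
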(event `self.RotateEvent`
  (`parent.RotateEvent`)
  (if (`self.isFinalBridge`)
    _
    (elif (`self.isActivate`)
      (`PrimitiveComponent.SetCollisionEnabled` (`self.Cube2`) "NoCollision")
      (`PrimitiveComponent.SetCollisionEnabled` (`self.Cube3`) "NoCollision")
      (else
        (`PrimitiveComponent.SetCollisionEnabled` (`self.Cube2`) "QueryAndPhysics")
        (`PrimitiveComponent.SetCollisionEnabled` (`self.Cube3`) "QueryAndPhysics")))))

(event `self.ReceiveBeginPlay`
  (if (`self.isFinalBridge`)
    (`PrimitiveComponent.SetCollisionEnabled` (`self.Cube3`) "NoCollision")))

(fn `UserConstructionScript`
  (`parent.UserConstructionScript`))