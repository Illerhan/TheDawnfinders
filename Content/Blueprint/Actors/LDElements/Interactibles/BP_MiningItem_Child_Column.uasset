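; Mining item child Blueprint for a column that falls by rotating from a start to an end rotation.
; Both its box and outline colliders have collision disabled at BeginPlay, after the parent's setup runs.
; FallEvent plays a timeline at a rate set by Timer, lerping the root's world rotation and enabling box physics and query collision plus query-only outline collision on update.
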(event `self.ReceiveBeginPlay`
  (`parent.ReceiveBeginPlay`)
  (`PrimitiveComponent.SetCollisionEnabled` (`self.BoxCollider`) "NoCollision")
  (`PrimitiveComponent.SetCollisionEnabled` (`self.OutlineCollider`) "NoCollision"))

(event `FallEvent`
  (`TimelineComponent.SetPlayRate` (`self.Timeline`) (`self.Timer`))
  (bind (_direction _track01) (`Timeline|Timeline`)
    (:`Update`
      (`SceneComponent.K2_SetWorldRotation` (`self.Rooot`) (`KismetMathLibrary.RLerp` (`self.StartRotation`) (`self.EndRotation`) _track01) false false)
      (`PrimitiveComponent.SetCollisionEnabled` (`self.BoxCollider`) "QueryAndPhysics")
      (`PrimitiveComponent.SetCollisionEnabled` (`self.OutlineCollider`) "QueryOnly"))))

(fn `UserConstructionScript`
  (`parent.UserConstructionScript`))