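; Base Blueprint for interactible chests, handling the opening interaction's animation and player positioning.
; The interaction animation event calls a multicast that plays the chest mesh's animation once at normal speed on networked clients.
; The auto-move event sends the interacting player to the location and rotation of the PlayerPos component.
; Construction defers to the parent class.
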(event `self.DoInteractionAnim`
  (params (Interactor :type "Actor Object Reference"))
  (`self.Multicast_PlayAnimation`))

(event `Multicast_PlayAnimation`
  (bind _chestmesh (`self.ChestMesh`))
  (`SkeletalMeshComponent.SetPlayRate` _chestmesh 1.0)
  (`SkeletalMeshComponent.Play` _chestmesh false))

(event `self.DoPlayerAutoMove`
  (params (PlayerToMove :type "APlayerCharacter Object Reference"))
  (`APlayerCharacter.StartAutoMoveCharacter` PlayerToMove (`SceneComponent.K2_GetComponentLocation` (`self.PlayerPos`)) (`SceneComponent.K2_GetComponentRotation` (`self.PlayerPos`)) self))

(fn `UserConstructionScript`
  (`parent.UserConstructionScript`))