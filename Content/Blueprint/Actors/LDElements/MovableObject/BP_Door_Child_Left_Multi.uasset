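; Left-side child door Blueprint that shoves players out of its Box volume while the door is neither fully open nor moving forward.
; Entering players' CharacterMovement components are tracked and pushed with a large force along the Box's right axis, toward their side of entry.
; A looping per-frame timer reapplies one shared force, set by the latest entrant, to all tracked players until the last one exits.
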(event `self.Box.OnComponentBeginOverlap`
  (params (OverlappedComponent :type "PrimitiveComponent Object Reference") (OtherActor :type "Actor Object Reference") (OtherComp :type "PrimitiveComponent Object Reference") (OtherBodyIndex :type Integer) (bFromSweep :type Boolean) (SweepResult :type "HitResult Structure (by ref)"))
  (bind _box (`self.Box`))
  (bind _returnvalue (`KismetMathLibrary.Normal` (`SceneComponent.GetRightVector` _box)))
  (bind _returnvalue_2 (* _returnvalue (* 1.0 2000000.0)))
  (bind _returnvalue_3 (* _returnvalue (* -1.0 2000000.0)))
  (if (and (not (`self.bIsFullyOpen`)) (not (`self.bIsMovingForward`)))
    (if (`self.ActorHasTag` OtherActor "Player")
      (bind _ascharacter (cast `Character` OtherActor))
      (bind _charactermovement (`Character.CharacterMovement` _ascharacter))
      (if (not (`KismetArrayLibrary.Array_Contains` (`self.PushCharacterMovement`) _charactermovement))
        (`KismetArrayLibrary.Array_Add` (`self.PushCharacterMovement`) _charactermovement)
        (if (< (`KismetMathLibrary.Dot_VectorVector` (`KismetMathLibrary.Normal` (- (`self.K2_GetActorLocation` OtherActor) (`SceneComponent.K2_GetComponentLocation` _box))) _returnvalue) 0.0)
          (set `self.Force` _returnvalue_3)
          (`CharacterMovementComponent.AddForce` _charactermovement _returnvalue_3)
          (else
            (set `self.Force` _returnvalue_2)
            (`CharacterMovementComponent.AddForce` _charactermovement _returnvalue_2)))
        (if (== (`KismetArrayLibrary.Array_Length` (`self.PushCharacterMovement`)) 1)
          (bind _returnvalue_4 (`KismetSystemLibrary.K2_SetTimerDelegate` (delegate `PushPlayer`) (`GameplayStatics.GetWorldDeltaSeconds`) true))
          (set `self.TimerHandle` _returnvalue_4))))))

(event `PushPlayer`
  (for _array_element (`self.PushCharacterMovement`)
    (`CharacterMovementComponent.AddForce` _array_element (`self.Force`))))

(event `self.Box.OnComponentEndOverlap`
  (params (OverlappedComponent :type "PrimitiveComponent Object Reference") (OtherActor :type "Actor Object Reference") (OtherComp :type "PrimitiveComponent Object Reference") (OtherBodyIndex :type Integer))
  (if (`self.ActorHasTag` OtherActor "Player")
    (bind _ascharacter (cast `Character` OtherActor))
    (`KismetArrayLibrary.Array_RemoveItem` (`self.PushCharacterMovement`) (`Character.CharacterMovement` _ascharacter))
    (if (== (`KismetArrayLibrary.Array_Length` (`self.PushCharacterMovement`)) 0)
      (`KismetSystemLibrary.K2_ClearAndInvalidateTimerHandle` (`self.TimerHandle`)))))

(fn `UserConstructionScript`
  (`parent.UserConstructionScript`))