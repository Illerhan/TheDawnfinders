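; AC_Light is a light component that extends its parent's light state handling to drive fog-of-war collision.
; After the parent ApplyLightState runs, LightOn switches FogOfWarLightOn between query-only and no collision.
; The off state also enables query collision on FogOfWarLightOff.
; The node that would disable FogOfWarLightOff is unconnected, so turning the light on leaves that collision unchanged.
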(event `self.ApplyLightState`
  (`parent.ApplyLightState`)
  (if (`self.bLightOn`)
    (`PrimitiveComponent.SetCollisionEnabled` (`self.FogOfWarLightOn`) "QueryOnly")
    (else
      (`PrimitiveComponent.SetCollisionEnabled` (`self.FogOfWarLightOn`) "NoCollision")
      (`PrimitiveComponent.SetCollisionEnabled` (`self.FogOfWarLightOff`) "QueryOnly"))))