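; Custom Game Instance that sets up the local player save and starts a multiplayer session when the game launches in a Lobby level.
; Init loads or creates the PlayerSave object and sets its Gold to a fixed amount either way.
; In a Lobby level, after a brief delay, it creates a session if the game state has none, then reopens L_LobbyMain as a listen server.
; SavePlayerData writes the save to its slot.
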(event `self.ReceiveInit`
  (`|ExecutionSequence`
    (:`then_0`
      (bind _returnvalue (`GameplayStatics.DoesSaveGameExist` "PlayerSave"))
      (if _returnvalue
        (bind _returnvalue_2 (`GameplayStatics.LoadGameFromSlot` "PlayerSave"))
        (bind _asbp_local_save (cast `/Game/Blueprint/GameFramework/BP_LocalSave` _returnvalue_2))
        (bind _output_get (set `self.GameSave` _asbp_local_save))
        (set `/Game/Blueprint/GameFramework/BP_LocalSave.Gold` 500 _output_get)
        (else
          (bind _returnvalue_3 (`GameplayStatics.CreateSaveGameObject` "/Game/Blueprint/GameFramework/BP_LocalSave.BP_LocalSave_C"))
          (bind _output_get_2 (set `self.GameSave` _returnvalue_3))
          (set `/Game/Blueprint/GameFramework/BP_LocalSave.Gold` 500 _output_get_2))))
    (:`then_1`
      (bind _returnvalue_4 (`GameplayStatics.GetCurrentLevelName` true))
      (if (not (== (`KismetStringLibrary.FindSubstring` _returnvalue_4 "Lobby") -1))
        (`KismetSystemLibrary.Delay` 0.2)
        (bind _asbp_custom_game_state (cast `/Game/Blueprint/GameFramework/BP_CustomGameState` (`GameplayStatics.GetGameState`)))
        (if (not (`/Game/Blueprint/GameFramework/BP_CustomGameState.bInSession` _asbp_custom_game_state))
          (`SessionManagerSubsystem.CreateAdvancesSession` (subsystem `SessionManagerSubsystem`) 4 4 false true false true)
          (set `/Game/Blueprint/GameFramework/BP_CustomGameState.bInSession` true _asbp_custom_game_state)
          (`GameplayStatics.OpenLevel` "L_LobbyMain" true "listen"))))))

(event `OnSessionCreated_Event`
  (params (bWasSuccesful :type Boolean)))

(fn `SavePlayerData`
  (`GameplayStatics.SaveGameToSlot` (`self.GameSave`) "PlayerSave"))