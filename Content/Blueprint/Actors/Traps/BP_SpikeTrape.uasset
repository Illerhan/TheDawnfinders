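; Spike trap actor that raises and lowers its spikes and damages actors that touch them.
; DoSpikeAnim, guarded against re-entry, drives spike height with a timeline while timed delays briefly enable the damage collider.
; Overlapping that collider sends a damage message to the other actor.
; BeginPlay gives spikes and base dynamic materials, stores them, and sets their opacity to zero.
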(event `self.ReceiveBeginPlay`
  (`parent.ReceiveBeginPlay`)
  (set `self.Spikes` (`|MakeArray` (`self.Spike8`) (`self.Spike7`) (`self.Spike6`) (`self.Spike5`) (`self.Spike4`) (`self.Spike3`) (`self.Spike2`) (`self.Spike1`) (`self.Spike`)))
  (for _array_element (`|MakeArray` (`self.Spike8`) (`self.Spike7`) (`self.Spike6`) (`self.Spike5`) (`self.Spike4`) (`self.Spike3`) (`self.Spike2`) (`self.Spike1`) (`self.Spike`) (`self.Base`) :!type "MeshComponent Object Reference")
    (for (_array_element_2 _array_index) (`MeshComponent.GetMaterials` _array_element)
      (bind _returnvalue (`KismetMaterialLibrary.CreateDynamicMaterialInstance` _array_element_2))
      (`KismetArrayLibrary.Array_Add` (`self.Materials`) _returnvalue)
      (`MaterialInstanceDynamic.SetScalarParameterValue` _returnvalue "Opacity" 0.0)
      (`PrimitiveComponent.SetMaterial` _array_element _array_index _returnvalue))))

(event `self.DoSpikeAnim`
  (if (not (`self.IsDoingAnim`))
    (set `self.IsDoingAnim` true)
    (`|ExecutionSequence`
      (:`then_0`
        (bind (_direction _newtrack_0) (`Timeline|SpikeYTimeline` :!via `PlayFromStart`)
          (:`Update`
            (for _array_element (`self.Spikes`)
              (`SceneComponent.K2_SetRelativeLocation` _array_element (`KismetMathLibrary.MakeVector` (.x (`SceneComponent.RelativeLocation` _array_element)) (.y (`SceneComponent.RelativeLocation` _array_element)) (+ (* _newtrack_0 100.0) -50.0)) false false)))
          (:`Finished`
            (set `self.IsDoingAnim` false))))
      (:`then_1`
        (`KismetSystemLibrary.Delay` 0.45)
        (`PrimitiveComponent.SetCollisionEnabled` (`self.SpikesOutCollider`) "QueryOnly")
        (`KismetSystemLibrary.Delay` 0.5)
        (`PrimitiveComponent.SetCollisionEnabled` (`self.SpikesOutCollider`) "NoCollision")))))

(event `self.SpikesOutCollider.OnComponentBeginOverlap`
  (params (OverlappedComponent :type "PrimitiveComponent Object Reference") (OtherActor :type "Actor Object Reference") (OtherComp :type "PrimitiveComponent Object Reference") (OtherBodyIndex :type Integer) (bFromSweep :type Boolean) (SweepResult :type "HitResult Structure (by ref)"))
  (message `Damageable.ReceiveDamage` OtherActor (`KismetMathLibrary.Conv_IntToDouble` (`self.Damages`)) self))

(fn `UserConstructionScript`)