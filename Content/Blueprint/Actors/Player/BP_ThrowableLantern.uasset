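; BP_ThrowableLantern is a player throwable lantern actor that carries a fog of war component.
; On BeginPlay it switches that component to absolute rotation, so it does not inherit the lantern's rotation.
; Every tick it moves the component to a fixed height above the mesh in world space, keeping it overhead however the lantern tumbles.
; Other behavior comes from the parent class, whose construction, BeginPlay and Tick it calls.
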(event `self.ReceiveBeginPlay`
  (`parent.ReceiveBeginPlay`)
  (set `SceneComponent.bAbsoluteRotation` true (`self.BP_FogOfWar`)))

(event `self.ReceiveTick`
  (params (DeltaSeconds :type "Float (single-precision)"))
  (`parent.ReceiveTick` DeltaSeconds)
  (`SceneComponent.K2_SetWorldLocation` (`self.BP_FogOfWar`) (+ (`SceneComponent.K2_GetComponentLocation` (`self.Mesh`)) (0.0 0.0 320.0)) false false))

(fn `UserConstructionScript`
  (`parent.UserConstructionScript`))